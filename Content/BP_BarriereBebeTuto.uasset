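; BP_BarriereBebeTuto is a barrier, apparently for the tutorial, that moves away once no BP_LilCrab actors remain in the world.
; Activate waits briefly, then enables a Tick check that polls GetAllActorsOfClass until none are found.
; It then calls GetUp, whose DoOnce-guarded timeline lerps the actor from its start location to EndPos, an offset converted to world space at BeginPlay.
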(event `self.ReceiveBeginPlay`
  (bind _returnvalue (`self.K2_GetActorLocation`))
  (set `self.InitialPos` _returnvalue)
  (set `self.EndPos` (+ (`self.EndPos`) _returnvalue)))

(event `Activate`
  (`KismetSystemLibrary.Delay` 0.8)
  (set `self.isActive` true))

(event `self.ReceiveTick`
  (params (DeltaSeconds :type "Float (single-precision)"))
  (if (`self.isActive`)
    (bind _outactors (`GameplayStatics.GetAllActorsOfClass` "/Game/Characters/Enemy/TrashMob/Ptit_Crab/BP_LilCrab.BP_LilCrab_C"))
    (if (<= (`KismetArrayLibrary.Array_Length` _outactors) 0)
      (set `self.isActive` false)
      (`self.GetUp`))))

(event `GetUp`
  (`/Engine/EditorBlueprintResources/StandardMacros.DoOnce` false
    (:`Completed`
      (bind (_direction _newtrack_0) (`Timeline|Timeline_0`)
        (:`Update`
          (`self.K2_SetActorLocation` (`KismetMathLibrary.VLerp` (`self.InitialPos`) (`self.EndPos`) _newtrack_0)))))))

(fn `UserConstructionScript`)