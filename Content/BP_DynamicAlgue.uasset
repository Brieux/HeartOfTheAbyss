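; BP_DynamicAlgue is an algae actor rendered with Niagara that feeds the player's position to its effect.
; The construction script passes spline offset, density and dispersion to Niagara and picks a Zlag or default material.
; The Zlag variant also adds point lights at regular intervals along the spline.
; Each tick, it converts the player mesh's location to actor space and sends X and Y to Niagara's Attr parameter.
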(event `self.ReceiveBeginPlay`)

(event `self.ReceiveTick`
  (params (DeltaSeconds :type "Float (single-precision)"))
  (bind (_returnvalue_x _returnvalue_y) (`KismetMathLibrary.BreakVector` (`KismetMathLibrary.InverseTransformLocation` (`self.GetTransform`) (`SceneComponent.K2_GetComponentLocation` (`Character.Mesh` (`GameplayStatics.GetPlayerCharacter` 0))))))
  (`FXSystemComponent.SetVectorParameter` (`self.Niagara`) "Attr" (`KismetMathLibrary.MakeVector` _returnvalue_x _returnvalue_y)))

(fn `UserConstructionScript`
  (bind _niagara (`self.Niagara`))
  (`FXSystemComponent.SetFloatParameter` (`self.Niagara`) "OffsetSpline" (`self.Offset`))
  (`FXSystemComponent.SetFloatParameter` (`self.Niagara`) "Density" (`self.Density`))
  (`FXSystemComponent.SetFloatParameter` _niagara "Dispertion" (`self.Disparité`))
  (`NiagaraComponent.SetVariableMaterial` _niagara "isZlag" (select `bool` (`self.isZlag`) :`false` "/Game/Props/Mesh/Algues/lambert1.lambert1" :`true` "/Game/Props/Mesh/Algues/algueBasicZlag.algueBasicZlag" :!type "MaterialInterface Object Reference"))
  (if (`self.isZlag`)
    (for _index (range 10)
      (if (== (mod _index 2) 0)
        (`AddComponent|NODE_AddPointLightComponent-0` :`RelativeTransform` (`KismetMathLibrary.MakeTransform` (`SplineComponent.GetLocationAtTime` (`self.Spline`) (/ _index 9) "Local" false)))))))