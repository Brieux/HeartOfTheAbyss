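; Ambience transition volume that tracks the state of overlap with two boxes, A and B, but plays no audio itself.
; Begin and end overlap events drive an AmbienceState enum through entry, both and exit states.
; BoxB's end overlap sets ExitA, not ExitB, from the unnamed state.
; While Active, Tick prints the state and turns two text labels toward the player character as debug feedback.
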(event `self.ReceiveTick`
  (params (DeltaSeconds :type "Float (single-precision)"))
  (bind _textrendera1 (`self.TextRenderA1`))
  (bind _textrendera (`self.TextRenderA`))
  (if (`self.Active`)
    (`KismetSystemLibrary.PrintString` (`|GetEnumeratorNameAsString` (`self.AmbienceState`)) true true (struct :`G` 0.66 :`B` 1.0 :`A` 1.0) 0.0)
    (`SceneComponent.K2_SetWorldRotation` _textrendera1 (`KismetMathLibrary.FindLookAtRotation` (`SceneComponent.K2_GetComponentLocation` _textrendera1) (`self.K2_GetActorLocation` (`GameplayStatics.GetPlayerCharacter` 0))) false false)
    (`SceneComponent.K2_SetWorldRotation` _textrendera (`KismetMathLibrary.FindLookAtRotation` (`SceneComponent.K2_GetComponentLocation` _textrendera) (`self.K2_GetActorLocation` (`GameplayStatics.GetPlayerCharacter` 0))) false false)))

(event `self.BoxA.OnComponentBeginOverlap`
  (params (OverlappedComponent :type "PrimitiveComponent Object Reference") (OtherActor :type "Actor Object Reference") (OtherComp :type "PrimitiveComponent Object Reference") (OtherBodyIndex :type Integer) (bFromSweep :type Boolean) (SweepResult :type "HitResult Structure (by ref)"))
  (switch `/Game/Mechanics/AmbienceTransition/EAmbienceType` (`self.AmbienceState`)
    (:`NewEnumerator0`
      (set `self.AmbienceState` "NewEnumerator1" :!label _label))
    (:`NewEnumerator2`
      (goto _label))
    (:`NewEnumerator3`
      (set `self.AmbienceState` "NewEnumerator5"))
    (:`NewEnumerator4`
      (goto _label))))

(event `self.BoxA.OnComponentEndOverlap`
  (params (OverlappedComponent :type "PrimitiveComponent Object Reference") (OtherActor :type "Actor Object Reference") (OtherComp :type "PrimitiveComponent Object Reference") (OtherBodyIndex :type Integer))
  (switch `/Game/Mechanics/AmbienceTransition/EAmbienceType` (`self.AmbienceState`)
    (:`NewEnumerator0`
      (set `self.AmbienceState` "NewEnumerator2"))
    (:`NewEnumerator1`
      (set `self.AmbienceState` "NewEnumerator2"))
    (:`NewEnumerator5`
      (set `self.AmbienceState` "NewEnumerator3"))))

(event `self.BoxB.OnComponentBeginOverlap`
  (params (OverlappedComponent :type "PrimitiveComponent Object Reference") (OtherActor :type "Actor Object Reference") (OtherComp :type "PrimitiveComponent Object Reference") (OtherBodyIndex :type Integer) (bFromSweep :type Boolean) (SweepResult :type "HitResult Structure (by ref)"))
  (switch `/Game/Mechanics/AmbienceTransition/EAmbienceType` (`self.AmbienceState`)
    (:`NewEnumerator0`
      (set `self.AmbienceState` "NewEnumerator3" :!label _label_2))
    (:`NewEnumerator1`
      (set `self.AmbienceState` "NewEnumerator5"))
    (:`NewEnumerator2`
      (goto _label_2))
    (:`NewEnumerator4`
      (goto _label_2))))

(event `self.BoxB.OnComponentEndOverlap`
  (params (OverlappedComponent :type "PrimitiveComponent Object Reference") (OtherActor :type "Actor Object Reference") (OtherComp :type "PrimitiveComponent Object Reference") (OtherBodyIndex :type Integer))
  (switch `/Game/Mechanics/AmbienceTransition/EAmbienceType` (`self.AmbienceState`)
    (:`NewEnumerator0`
      (set `self.AmbienceState` "NewEnumerator2"))
    (:`NewEnumerator3`
      (set `self.AmbienceState` "NewEnumerator4"))
    (:`NewEnumerator5`
      (set `self.AmbienceState` "NewEnumerator1"))))

(fn `UserConstructionScript`)