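; BP_DissloveTree is a VFX Blueprint that dissolves six spheres when a BP_SeaWatcher enters its SphereDestroy trigger while Activable is set.
; The overlap clears Activable and plays a timeline that drives Dissolve, Deforme and Brightness material parameters and multiplies each sphere's current world scale every update.
; When the timeline finishes, it destroys the spheres and BoxDestroy, then activates six Niagara effects.
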(event `self.SphereDestroy.OnComponentBeginOverlap`
  (params (OverlappedComponent :type "PrimitiveComponent Object Reference") (OtherActor :type "Actor Object Reference") (OtherComp :type "PrimitiveComponent Object Reference") (OtherBodyIndex :type Integer) (bFromSweep :type Boolean) (SweepResult :type "HitResult Structure (by ref)"))
  (if (`self.Activable`)
    (cast `/Game/Characters/SeaWatcher/BP_SeaWatcher` OtherActor)
    (`self.SphereAnimation`)))

(event `SphereAnimation`
  (bind _sphere3 (`self.Sphere3`))
  (bind _sphere1 (`self.Sphere1`))
  (bind _sphere2 (`self.Sphere2`))
  (bind _sphere4 (`self.Sphere4`))
  (bind _sphere5 (`self.Sphere5`))
  (bind _sphere6 (`self.Sphere6`))
  ;[0 1 0 1 30] ANIMATION VFX SPHERE
  (set `self.Activable` false)
  (bind (_direction _dissolve _deforme _brightness _scalecoef) (`Timeline|Timeline_SphereAnimation`)
    (:`Update`
      (`MeshComponent.SetScalarParameterValueOnMaterials` _sphere3 "Dissolve" _dissolve)
      (`MeshComponent.SetScalarParameterValueOnMaterials` _sphere1 "Dissolve" _dissolve)
      (`MeshComponent.SetScalarParameterValueOnMaterials` _sphere2 "Dissolve" _dissolve)
      (`MeshComponent.SetScalarParameterValueOnMaterials` _sphere4 "Dissolve" _dissolve)
      (`MeshComponent.SetScalarParameterValueOnMaterials` _sphere5 "Dissolve" _dissolve)
      (`MeshComponent.SetScalarParameterValueOnMaterials` _sphere6 "Dissolve" _dissolve)
      (`MeshComponent.SetScalarParameterValueOnMaterials` _sphere1 "Deforme" _deforme)
      (`MeshComponent.SetScalarParameterValueOnMaterials` _sphere2 "Deforme" _deforme)
      (`MeshComponent.SetScalarParameterValueOnMaterials` _sphere3 "Deforme" _deforme)
      (`MeshComponent.SetScalarParameterValueOnMaterials` _sphere4 "Deforme" _deforme)
      (`MeshComponent.SetScalarParameterValueOnMaterials` _sphere5 "Deforme" _deforme)
      (`MeshComponent.SetScalarParameterValueOnMaterials` _sphere6 "Deforme" _deforme)
      (`MeshComponent.SetScalarParameterValueOnMaterials` _sphere1 "Brightness" _brightness)
      (`MeshComponent.SetScalarParameterValueOnMaterials` _sphere2 "Brightness" _brightness)
      (`MeshComponent.SetScalarParameterValueOnMaterials` _sphere3 "Brightness" _brightness)
      (`MeshComponent.SetScalarParameterValueOnMaterials` _sphere4 "Brightness" _brightness)
      (`MeshComponent.SetScalarParameterValueOnMaterials` _sphere5 "Brightness" _brightness)
      (`MeshComponent.SetScalarParameterValueOnMaterials` _sphere6 "Brightness" _brightness)
      (`SceneComponent.SetWorldScale3D` _sphere1 (* (`SceneComponent.K2_GetComponentScale` _sphere1) _scalecoef))
      (`SceneComponent.SetWorldScale3D` _sphere2 (* (`SceneComponent.K2_GetComponentScale` _sphere2) _scalecoef))
      (`SceneComponent.SetWorldScale3D` _sphere3 (* (`SceneComponent.K2_GetComponentScale` _sphere3) _scalecoef))
      (`SceneComponent.SetWorldScale3D` _sphere4 (* (`SceneComponent.K2_GetComponentScale` _sphere4) _scalecoef))
      (`SceneComponent.SetWorldScale3D` _sphere5 (* (`SceneComponent.K2_GetComponentScale` _sphere5) _scalecoef))
      (`SceneComponent.SetWorldScale3D` _sphere6 (* (`SceneComponent.K2_GetComponentScale` _sphere6) _scalecoef)))
    (:`Finished`
      (`ActorComponent.K2_DestroyComponent` _sphere1)
      (`ActorComponent.K2_DestroyComponent` _sphere2)
      (`ActorComponent.K2_DestroyComponent` _sphere3)
      (`ActorComponent.K2_DestroyComponent` _sphere4)
      (`ActorComponent.K2_DestroyComponent` _sphere5)
      (`ActorComponent.K2_DestroyComponent` _sphere6)
      (`ActorComponent.K2_DestroyComponent` (`self.BoxDestroy`))
      ;;[1 0 1 1 30] ACTIVATE NS
      (`ActorComponent.Activate` (`self.Niagara1`) false)
      (`ActorComponent.Activate` (`self.Niagara2`) false)
      (`ActorComponent.Activate` (`self.Niagara3`) false)
      (`ActorComponent.Activate` (`self.Niagara4`) false)
      (`ActorComponent.Activate` (`self.Niagara5`) false)
      (`ActorComponent.Activate` (`self.Niagara6`) false))))

(fn `UserConstructionScript`)