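; BP_TentaclesType is a tentacle VFX actor that turns its Niagara effect on and off around a BP_SeaWatcher.
; The construction script sizes the trigger box and uses TentaculeType to pick the large or small tentacle system, setting it to auto-activate.
; Overlap events on the box activate the chosen system when a BP_SeaWatcher enters and deactivate it when one leaves.
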(event `self.TriggerActivate.OnComponentBeginOverlap`
  (params (OverlappedComponent :type "PrimitiveComponent Object Reference") (OtherActor :type "Actor Object Reference") (OtherComp :type "PrimitiveComponent Object Reference") (OtherBodyIndex :type Integer) (bFromSweep :type Boolean) (SweepResult :type "HitResult Structure (by ref)"))
  (cast `/Game/Characters/SeaWatcher/BP_SeaWatcher` OtherActor)
  (`ActorComponent.Activate` (`self.NS Tentacle`) false))

(event `self.TriggerActivate.OnComponentEndOverlap`
  (params (OverlappedComponent :type "PrimitiveComponent Object Reference") (OtherActor :type "Actor Object Reference") (OtherComp :type "PrimitiveComponent Object Reference") (OtherBodyIndex :type Integer))
  (cast `/Game/Characters/SeaWatcher/BP_SeaWatcher` OtherActor)
  (`ActorComponent.Deactivate` (`self.NS Tentacle`)))

(fn `UserConstructionScript`
  (`SceneComponent.SetWorldScale3D` (`self.TriggerActivate`) (`self.ScaleBoxTrigger`))
  (if (>= (`self.TentaculeType`) 1)
    (bind _output_get (set `self.NS Tentacle` (`self.NS Grand Tentacles`)))
    (`ActorComponent.SetAutoActivate` _output_get true)
    (else
      (bind _output_get_2 (set `self.NS Tentacle` (`self.NS Petit Tentacles`)))
      (`ActorComponent.SetAutoActivate` _output_get_2 true))))