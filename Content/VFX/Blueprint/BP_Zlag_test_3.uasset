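; Test VFX actor for a zlag absorption effect that travels from a BP_Crabe toward the BP_SeaWatcher's pearl, then destroys itself six seconds after spawning.
; Every tick it feeds the crab's location and the SeaWatcher's Bind_PearlSocket location into Niagara as spawn and aim positions, finding both actors by class lookup.
; An author comment notes that the link to the sphere socket does not work.
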(event `self.ReceiveBeginPlay`
  (`KismetSystemLibrary.Delay` 6.0)
  (`self.K2_DestroyActor`))

(event `TargetPosition`
  ;[1 1 1] Démarre une absorption de zlag qui va vers le joueur/sphere (le lien avec le socket de la sphere foctionne pas)
  (bind _returnvalue (`GameplayStatics.GetActorOfClass` "/Game/Characters/SeaWatcher/BP_SeaWatcher.BP_SeaWatcher_C"))
  (`NiagaraComponent.SetVariableVec3` (`self.Niagara`) "Aim_Position" (`SceneComponent.GetSocketLocation` (`Character.Mesh` _returnvalue) "Bind_PearlSocket")))

(event `SpawnPosition`
  ;[1 1 1] Démarre une absorption de zlag qui va vers le joueur/sphere (le lien avec le socket de la sphere foctionne pas)
  (bind _returnvalue (`GameplayStatics.GetActorOfClass` "/Game/Characters/Enemy/Boss/Crabe/BP_Crabe.BP_Crabe_C"))
  (`NiagaraComponent.SetVariableVec3` (`self.Niagara`) "Spawn_Position" (`self.K2_GetActorLocation` _returnvalue)))

(event `self.ReceiveTick`
  (params (DeltaSeconds :type "Float (single-precision)"))
  ;[1 1 1] Démarre une absorption de zlag qui va vers le joueur/sphere (le lien avec le socket de la sphere foctionne pas)
  (`self.TargetPosition`)
  (`self.SpawnPosition`))

(fn `UserConstructionScript`)