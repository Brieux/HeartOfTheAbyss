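; Zlag puddle hazard that slows and crouches the BP_SeaWatcher player and deals looping timer damage from BalancerRef while inside TriggerSlow.
; A second trigger, TriggerActivateTentacule, toggles the tentacle and bubble Niagara effects.
; While the player is caught, tentacle springs track a tail socket each Tick, with brightness and opacity ramping up, then fading on release.
; The construction script applies exposed scale values to the puddle sprite, tentacle shape and both triggers.
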(event `self.TriggerSlow.OnComponentBeginOverlap`
  (params (OverlappedComponent :type "PrimitiveComponent Object Reference") (OtherActor :type "Actor Object Reference") (OtherComp :type "PrimitiveComponent Object Reference") (OtherBodyIndex :type Integer) (bFromSweep :type Boolean) (SweepResult :type "HitResult Structure (by ref)"))
  (bind _asbp_sea_watcher (cast `/Game/Characters/SeaWatcher/BP_SeaWatcher` OtherActor))
  (set `/Game/Characters/SeaWatcher/BP_SeaWatcher.Slow` true _asbp_sea_watcher)
  (set `self.PlayerSlow` true)
  (`self.TentaclesCatchingPlayer`)
  (`Character.Crouch` _asbp_sea_watcher)
  (bind _returnvalue (`KismetSystemLibrary.K2_SetTimerDelegate` (delegate `DealDammage`) 1.0 true))
  (set `self.DOTHandler` _returnvalue))

(event `DealDammage`
  (bind _balancerref_dammageapply (break `/Game/GeneralSettings/Struct_DammageApplyOnPlayer` (`self.balancerRef`)))
  (bind _asbp_sea_watcher (cast `/Game/Characters/SeaWatcher/BP_SeaWatcher` (`GameplayStatics.GetPlayerCharacter` 0)))
  (`GameplayStatics.ApplyDamage` _asbp_sea_watcher (`BlueprintMapLibrary.Map_Find` _balancerref_dammageapply "NewEnumerator3"))
  (`/Game/Characters/SeaWatcher/BP_SeaWatcher.ResetDammage` _asbp_sea_watcher))

(event `self.ReceiveTick`
  (params (DeltaSeconds :type "Float (single-precision)"))
  (`self.PositionsCalcul`))

(event `self.TriggerSlow.OnComponentEndOverlap`
  (params (OverlappedComponent :type "PrimitiveComponent Object Reference") (OtherActor :type "Actor Object Reference") (OtherComp :type "PrimitiveComponent Object Reference") (OtherBodyIndex :type Integer))
  (bind _asbp_sea_watcher (cast `/Game/Characters/SeaWatcher/BP_SeaWatcher` OtherActor))
  (set `/Game/Characters/SeaWatcher/BP_SeaWatcher.Slow` false _asbp_sea_watcher)
  (set `self.PlayerSlow` false)
  (`self.TentaclesCatchingPlayer`)
  (`Character.UnCrouch` _asbp_sea_watcher)
  (if (`KismetSystemLibrary.K2_IsValidTimerHandle` (`self.DOTHandler`))
    (`KismetSystemLibrary.K2_ClearAndInvalidateTimerHandle` (`self.DOTHandler`))))

(event `self.ReceiveBeginPlay`
  (bind _returnvalue (`GameplayStatics.GetActorOfClass` "/Game/Characters/SeaWatcher/BP_SeaWatcher.BP_SeaWatcher_C"))
  (set `self.BP Sea Watcher Ref` _returnvalue)
  (set `self.SocketName_Aim` "Bind_Tail_01"))

(event `PositionsCalcul`
  ;[1 1 1] VFX CATCH AND FREE PLAYER
  (if (`self.PlayerSlow`)
    (`NiagaraComponent.SetVariableVec3` (`self.NS TentaclesCatchingPlayer`) "SpringEPosition" (`SceneComponent.GetSocketLocation` (`Character.Mesh` (`self.BP Sea Watcher Ref`)) (`self.SocketName_Aim`)))
    (`NiagaraComponent.SetVariableFloat` (`self.NS TentaclesCatchingPlayer`) "Brightness" (`self.BrightnessValue`))
    (`NiagaraComponent.SetVariableFloat` (`self.NS TentaclesCatchingPlayer`) "Opacity" (`self.OpacityValue`))
    (if (< (`self.BrightnessValue`) 100.0)
      (set `self.BrightnessValue` (+ (`self.BrightnessValue`) 5.0))
      (else
        (set `self.BrightnessValue` 100.0)))
    (if (< (`self.OpacityValue`) 2.0)
      (set `self.OpacityValue` (+ (`self.OpacityValue`) 0.1))
      (else
        (set `self.OpacityValue` 2.0)))
    (else
      (`NiagaraComponent.SetVariableFloat` (`self.NS TentaclesCatchingPlayer`) "Brightness" (`self.BrightnessValue`))
      (`NiagaraComponent.SetVariableFloat` (`self.NS TentaclesCatchingPlayer`) "Opacity" (`self.OpacityValue`))
      (if (> (`self.BrightnessValue`) 10.0)
        (set `self.BrightnessValue` (- (`self.BrightnessValue`) 10.0))
        (else
          (set `self.BrightnessValue` 10.0)))
      (if (> (`self.OpacityValue`) 0.0)
        (set `self.OpacityValue` (- (`self.OpacityValue`) 0.2))
        (else
          (set `self.OpacityValue` 0.0))))))

(event `TentaclesCatchingPlayer`
  ;[1 1 1] VFX CATCH AND FREE PLAYER
  (if (`/Game/Characters/SeaWatcher/BP_SeaWatcher.isDead` (`self.BP Sea Watcher Ref`))
    (`NiagaraComponent.SetVariableFloat` (`self.NS TentaclesCatchingPlayer`) "SpringForce" 0.0 :!label _label)
    (`ActorComponent.Deactivate` (`/Game/Characters/SeaWatcher/BP_SeaWatcher.NS ZlagSlow` (`self.BP Sea Watcher Ref`)))
    (elif (`self.PlayerSlow`)
      (`NiagaraComponent.SetVariableFloat` (`self.NS TentaclesCatchingPlayer`) "SpringForce" 10.0)
      (`ActorComponent.Activate` (`/Game/Characters/SeaWatcher/BP_SeaWatcher.NS ZlagSlow` (`self.BP Sea Watcher Ref`)) false)
      (else
        (goto _label)))))

(event `ScaleFlaque`
  ;[1 1 1] VFX CATCH AND FREE PLAYER
  (`NiagaraComponent.SetVariableFloat` (`self.NS ZlagZone`) "ScaleSpriteX" (`self.ScaleSpriteXValue`))
  (`NiagaraComponent.SetVariableFloat` (`self.NS ZlagZone`) "ScaleSpriteY" (`self.ScaleSpriteYValue`)))

(event `ScaleTentShapeLoc`
  ;[1 1 1] VFX CATCH AND FREE PLAYER
  (`NiagaraComponent.SetVariableVec2` (`self.NS TentaclesCatchingPlayer`) "ScaleShapeLocation" (`self.ScaleShapeLocationValue`)))

(event `ScaleTriggerSlow`
  ;[1 1 1] VFX CATCH AND FREE PLAYER
  (`SceneComponent.SetWorldScale3D` (`self.TriggerSlow`) (`self.ScaleTriggerSlowValue`)))

(event `ScaleTriggerActivate`
  ;[1 1 1] VFX CATCH AND FREE PLAYER
  (`SceneComponent.SetWorldScale3D` (`self.TriggerActivateTentacule`) (`self.ScaleTriggerActivateValue`)))

(event `self.TriggerActivateTentacule.OnComponentBeginOverlap`
  (params (OverlappedComponent :type "PrimitiveComponent Object Reference") (OtherActor :type "Actor Object Reference") (OtherComp :type "PrimitiveComponent Object Reference") (OtherBodyIndex :type Integer) (bFromSweep :type Boolean) (SweepResult :type "HitResult Structure (by ref)"))
  (cast `/Game/Characters/SeaWatcher/BP_SeaWatcher` OtherActor)
  (`ActorComponent.Activate` (`self.NS TentaclesCatchingPlayer`) false)
  (`ActorComponent.Activate` (`self.NS ZlagZoneBubble`) false))

(event `self.TriggerActivateTentacule.OnComponentEndOverlap`
  (params (OverlappedComponent :type "PrimitiveComponent Object Reference") (OtherActor :type "Actor Object Reference") (OtherComp :type "PrimitiveComponent Object Reference") (OtherBodyIndex :type Integer))
  (cast `/Game/Characters/SeaWatcher/BP_SeaWatcher` OtherActor)
  (`ActorComponent.Deactivate` (`self.NS TentaclesCatchingPlayer`))
  (`ActorComponent.Deactivate` (`self.NS ZlagZoneBubble`)))

(fn `UserConstructionScript`
  (`self.ScaleFlaque`)
  (`self.ScaleTriggerSlow`)
  (`self.ScaleTentShapeLoc`)
  (`self.ScaleTriggerActivate`))