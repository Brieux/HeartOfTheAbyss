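; BP_ZlagBall is a projectile pickup that adds to the BP_SeaWatcher player's Jauge gauge.
; The construction script sets launch speed from the player's WhoIsHit value: zero for CrabDeath, randomized for Blop or Eugene.
; Its first hit stops movement and physics, swaps spawn VFX for emission, starts a timeline bounce and enables pickup collision.
; Player overlap triggers the UI flip, spawns BP_Zlag_test_2 and destroys the ball.
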(event `self.ReceiveBeginPlay`
  (`TimelineComponent.SetPlayRate` (`self.Timeline_0`) (`KismetMathLibrary.RandomFloatInRange` 0.4 0.6))
  (`PrimitiveComponent.SetCollisionEnabled` (`self.Sphere1`) "NoCollision")
  (`self.SwitchColorMat`))

(event `Bounce`
  (bind _zoffset (`self.ZOffset`))
  (bind _sphere (`self.Sphere`))
  (bind (_relativelocation_x _relativelocation_y) (`KismetMathLibrary.BreakVector` (`SceneComponent.RelativeLocation` _sphere)))
  (bind (_relativelocation_x_2 _relativelocation_y_2 _relativelocation_z) (`KismetMathLibrary.BreakVector` (`SceneComponent.RelativeLocation` (`self.Sphere`))))
  ;[1 1 1] BOUNCE EFFECT
  (set `self.ZOffset` _relativelocation_z)
  (bind (_direction _newtrack_0) (`Timeline|Timeline_0`)
    (:`Update`
      (`SceneComponent.K2_SetRelativeLocation` _sphere (`KismetMathLibrary.VLerp` (`KismetMathLibrary.MakeVector` _relativelocation_x _relativelocation_y _zoffset) (`KismetMathLibrary.MakeVector` _relativelocation_x _relativelocation_y (+ _zoffset (* _newtrack_0 10.0))) _newtrack_0) false false))))

(event `SwitchColorMat`
  (`MeshComponent.SetVectorParameterValueOnMaterials` (`self.Sphere`) "ColorFresnel1" (6.0 0.0 2.0))
  (`MeshComponent.SetVectorParameterValueOnMaterials` (`self.Sphere`) "ExplosionColor" (6.0 0.0 2.0))
  (`Timeline|Timeline_SwitchColorMat`))

(event `self.Sphere1.OnComponentBeginOverlap`
  (params (OverlappedComponent :type "PrimitiveComponent Object Reference") (OtherActor :type "Actor Object Reference") (OtherComp :type "PrimitiveComponent Object Reference") (OtherBodyIndex :type Integer) (bFromSweep :type Boolean) (SweepResult :type "HitResult Structure (by ref)"))
  ;[1 1 1] OVERLAP PLAYER
  (bind _asbp_sea_watcher (cast `/Game/Characters/SeaWatcher/BP_SeaWatcher` OtherActor))
  (if true
    (set `/Game/Characters/SeaWatcher/BP_SeaWatcher.Jauge` (+ (`/Game/Characters/SeaWatcher/BP_SeaWatcher.Jauge` _asbp_sea_watcher) 2.0) _asbp_sea_watcher)
    (`/Game/UI/UI_Interface.PlayFlip` (`/Game/Characters/SeaWatcher/BP_SeaWatcher.UI_Ref` _asbp_sea_watcher))
    (`|SpawnActorFromClass` "/Game/VFX/Blueprint/BP_Zlag_test_2.BP_Zlag_test_2_C" (`self.GetTransform`) "AlwaysSpawn" "OverrideRootScale" null null)
    (`self.K2_DestroyActor`)))

(event `self.Sphere.OnComponentHit`
  (params (HitComponent :type "PrimitiveComponent Object Reference") (OtherActor :type "Actor Object Reference") (OtherComp :type "PrimitiveComponent Object Reference") (NormalImpulse :type "Vector Structure") (Hit :type "HitResult Structure (by ref)"))
  ;[1 1 1] ON HIT WITH GROUNG
  (`/Engine/EditorBlueprintResources/StandardMacros.DoOnce` false
    (:`Completed`
      (set `self.CanBeTake` true)
      (`self.K2_SetActorRotation` (struct))
      (`ActorComponent.K2_DestroyComponent` (`self.NS Spawn`))
      (`ActorComponent.Activate` (`self.NS Emission`) false)
      (`ActorComponent.K2_DestroyComponent` (`self.ProjectileMovement`))
      (`PrimitiveComponent.SetSimulatePhysics` (`self.Sphere`) false)
      (`self.Bounce`)
      (`PrimitiveComponent.SetCollisionEnabled` (`self.Sphere1`) "QueryOnly"))))

(fn `UserConstructionScript`
  (bind _projectilemovement (`self.ProjectileMovement`))
  (bind _speed (`self.Speed`))
  (bind _returnvalue (`GameplayStatics.GetActorOfClass` "/Game/Characters/SeaWatcher/BP_SeaWatcher.BP_SeaWatcher_C"))
  (set `self.BP SeaWatcher Ref` _returnvalue)
  (if (`KismetStringLibrary.EqualEqual_StrStr` (`/Game/Characters/SeaWatcher/BP_SeaWatcher.WhoIsHit` (`self.BP SeaWatcher Ref`)) "CrabDeath")
    (set `self.Speed` (`KismetMathLibrary.RandomFloatInRange` 0.0))
    (set `ProjectileMovementComponent.InitialSpeed` _speed _projectilemovement :!label _label)
    (set `ProjectileMovementComponent.MaxSpeed` _speed _projectilemovement)
    (elif (`KismetStringLibrary.EqualEqual_StrStr` (`/Game/Characters/SeaWatcher/BP_SeaWatcher.WhoIsHit` (`self.BP SeaWatcher Ref`)) "Blop")
      (set `self.Speed` (`KismetMathLibrary.RandomFloatInRange` 750.0 1250.0))
      (goto _label)
      (elif (`KismetStringLibrary.EqualEqual_StrStr` (`/Game/Characters/SeaWatcher/BP_SeaWatcher.WhoIsHit` (`self.BP SeaWatcher Ref`)) "Eugene")
        (set `self.Speed` (`KismetMathLibrary.RandomFloatInRange` 1000.0 1250.0))
        (goto _label)))))