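; Spline fish VFX actor that moves two Niagara effects along a spline, with an attached fish-wave ambient sound.
; On BeginPlay it starts the sound and a timeline whose play rate scales inversely with the Time variable.
; The timeline's track maps to distance along the spline, moving the first effect every update.
; The second follows through a Delay, so it jumps to the current position about every 1.5 seconds rather than trailing smoothly.
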(event `self.ReceiveBeginPlay`
  (bind _spline (`self.Spline`))
  (`GameplayStatics.SpawnSoundAttached` "/Game/Sound/Ambs/Fish/AMB_FishWaves_LP_Cue.AMB_FishWaves_LP_Cue" (`self.Audio`) "None" (0.0 0.0 0.0) (struct) "KeepRelativeOffset" false 1.0 1.0 0.0 null null)
  (`TimelineComponent.SetPlayRate` (`self.Timeline_0`) (/ 0.4 (`self.time`)))
  (bind (_direction _movetrack) (`Timeline|Timeline_0`)
    (:`Update`
      (bind _returnvalue (`SplineComponent.GetLocationAtDistanceAlongSpline` _spline (`KismetMathLibrary.Lerp` 0.0 (`SplineComponent.GetSplineLength` _spline) _movetrack) "World"))
      (`SceneComponent.K2_SetWorldLocation` (`self.Niagara`) _returnvalue false false)
      (`KismetSystemLibrary.Delay` 1.5)
      (`SceneComponent.K2_SetWorldLocation` (`self.Niagara1`) _returnvalue false false))))

(fn `UserConstructionScript`)