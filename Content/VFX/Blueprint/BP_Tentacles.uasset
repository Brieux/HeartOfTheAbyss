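; BP_Tentacles is a VFX actor that shows a large or small tentacle effect, which reacts to the proximity of BP_SeaWatcher.
; The construction script uses TentaculeType to pick NSGrandTentacule or NSPetitTentacule and sets it to auto-activate.
; A SetTentaculeType event makes the same choice and disables auto-activation on the other effect.
; The TriggerActivate volume activates the chosen effect when a SeaWatcher enters and deactivates it on exit.
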(event `self.ReceiveBeginPlay`
  (bind _returnvalue (`GameplayStatics.GetActorOfClass` "/Game/Characters/SeaWatcher/BP_SeaWatcher.BP_SeaWatcher_C"))
  (set `self.BP Sea Watcher Ref` _returnvalue))

(event `SetTentaculeType`
  (bind _ns_grand_tentacule (`self.NS Grand Tentacule`))
  (bind _ns_petit_tentacule (`self.NS Petit Tentacule`))
  (if (>= (`self.TentaculeType`) 1)
    (set `self.NS Tentacule` _ns_grand_tentacule)
    (`ActorComponent.SetAutoActivate` _ns_grand_tentacule true)
    (`ActorComponent.SetAutoActivate` (`self.NS Petit Tentacule`) false)
    (else
      (set `self.NS Tentacule` _ns_petit_tentacule)
      (`ActorComponent.SetAutoActivate` _ns_petit_tentacule true)
      (`ActorComponent.SetAutoActivate` (`self.NS Grand Tentacule`) false))))

(event `self.TriggerActivate.OnComponentBeginOverlap`
  (params (OverlappedComponent :type "PrimitiveComponent Object Reference") (OtherActor :type "Actor Object Reference") (OtherComp :type "PrimitiveComponent Object Reference") (OtherBodyIndex :type Integer) (bFromSweep :type Boolean) (SweepResult :type "HitResult Structure (by ref)"))
  (cast `/Game/Characters/SeaWatcher/BP_SeaWatcher` OtherActor)
  (`ActorComponent.Activate` (`self.NS Tentacule`) false))

(event `self.TriggerActivate.OnComponentEndOverlap`
  (params (OverlappedComponent :type "PrimitiveComponent Object Reference") (OtherActor :type "Actor Object Reference") (OtherComp :type "PrimitiveComponent Object Reference") (OtherBodyIndex :type Integer))
  (cast `/Game/Characters/SeaWatcher/BP_SeaWatcher` OtherActor)
  (`ActorComponent.Deactivate` (`self.NS Tentacule`)))

(fn `UserConstructionScript`
  (if (>= (`self.TentaculeType`) 1)
    (bind _output_get (set `self.NS Tentacule` (`self.NS Grand Tentacule`)))
    (`ActorComponent.SetAutoActivate` _output_get true)
    (else
      (bind _output_get_2 (set `self.NS Tentacule` (`self.NS Petit Tentacule`)))
      (`ActorComponent.SetAutoActivate` _output_get_2 true))))