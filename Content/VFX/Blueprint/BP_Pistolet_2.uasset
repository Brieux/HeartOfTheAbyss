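; BP_Pistolet_2 is a homing projectile tied to a crab reference (CrabeRef) that seeks and damages the BP_SeaWatcher player.
; On BeginPlay it finds the SeaWatcher and sets its mesh as the ProjectileMovement homing target.
; Box overlap applies fixed damage to the SeaWatcher, credited to the crab's controller.
; Other overlapping actors go through a second cast, whose target type is unnamed, to call HitByCrabe.
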(event `self.ReceiveBeginPlay`
  (bind _returnvalue (`GameplayStatics.GetActorOfClass` "/Game/Characters/SeaWatcher/BP_SeaWatcher.BP_SeaWatcher_C"))
  (bind _output_get (set `self.PlayerRef` _returnvalue))
  (set `ProjectileMovementComponent.HomingTargetComponent` (`Character.Mesh` _output_get) (`self.ProjectileMovement`)))

(event `self.Box.OnComponentBeginOverlap`
  (params (OverlappedComponent :type "PrimitiveComponent Object Reference") (OtherActor :type "Actor Object Reference") (OtherComp :type "PrimitiveComponent Object Reference") (OtherBodyIndex :type Integer) (bFromSweep :type Boolean) (SweepResult :type "HitResult Structure (by ref)"))
  (bind _asbp_sea_watcher (cast `/Game/Characters/SeaWatcher/BP_SeaWatcher` OtherActor)
    (:`then`
      (`GameplayStatics.ApplyDamage` _asbp_sea_watcher 20.0 null (`Pawn.GetController` (`self.CrabeRef`))))
    (:`CastFailed`
      (bind _asbp_socle_pillar (cast `` OtherActor))
      (`self.HitByCrabe` _asbp_socle_pillar))))

(fn `UserConstructionScript`)