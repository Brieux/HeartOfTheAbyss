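; Spline fish VFX actor that moves a Niagara effect along a spline from start to end.
; On BeginPlay it sets a timeline play rate from the Time variable and plays the movement timeline.
; Each update maps the Movetrack value to a distance along the spline and places the Niagara component at that world location, leaving rotation untouched.
; A trailing Delay follows each update with nothing connected after it.
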(event `self.ReceiveBeginPlay`
  (bind _spline (`self.Spline`))
  (`TimelineComponent.SetPlayRate` (`self.Timeline_0`) (/ 0.4 (`self.time`)))
  (bind (_direction _movetrack) (`Timeline|Timeline_0`)
    (:`Update`
      (`SceneComponent.K2_SetWorldLocation` (`self.Niagara`) (`SplineComponent.GetLocationAtDistanceAlongSpline` _spline (`KismetMathLibrary.Lerp` 0.0 (`SplineComponent.GetSplineLength` _spline) _movetrack) "World") false false)
      (`KismetSystemLibrary.Delay` 1.5))))

(fn `UserConstructionScript`)