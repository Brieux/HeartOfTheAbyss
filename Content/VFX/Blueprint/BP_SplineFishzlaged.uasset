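; Spline fish VFX actor that moves two Niagara effects and a small fish-group sound along a spline.
; On BeginPlay it attaches the sound to the Audio component and plays a timeline, its rate scaled by the Time variable.
; The timeline track sets the first effect's distance along the spline each update.
; A Delay inside the update makes the second effect and audio jump to the current point only periodically.
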(event `self.ReceiveBeginPlay`
  (bind _spline (`self.Spline`))
  (`GameplayStatics.SpawnSoundAttached` "/Game/Sound/Ambs/Fish/SFX_Small_GrpFish_LP_TEST.SFX_Small_GrpFish_LP_TEST" (`self.Audio`) "None" (0.0 0.0 0.0) (struct) "KeepRelativeOffset" false 1.0 1.0 0.0 null null)
  (`TimelineComponent.SetPlayRate` (`self.Timeline_0`) (/ 0.4 (`self.time`)))
  (bind (_direction _movetrack) (`Timeline|Timeline_0`)
    (:`Update`
      (bind _returnvalue (`SplineComponent.GetLocationAtDistanceAlongSpline` _spline (`KismetMathLibrary.Lerp` 0.0 (`SplineComponent.GetSplineLength` _spline) _movetrack) "World"))
      (`SceneComponent.K2_SetWorldLocation` (`self.Niagara`) _returnvalue false false)
      (`KismetSystemLibrary.Delay` 1.5)
      (`SceneComponent.K2_SetWorldLocation` (`self.Niagara1`) _returnvalue false false)
      (`SceneComponent.K2_SetWorldLocation` (`self.Audio`) _returnvalue false false))))

(fn `UserConstructionScript`)