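; BP_SwitchSandPatticles is a trigger volume that recolors the SeaWatcher's sand dust effects as it enters or leaves a sand area.
; Overlap events on the SandYelow component cast the other actor to BP_SeaWatcher and set the Color parameter on its move, idle and dash dust effects.
; Entering applies a warm yellow tint and leaving applies a pale cyan one.
; The construction script sizes the trigger from the ScaleTrigger variable.
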(event `self.ReceiveBeginPlay`)

(event `self.SandYelow.OnComponentBeginOverlap`
  (params (OverlappedComponent :type "PrimitiveComponent Object Reference") (OtherActor :type "Actor Object Reference") (OtherComp :type "PrimitiveComponent Object Reference") (OtherBodyIndex :type Integer) (bFromSweep :type Boolean) (SweepResult :type "HitResult Structure (by ref)"))
  (bind _asbp_sea_watcher (cast `/Game/Characters/SeaWatcher/BP_SeaWatcher` OtherActor))
  (`NiagaraComponent.SetVariableVec3` (`/Game/Characters/SeaWatcher/BP_SeaWatcher.NS DustSandMove` _asbp_sea_watcher) "Color" (1.0 0.7 0.4))
  (`NiagaraComponent.SetVariableVec3` (`/Game/Characters/SeaWatcher/BP_SeaWatcher.NS DustSandIddle` _asbp_sea_watcher) "Color" (1.0 0.7 0.4))
  (`NiagaraComponent.SetVariableVec3` (`/Game/Characters/SeaWatcher/BP_SeaWatcher.NS_DustDash` _asbp_sea_watcher) "Color" (1.0 0.7 0.4)))

(event `self.SandYelow.OnComponentEndOverlap`
  (params (OverlappedComponent :type "PrimitiveComponent Object Reference") (OtherActor :type "Actor Object Reference") (OtherComp :type "PrimitiveComponent Object Reference") (OtherBodyIndex :type Integer))
  (bind _asbp_sea_watcher (cast `/Game/Characters/SeaWatcher/BP_SeaWatcher` OtherActor))
  (`NiagaraComponent.SetVariableVec3` (`/Game/Characters/SeaWatcher/BP_SeaWatcher.NS DustSandMove` _asbp_sea_watcher) "Color" (0.7 1.0 0.9))
  (`NiagaraComponent.SetVariableVec3` (`/Game/Characters/SeaWatcher/BP_SeaWatcher.NS DustSandIddle` _asbp_sea_watcher) "Color" (0.7 1.0 0.9))
  (`NiagaraComponent.SetVariableVec3` (`/Game/Characters/SeaWatcher/BP_SeaWatcher.NS_DustDash` _asbp_sea_watcher) "Color" (0.7 1.0 0.9)))

(fn `UserConstructionScript`
  (`SceneComponent.SetWorldScale3D` (`self.SandYelow`) (`self.ScaleTrigger`)))