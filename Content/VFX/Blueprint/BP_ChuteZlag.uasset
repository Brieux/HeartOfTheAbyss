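; Zlag chute actor with a puddle (Flaque) that reacts to BP_SeaWatcher.
; Spawner instances spawn Zlag on a looping timer while the watcher is in the Box, until its gauge fills.
; ResetDeath spawns a BP_BIGZlagBall once on spawners, enabling sphere overlaps that dissolve the puddle in or out, with collection audio.
; Scaling and Descaling timelines alternate with random delays to pulse the puddle's size.
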(event `DesableChute`
  ;[1 1 1] PasUtilisé
  (`SceneComponent.SetVisibility` (`self.Chute`) false false)
  (`SceneComponent.SetVisibility` (`self.Trou`) true false))

(event `self.SphereCollison_Spawn.OnComponentBeginOverlap`
  (params (OverlappedComponent :type "PrimitiveComponent Object Reference") (OtherActor :type "Actor Object Reference") (OtherComp :type "PrimitiveComponent Object Reference") (OtherBodyIndex :type Integer) (bFromSweep :type Boolean) (SweepResult :type "HitResult Structure (by ref)"))
  (cast `/Game/Characters/SeaWatcher/BP_SeaWatcher` OtherActor)
  (if (`self.BZBSpawned`)
    (`self.ApparitionFlaque`)))

(event `EnableChute`
  ;[1 1 1] PasUtilisé
  (`SceneComponent.SetVisibility` (`self.Chute`) true false)
  (`SceneComponent.SetVisibility` (`self.Trou`) false false))

(event `self.SphereCollision_Ramassage.OnComponentBeginOverlap`
  (params (OverlappedComponent :type "PrimitiveComponent Object Reference") (OtherActor :type "Actor Object Reference") (OtherComp :type "PrimitiveComponent Object Reference") (OtherBodyIndex :type Integer) (bFromSweep :type Boolean) (SweepResult :type "HitResult Structure (by ref)"))
  (cast `/Game/Characters/SeaWatcher/BP_SeaWatcher` OtherActor)
  (if (`self.BZBSpawned`)
    (`self.DisparitionFlaque`)
    (`GameplayStatics.PlaySound2D` "/Game/Sound/UI/SFX_FontaineZlag_Collect.SFX_FontaineZlag_Collect" 1.0 1.0 0.0 null null)
    (`AudioComponent.FadeOut` (`self.AudioLoopFontaine`) 0.5 0.0 "Linear")))

(event `Scaling`
  ;[1 1 1] Scaling flaque random delay
  (`KismetSystemLibrary.Delay` (`KismetMathLibrary.RandomFloatInRange` 1.0 6.0))
  (bind (_direction _multiplyscale) (`Timeline|Timeline_Scaling` :!via `PlayFromStart`)
    (:`Update`
      (set `self.ScaleCurent` (* _multiplyscale (`self.ScaleBase`)))
      (`SceneComponent.SetWorldScale3D` (`self.Flaque`) (`self.ScaleCurent`)))
    (:`Finished`
      (`self.Descaling`))))

(event `ApparitionFlaque`
  ;[1 0.8608 0] SPAWN & DESPAWN FLAQUE (played in BP_BIGZlagBall)
  (bind (_direction _dissolvevalue) (`Timeline|Timeline_Spawn`)
    (:`Update`
      (`MeshComponent.SetScalarParameterValueOnMaterials` (`self.Flaque`) "Dissolve" _dissolvevalue))))

(event `DisparitionFlaque`
  (bind _flaque (`self.Flaque`))
  ;[1 0.8608 0] SPAWN & DESPAWN FLAQUE (played in BP_BIGZlagBall)
  (bind (_direction _dissolvevalue2) (`Timeline|Timeline_Despawn`)
    (:`Update`
      (`MeshComponent.SetScalarParameterValueOnMaterials` _flaque "Dissolve" _dissolvevalue2))
    (:`Finished`
      (`SceneComponent.SetVisibility` _flaque false false))))

(event `Descaling`
  ;[1 1 1] Scaling flaque random delay
  (`KismetSystemLibrary.Delay` (`KismetMathLibrary.RandomFloatInRange` 1.0 6.0))
  (bind (_direction _multiplyscale) (`Timeline|Timeline_Descaling` :!via `PlayFromStart`)
    (:`Update`
      (set `self.ScaleCurent` (/ (* (`self.ScaleBase`) 1.5) _multiplyscale))
      (`SceneComponent.SetWorldScale3D` (`self.Flaque`) (`self.ScaleCurent`)))
    (:`Finished`
      (`self.Scaling`))))

(event `AddJauge`
  (`|SpawnActorFromClass` "/Game/VFX/Blueprint/BP_Zlag_test_2.BP_Zlag_test_2_C" (`self.GetTransform`) "Undefined" "OverrideRootScale" null null)
  (if (>= (`/Game/Characters/SeaWatcher/BP_SeaWatcher.Jauge` (`self.As BP Sea Watcher`)) 100.0)
    (`KismetSystemLibrary.K2_ClearAndInvalidateTimerHandle` (`self.NewVar`))))

(event `self.Box.OnComponentBeginOverlap`
  (params (OverlappedComponent :type "PrimitiveComponent Object Reference") (OtherActor :type "Actor Object Reference") (OtherComp :type "PrimitiveComponent Object Reference") (OtherBodyIndex :type Integer) (bFromSweep :type Boolean) (SweepResult :type "HitResult Structure (by ref)"))
  (bind _asbp_sea_watcher (cast `/Game/Characters/SeaWatcher/BP_SeaWatcher` OtherActor))
  (set `self.As BP Sea Watcher` _asbp_sea_watcher)
  (bind _returnvalue (`KismetSystemLibrary.K2_SetTimerDelegate` (delegate `AddJauge`) 0.5 true))
  (set `self.NewVar` _returnvalue))

(event `ResetDeath`
  (if (`self.isSpawner`)
    (if (not (`self.BZBSpawned`))
      (`KismetSystemLibrary.Delay` 5.0)
      (`KismetSystemLibrary.PrintString` "SpawnBZB")
      (`|SpawnActorFromClass` "/Game/VFX/Blueprint/BP_BIGZlagBall.BP_BIGZlagBall_C" (`KismetMathLibrary.MakeTransform` (`SceneComponent.K2_GetComponentLocation` (`self.SphereCollision_Ramassage`))) "Undefined" "OverrideRootScale" null null)
      (`SceneComponent.SetVisibility` (`self.Flaque`) true false)
      (set `self.BZBSpawned` true))))

(event `self.Box.OnComponentEndOverlap`
  (params (OverlappedComponent :type "PrimitiveComponent Object Reference") (OtherActor :type "Actor Object Reference") (OtherComp :type "PrimitiveComponent Object Reference") (OtherBodyIndex :type Integer))
  (cast `/Game/Characters/SeaWatcher/BP_SeaWatcher` OtherActor)
  (set `self.As BP Sea Watcher` null)
  (`KismetSystemLibrary.K2_ClearAndInvalidateTimerHandle` (`self.NewVar`)))

(fn `UserConstructionScript`
  (if (not (`self.isSpawner`))
    (`ActorComponent.K2_DestroyComponent` (`self.Box`))))