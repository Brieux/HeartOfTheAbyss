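; BP_Fumerol_002 is a fumarole VFX actor that emits bubbles while a BP_SeaWatcher is nearby.
; A TriggerActivation sphere activates the NSFumeroleBubble effect on begin overlap with that actor and deactivates it on end overlap.
; The TriggerRadius variable sets the sphere's size in the construction script and again on BeginPlay.
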(event `self.ReceiveBeginPlay`
  (`SphereComponent.SetSphereRadius` (`self.Trigger Activation`) (`self.TriggerRadius`) true))

(event `self.Trigger Activation.OnComponentBeginOverlap`
  (params (OverlappedComponent :type "PrimitiveComponent Object Reference") (OtherActor :type "Actor Object Reference") (OtherComp :type "PrimitiveComponent Object Reference") (OtherBodyIndex :type Integer) (bFromSweep :type Boolean) (SweepResult :type "HitResult Structure (by ref)"))
  (cast `/Game/Characters/SeaWatcher/BP_SeaWatcher` OtherActor)
  (`ActorComponent.Activate` (`self.NS Fumerole Bubble`) false))

(event `self.Trigger Activation.OnComponentEndOverlap`
  (params (OverlappedComponent :type "PrimitiveComponent Object Reference") (OtherActor :type "Actor Object Reference") (OtherComp :type "PrimitiveComponent Object Reference") (OtherBodyIndex :type Integer))
  (cast `/Game/Characters/SeaWatcher/BP_SeaWatcher` OtherActor)
  (`ActorComponent.Deactivate` (`self.NS Fumerole Bubble`)))

(fn `UserConstructionScript`
  (`SphereComponent.SetSphereRadius` (`self.Trigger Activation`) (`self.TriggerRadius`) true))