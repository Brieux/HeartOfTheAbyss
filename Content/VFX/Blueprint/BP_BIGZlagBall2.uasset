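; BP_BIGZlagBall2 is a collectible big Zlag ball that appears when BP_SeaWatcher approaches and is picked up on contact.
; The spawn collision sphere triggers a Niagara spawn effect, then after a delay reveals the ball with emission particles and a timeline-driven vertical bounce.
; The pickup sphere spawns a BP_Zlag_test_3 and a collect sound, then shrinks the ball by timeline before destroying it.
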(event `self.ReceiveBeginPlay`
  (bind _returnvalue (`GameplayStatics.GetActorOfClass` "/Game/VFX/Blueprint/BP_ChuteZlag.BP_ChuteZlag_C"))
  (set `self.BP Chute Zlag Ref` _returnvalue))

(event `Bounce`
  (bind _zoffset (`self.ZOffset`))
  (bind _sphere (`self.Sphere`))
  (bind (_relativelocation_x _relativelocation_y) (`KismetMathLibrary.BreakVector` (`SceneComponent.RelativeLocation` _sphere)))
  (bind (_relativelocation_x_2 _relativelocation_y_2 _relativelocation_z) (`KismetMathLibrary.BreakVector` (`SceneComponent.RelativeLocation` (`self.Sphere`))))
  ;[1 1 0] BOUNCE EFFECT
  (set `self.ZOffset` _relativelocation_z)
  (bind (_direction _newtrack_0) (`Timeline|Timeline_0`)
    (:`Update`
      (`SceneComponent.K2_SetRelativeLocation` _sphere (`KismetMathLibrary.VLerp` (`KismetMathLibrary.MakeVector` _relativelocation_x _relativelocation_y _zoffset) (`KismetMathLibrary.MakeVector` _relativelocation_x _relativelocation_y (+ _zoffset (* _newtrack_0 10.0))) _newtrack_0) false false))))

(event `self.SphereCollison_Spawn.OnComponentBeginOverlap`
  (params (OverlappedComponent :type "PrimitiveComponent Object Reference") (OtherActor :type "Actor Object Reference") (OtherComp :type "PrimitiveComponent Object Reference") (OtherBodyIndex :type Integer) (bFromSweep :type Boolean) (SweepResult :type "HitResult Structure (by ref)"))
  (cast `/Game/Characters/SeaWatcher/BP_SeaWatcher` OtherActor)
  (`self.SpawnPosition`))

(event `self.SphereCollision_Ramassage.OnComponentBeginOverlap`
  (params (OverlappedComponent :type "PrimitiveComponent Object Reference") (OtherActor :type "Actor Object Reference") (OtherComp :type "PrimitiveComponent Object Reference") (OtherBodyIndex :type Integer) (bFromSweep :type Boolean) (SweepResult :type "HitResult Structure (by ref)"))
  (bind _sphere (`self.Sphere`))
  ;[0 0 1] OVERLAP PLAYER
  (bind _asbp_sea_watcher (cast `/Game/Characters/SeaWatcher/BP_SeaWatcher` OtherActor))
  (`|SpawnActorFromClass` "/Game/VFX/Blueprint/BP_Zlag_test_3.BP_Zlag_test_3_C" (`self.GetTransform`) "AlwaysSpawn" "OverrideRootScale" null null)
  (`GameplayStatics.SpawnSoundAtLocation` "/Game/Sound/Characters/MC/Cues/Cue_Collec_Heal_Pop.Cue_Collec_Heal_Pop" (`SceneComponent.K2_GetComponentLocation` (`/Game/Characters/SeaWatcher/BP_SeaWatcher.SpringArm` _asbp_sea_watcher)) (struct) 1.0 1.0 0.0 null null)
  (bind (_direction _scalecoef) (`Timeline|Timeline_Descale`)
    (:`Update`
      (`SceneComponent.SetWorldScale3D` _sphere (* (`SceneComponent.K2_GetComponentScale` _sphere) _scalecoef)))
    (:`Finished`
      (`ActorComponent.Deactivate` (`self.NS Emission`))
      (`self.K2_DestroyActor`))))

(event `SpawnPosition`
  ;[1 1 1] SpawnZlagBall
  (`ActorComponent.Activate` (`self.NS Spawn`) false)
  (`KismetSystemLibrary.Delay` 2.0)
  (`ActorComponent.Activate` (`self.NS Emission`) false)
  (`SceneComponent.SetVisibility` (`self.Sphere`) true false)
  (`self.Bounce`))

(fn `UserConstructionScript`)