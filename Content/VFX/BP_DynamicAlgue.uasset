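; BP_DynamicAlgue is a Niagara-driven algae effect that reacts to the player character's position.
; The construction script pushes the offset, density and dispersion settings to Niagara and picks the normal or "Zlag" algae material from IsZlaged.
; Each tick converts the player mesh's world location into the actor's local space and feeds its X and Y to the "Attr" vector parameter.
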(event `self.ReceiveBeginPlay`)

(event `self.ReceiveTick`
  (params (DeltaSeconds :type "Float (single-precision)"))
  (bind (_returnvalue_x _returnvalue_y) (`KismetMathLibrary.BreakVector` (`KismetMathLibrary.InverseTransformLocation` (`self.GetTransform`) (`SceneComponent.K2_GetComponentLocation` (`Character.Mesh` (`GameplayStatics.GetPlayerCharacter` 0))))))
  (`FXSystemComponent.SetVectorParameter` (`self.Niagara`) "Attr" (`KismetMathLibrary.MakeVector` _returnvalue_x _returnvalue_y)))

(fn `UserConstructionScript`
  (`FXSystemComponent.SetFloatParameter` (`self.Niagara`) "OffsetSpline" (`self.Offset`))
  (`FXSystemComponent.SetFloatParameter` (`self.Niagara`) "Density" (`self.Density`))
  (`FXSystemComponent.SetFloatParameter` (`self.Niagara`) "Dispertion" (`self.Disparité`))
  (`NiagaraComponent.SetVariableMaterial` (`self.Niagara`) "ZlagMat" (select `bool` (`self.isZlaged`) :`false` "/Game/Props/Mesh/Algues/Algue_Basic.Algue_Basic" :`true` "/Game/Props/Mesh/Algues/Algue_Basic_Zlag.Algue_Basic_Zlag" :!type "MaterialInterface Object Reference")))