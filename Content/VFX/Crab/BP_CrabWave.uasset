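; Crab shockwave attack that fires three staggered, growing Niagara rings with controller rumble, then resets the player's damage state and destroys itself.
; Each ring pairs outer and inner sphere colliders, whose overlap events flag whether BP_SeaWatcher is inside.
; A timer per ring later deals damage credited to the crab only if the player stands in the band between the two spheres.
; An older timeline-driven expanding wave remains but never runs.
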(event `Print`
  (bind _int (`self.Int`))
  (`KismetSystemLibrary.PrintString` (`KismetStringLibrary.Conv_IntToString` _int) true true (struct :`G` 0.66 :`B` 1.0 :`A` 1.0) 0.25)
  (set `self.Int` (+ _int 1))
  (`SceneComponent.SetRelativeScale3D` (`self.Sphere`) (`KismetMathLibrary.Conv_DoubleToVector` (/ (`KismetMathLibrary.Conv_IntToDouble` _int) (`self.NumberOfWave`)))))

(event `Wave`
  (bind _ns_wave (`self.NS_Wave`))
  (bind _ns_wave_2 (`self.NS_Wave_2`))
  (bind _ns_wave_3 (`self.NS_Wave_3`))
  (`ActorComponent.Activate` (`self.NS_Wave`) true)
  (`PlayerController.K2_ClientPlayForceFeedback` (`GameplayStatics.GetPlayerController` 0) "/Game/GeneralSettings/FFE_NS_Wave.FFE_NS_Wave" "None" false false false)
  (`KismetSystemLibrary.K2_SetTimerDelegate` (delegate `CustomEvent_0`) 7.0)
  (`FXSystemComponent.SetFloatParameter` _ns_wave "RingSize" 800.0)
  (`FXSystemComponent.SetFloatParameter` _ns_wave "RingPrevizSize" 2600.0)
  (`SphereComponent.SetSphereRadius` (`self.Sphere`) 1000.0 true)
  (`SphereComponent.SetSphereRadius` (`self.Sphere_int`) 600.0 true)
  (`KismetSystemLibrary.K2_SetTimerDelegate` (delegate `ColliderSphere`) 2.25)
  (`KismetSystemLibrary.Delay` 1.0)
  (`ActorComponent.Activate` _ns_wave_2 true)
  (`FXSystemComponent.SetFloatParameter` _ns_wave_2 "RingPrevizSize" 5100.0)
  (`FXSystemComponent.SetFloatParameter` _ns_wave_2 "RingSize" 2000.0)
  (`SphereComponent.SetSphereRadius` (`self.Sphere2`) 2200.0 true)
  (`SphereComponent.SetSphereRadius` (`self.Sphere2_int`) 1800.0 true)
  (`KismetSystemLibrary.K2_SetTimerDelegate` (delegate `CollisionSphere_2`) 2.25)
  (`KismetSystemLibrary.Delay` 1.0)
  (`ActorComponent.Activate` _ns_wave_3 true)
  (`FXSystemComponent.SetFloatParameter` _ns_wave_3 "RingPrevizSize" 8000.0)
  (`FXSystemComponent.SetFloatParameter` _ns_wave_3 "RingSize" 3200.0)
  (`SphereComponent.SetSphereRadius` (`self.Sphere3`) 3400.0 true)
  (`SphereComponent.SetSphereRadius` (`self.Sphere3_int`) 3000.0 true)
  (`KismetSystemLibrary.K2_SetTimerDelegate` (delegate `CollisionSphere3`) 2.25)
  (`KismetSystemLibrary.Delay` 4.0)
  (`ActorComponent.Deactivate` (`self.NS_Wave`))
  (`ActorComponent.Deactivate` (`self.NS_Wave_2`))
  (`ActorComponent.Deactivate` (`self.NS_Wave_3`))
  (bind _asbp_sea_watcher (cast `/Game/Characters/SeaWatcher/BP_SeaWatcher` (`GameplayStatics.GetPlayerCharacter` 0)))
  (`/Game/Characters/SeaWatcher/BP_SeaWatcher.ResetDammage` _asbp_sea_watcher)
  (`self.K2_DestroyActor`)
  (`KismetSystemLibrary.Delay` 1.0))

(event `ColliderSphere`
  (bind _asbp_sea_watcher (cast `/Game/Characters/SeaWatcher/BP_SeaWatcher` (`GameplayStatics.GetPlayerCharacter` 0)))
  (if (and (`self.CollideSphere1`) (not (`self.CollideSphere1_int`)))
    (`KismetSystemLibrary.PrintString` "Collision 1")
    (`GameplayStatics.ApplyDamage` _asbp_sea_watcher 20.0 null (`Pawn.GetController` (`self.crabeRef`)))))

(event `CustomEvent_0`
  (`PlayerController.ClientStopForceFeedback` (`GameplayStatics.GetPlayerController` 0) "/Game/GeneralSettings/FFE_NS_Wave.FFE_NS_Wave" "None"))

(event `CollisionSphere_2`
  (bind _asbp_sea_watcher (cast `/Game/Characters/SeaWatcher/BP_SeaWatcher` (`GameplayStatics.GetPlayerCharacter` 0)))
  (if (and (not (`self.CollideSphere2_int`)) (`self.CollideSphere2`))
    (`KismetSystemLibrary.PrintString` "Collision 2")
    (`KismetSystemLibrary.PrintString` "DEGATS VAGUE 2")
    (`GameplayStatics.ApplyDamage` _asbp_sea_watcher 20.0 null (`Pawn.GetController` (`self.crabeRef`)))))

(event `CollisionSphere3`
  (bind _asbp_sea_watcher (cast `/Game/Characters/SeaWatcher/BP_SeaWatcher` (`GameplayStatics.GetPlayerCharacter` 0)))
  (if (and (not (`self.CollideSphere3_int`)) (`self.CollideSphere3`))
    (`KismetSystemLibrary.PrintString` "Collision 3")
    (`GameplayStatics.ApplyDamage` _asbp_sea_watcher 20.0 null (`Pawn.GetController` (`self.crabeRef`)))))

(event `self.Sphere.OnComponentBeginOverlap`
  (params (OverlappedComponent :type "PrimitiveComponent Object Reference") (OtherActor :type "Actor Object Reference") (OtherComp :type "PrimitiveComponent Object Reference") (OtherBodyIndex :type Integer) (bFromSweep :type Boolean) (SweepResult :type "HitResult Structure (by ref)"))
  (cast `/Game/Characters/SeaWatcher/BP_SeaWatcher` OtherActor)
  (set `self.CollideSphere1` true))

(event `self.Sphere2.OnComponentBeginOverlap`
  (params (OverlappedComponent :type "PrimitiveComponent Object Reference") (OtherActor :type "Actor Object Reference") (OtherComp :type "PrimitiveComponent Object Reference") (OtherBodyIndex :type Integer) (bFromSweep :type Boolean) (SweepResult :type "HitResult Structure (by ref)"))
  (cast `/Game/Characters/SeaWatcher/BP_SeaWatcher` OtherActor)
  (set `self.CollideSphere2` true))

(event `self.Sphere3.OnComponentBeginOverlap`
  (params (OverlappedComponent :type "PrimitiveComponent Object Reference") (OtherActor :type "Actor Object Reference") (OtherComp :type "PrimitiveComponent Object Reference") (OtherBodyIndex :type Integer) (bFromSweep :type Boolean) (SweepResult :type "HitResult Structure (by ref)"))
  (cast `/Game/Characters/SeaWatcher/BP_SeaWatcher` OtherActor)
  (set `self.CollideSphere3` true))

(event `self.Sphere.OnComponentEndOverlap`
  (params (OverlappedComponent :type "PrimitiveComponent Object Reference") (OtherActor :type "Actor Object Reference") (OtherComp :type "PrimitiveComponent Object Reference") (OtherBodyIndex :type Integer))
  (cast `/Game/Characters/SeaWatcher/BP_SeaWatcher` OtherActor)
  (set `self.CollideSphere1` false))

(event `self.Sphere2.OnComponentEndOverlap`
  (params (OverlappedComponent :type "PrimitiveComponent Object Reference") (OtherActor :type "Actor Object Reference") (OtherComp :type "PrimitiveComponent Object Reference") (OtherBodyIndex :type Integer))
  (cast `/Game/Characters/SeaWatcher/BP_SeaWatcher` OtherActor)
  (set `self.CollideSphere2` false))

(event `self.Sphere3.OnComponentEndOverlap`
  (params (OverlappedComponent :type "PrimitiveComponent Object Reference") (OtherActor :type "Actor Object Reference") (OtherComp :type "PrimitiveComponent Object Reference") (OtherBodyIndex :type Integer))
  (cast `/Game/Characters/SeaWatcher/BP_SeaWatcher` OtherActor)
  (set `self.CollideSphere3` false))

(event `self.Sphere_int.OnComponentBeginOverlap`
  (params (OverlappedComponent :type "PrimitiveComponent Object Reference") (OtherActor :type "Actor Object Reference") (OtherComp :type "PrimitiveComponent Object Reference") (OtherBodyIndex :type Integer) (bFromSweep :type Boolean) (SweepResult :type "HitResult Structure (by ref)"))
  (cast `/Game/Characters/SeaWatcher/BP_SeaWatcher` OtherActor)
  (set `self.CollideSphere1_int` true))

(event `self.Sphere_int.OnComponentEndOverlap`
  (params (OverlappedComponent :type "PrimitiveComponent Object Reference") (OtherActor :type "Actor Object Reference") (OtherComp :type "PrimitiveComponent Object Reference") (OtherBodyIndex :type Integer))
  (cast `/Game/Characters/SeaWatcher/BP_SeaWatcher` OtherActor)
  (set `self.CollideSphere1_int` false))

(event `self.Sphere2_int.OnComponentBeginOverlap`
  (params (OverlappedComponent :type "PrimitiveComponent Object Reference") (OtherActor :type "Actor Object Reference") (OtherComp :type "PrimitiveComponent Object Reference") (OtherBodyIndex :type Integer) (bFromSweep :type Boolean) (SweepResult :type "HitResult Structure (by ref)"))
  (cast `/Game/Characters/SeaWatcher/BP_SeaWatcher` OtherActor)
  (set `self.CollideSphere2_int` true))

(event `self.Sphere2_int.OnComponentEndOverlap`
  (params (OverlappedComponent :type "PrimitiveComponent Object Reference") (OtherActor :type "Actor Object Reference") (OtherComp :type "PrimitiveComponent Object Reference") (OtherBodyIndex :type Integer))
  (cast `/Game/Characters/SeaWatcher/BP_SeaWatcher` OtherActor)
  (set `self.CollideSphere2_int` false))

(event `self.Sphere3_int.OnComponentBeginOverlap`
  (params (OverlappedComponent :type "PrimitiveComponent Object Reference") (OtherActor :type "Actor Object Reference") (OtherComp :type "PrimitiveComponent Object Reference") (OtherBodyIndex :type Integer) (bFromSweep :type Boolean) (SweepResult :type "HitResult Structure (by ref)"))
  (cast `/Game/Characters/SeaWatcher/BP_SeaWatcher` OtherActor)
  (set `self.CollideSphere3_int` true))

(event `self.Sphere3_int.OnComponentEndOverlap`
  (params (OverlappedComponent :type "PrimitiveComponent Object Reference") (OtherActor :type "Actor Object Reference") (OtherComp :type "PrimitiveComponent Object Reference") (OtherBodyIndex :type Integer))
  (cast `/Game/Characters/SeaWatcher/BP_SeaWatcher` OtherActor)
  (set `self.CollideSphere3_int` false))

(fn `UserConstructionScript`)