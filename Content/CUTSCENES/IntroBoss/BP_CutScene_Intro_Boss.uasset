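; Trigger-box actor that starts the boss intro cutscene when BP_SeaWatcher overlaps it.
; Overlap ducks audio and plays the cinematic sound, then a DoOnce hides the interface and SeaWatcher and plays the Intro_Boss Level Sequence.
; A timer matching the sequence length teleports SeaWatcher to a hardcoded location, restores visibility and pops the sound mix.
; Audio runs before the DoOnce, and the input-locking nodes are disconnected.
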(event `self.ReceiveBeginPlay`)

(event `self.Box.OnComponentBeginOverlap`
  (params (OverlappedComponent :type "PrimitiveComponent Object Reference") (OtherActor :type "Actor Object Reference") (OtherComp :type "PrimitiveComponent Object Reference") (OtherBodyIndex :type Integer) (bFromSweep :type Boolean) (SweepResult :type "HitResult Structure (by ref)"))
  (bind _asbp_sea_watcher (cast `/Game/Characters/SeaWatcher/BP_SeaWatcher` OtherActor))
  (set `self.As BP Sea Watcher` _asbp_sea_watcher)
  (bind _output_get (set `self.As BP Player Controller` (cast `/Game/GeneralSettings/BP_PlayerController` (`GameplayStatics.GetPlayerController` 0) :!pure true)))
  (`GameplayStatics.PushSoundMixModifier` "/Game/Sound/Mix/DuckCinematic.DuckCinematic")
  (`GameplayStatics.PlaySound2D` "/Game/Sound/Cutscene/DebutPhase01/HOTA_Cinematic_IntroBoss_Cue.HOTA_Cinematic_IntroBoss_Cue" 1.0 1.0 0.0 null null)
  (`/Engine/EditorBlueprintResources/StandardMacros.DoOnce` false
    (:`Completed`
      (`Widget.SetVisibility` (`/Game/GeneralSettings/BP_PlayerController.Interface` _output_get) "Hidden")
      (`self.SetActorHiddenInGame` (`self.As BP Sea Watcher`) true)
      (bind (_outactor _returnvalue) (`LevelSequencePlayer.CreateLevelSequencePlayer` "/Game/CUTSCENES/IntroBoss/Intro_Boss.Intro_Boss"))
      (`MovieSceneSequencePlayer.Play` _returnvalue)
      (`KismetSystemLibrary.K2_SetTimerDelegate` (delegate `CustomEvent`) (`TimeManagementBlueprintLibrary.Conv_QualifiedFrameTimeToSeconds` (`MovieSceneSequencePlayer.GetDuration` _returnvalue))))))

(event `CustomEvent`
  (bind _as_bp_sea_watcher (`self.As BP Sea Watcher`))
  (`self.K2_SetActorLocation` _as_bp_sea_watcher (-3254.170323 -87.864618 500.0) false true)
  (`self.SetActorHiddenInGame` _as_bp_sea_watcher false)
  (`Widget.SetVisibility` (`/Game/GeneralSettings/BP_PlayerController.Interface` (`self.As BP Player Controller`)) "Visible")
  (`GameplayStatics.PopSoundMixModifier` "/Game/Sound/Mix/DuckCinematic.DuckCinematic"))

(fn `UserConstructionScript`)