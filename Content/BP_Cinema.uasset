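; BP_Cinema is an automatic cinematic camera that follows the player with a SceneCaptureComponent2D.
; Each tick, the capture eases toward the nearest point to the player on two splines and smoothly turns to face them.
; Its FOV narrows as its distance from the player grows, giving a zoom effect.
; IsActiv gates the system: when false, construction destroys the capture component and BeginPlay disables tick.
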(event `self.ReceiveBeginPlay`
  (`self.SetActorTickEnabled` (`self.isActiv?`)))

(event `self.ReceiveTick`
  (params (DeltaSeconds :type "Float (single-precision)"))
  (bind _scenecapturecomponent2d (`self.SceneCaptureComponent2D`))
  (bind _scenecapturecomponent2d_2 (`self.SceneCaptureComponent2D`))
  (bind _returnvalue (`self.K2_GetActorLocation` (`GameplayStatics.GetPlayerCharacter` 0)))
  (bind _returnvalue_2 (`self.K2_GetActorLocation` (`GameplayStatics.GetPlayerCharacter` 0)))
  (bind _returnvalue_3 (`SplineComponent.FindLocationClosestToWorldLocation` (`self.Spline`) _returnvalue_2 "World"))
  (bind _returnvalue_4 (`SplineComponent.FindLocationClosestToWorldLocation` (`self.Spline1`) _returnvalue "World"))
  (`/Engine/EditorBlueprintResources/StandardMacros.IsValid` (`GameplayStatics.GetPlayerCharacter` 0)
    (:`Is Valid`
      (`SceneComponent.K2_SetWorldLocation` _scenecapturecomponent2d (`KismetMathLibrary.VInterpTo` (`SceneComponent.K2_GetComponentLocation` _scenecapturecomponent2d) (select `bool` (> (`KismetMathLibrary.Vector_Distance` _returnvalue_4 _returnvalue) (`KismetMathLibrary.Vector_Distance` _returnvalue_3 _returnvalue_2)) :`false` _returnvalue_4 :`true` _returnvalue_3) DeltaSeconds 1.0) false false)
      (`SceneComponent.K2_SetWorldRotation` (`self.SceneCaptureComponent2D`) (`KismetMathLibrary.RInterpTo` (`SceneComponent.K2_GetComponentRotation` _scenecapturecomponent2d_2) (`KismetMathLibrary.FindLookAtRotation` (`SceneComponent.K2_GetComponentLocation` _scenecapturecomponent2d_2) (`self.K2_GetActorLocation` (`GameplayStatics.GetPlayerCharacter` 0))) DeltaSeconds 1.5) false false)
      (set `SceneCaptureComponent2D.FOVAngle` (`KismetMathLibrary.Lerp` 120.0 75.0 (`KismetMathLibrary.MapRangeClamped` (`KismetMathLibrary.Vector_Distance` (`self.K2_GetActorLocation` (`GameplayStatics.GetPlayerCharacter` 0)) (`SceneComponent.K2_GetComponentLocation` (`self.SceneCaptureComponent2D`))) 0.0 4000.0 0.0 1.0)) (`self.SceneCaptureComponent2D`)))))

(fn `UserConstructionScript`
  (if (not (`self.isActiv?`))
    (`ActorComponent.K2_DestroyComponent` (`self.SceneCaptureComponent2D`))))