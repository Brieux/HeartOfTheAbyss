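; BP_Morve is a configurable hanging snot strand built from cable components, with an optional branching second strand.
; The construction script positions the cable and filament components from location variables and applies shared length, gravity, width and material.
; When SecondCable is set, it adds a cable at a random particle of the first and moves SceneEnd2 to NextCableEnd.
; Tick is empty; logic to make the branch follow that particle is unconnected.
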(event `self.ReceiveTick`
  (params (DeltaSeconds :type "Float (single-precision)")))

(fn `UserConstructionScript`
  (bind _secondcablerender (`self.SecondCableRender`))
  (bind _cable (`self.Cable`))
  (bind (_outitem _outindex) (`KismetArrayLibrary.Array_Random` (`CableComponent.GetCableParticleLocations` _cable)))
  (`SceneComponent.K2_SetRelativeLocation` (`self.Cable`) (`self.Narine`) false false)
  (`SceneComponent.K2_SetRelativeLocation` (`self.ZlagFilament2`) (`self.Narine`) false false)
  (`SceneComponent.K2_SetRelativeLocation` (`self.ZlagFilament3`) (`self.Caquine`) false false)
  (set `CableComponent.CableLength` (`self.Cable Length`) _cable)
  (set `CableComponent.CableGravityScale` (`self.Cable Gravity Scale`) _cable)
  (set `CableComponent.CableWidth` (`self.Cable Width`) _cable)
  (set `CableComponent.TileMaterial` (`self.Tile Material`) _cable)
  (if (`self.SecondCable`)
    (bind _output_get (set `self.NextCableDebut` (- _outitem (`self.K2_GetActorLocation`))))
    (set `self.Index` _outindex)
    (bind _returnvalue (`AddComponent|NODE_AddCableComponent-0` :`RelativeTransform` (`KismetMathLibrary.MakeTransform` _output_get)))
    (set `self.SecondCableRender` _returnvalue)
    (`SceneComponent.K2_SetRelativeLocation` (`self.SceneEnd2`) (`self.NextCableEnd`) false false)
    (set `CableComponent.CableLength` (`self.Cable Length`) _secondcablerender)
    (set `CableComponent.CableGravityScale` (`self.Cable Gravity Scale`) _secondcablerender)
    (set `CableComponent.CableWidth` (`self.Cable Width`) _secondcablerender)
    (set `CableComponent.TileMaterial` (`self.Tile Material`) _secondcablerender)))