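; Two-box level trigger meant to swap two World Partition data layers according to the direction in which BP_SeaWatcher passes through.
; ExitA and ExitB set opposite Activated/Unloaded runtime states on the load and unload layers.
; A StateEntry state machine tracks entry, overlap of both boxes and exit to choose the swap.
; That logic is disconnected: all four BOXA and BOXB overlap events are empty, so overlaps currently trigger nothing.
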(event `self.BOXA.OnComponentBeginOverlap`
  (params (OverlappedComponent :type "PrimitiveComponent Object Reference") (OtherActor :type "Actor Object Reference") (OtherComp :type "PrimitiveComponent Object Reference") (OtherBodyIndex :type Integer) (bFromSweep :type Boolean) (SweepResult :type "HitResult Structure (by ref)")))

(event `ExitA`
  (`DataLayerSubsystem.SetDataLayerRuntimeState` (subsystem `DataLayerSubsystem`) (`self.In Data Layer to Load`) "Unloaded" false)
  (`DataLayerSubsystem.SetDataLayerRuntimeState` (subsystem `DataLayerSubsystem`) (`self.In Data Layer to Unload`) "Activated" false))

(event `self.BOXA.OnComponentEndOverlap`
  (params (OverlappedComponent :type "PrimitiveComponent Object Reference") (OtherActor :type "Actor Object Reference") (OtherComp :type "PrimitiveComponent Object Reference") (OtherBodyIndex :type Integer)))

(event `ExitB`
  (`DataLayerSubsystem.SetDataLayerRuntimeState` (subsystem `DataLayerSubsystem`) (`self.In Data Layer to Load`) "Activated" false)
  (`DataLayerSubsystem.SetDataLayerRuntimeState` (subsystem `DataLayerSubsystem`) (`self.In Data Layer to Unload`) "Unloaded" false))

(event `self.BOXB.OnComponentBeginOverlap`
  (params (OverlappedComponent :type "PrimitiveComponent Object Reference") (OtherActor :type "Actor Object Reference") (OtherComp :type "PrimitiveComponent Object Reference") (OtherBodyIndex :type Integer) (bFromSweep :type Boolean) (SweepResult :type "HitResult Structure (by ref)")))

(event `self.BOXB.OnComponentEndOverlap`
  (params (OverlappedComponent :type "PrimitiveComponent Object Reference") (OtherActor :type "Actor Object Reference") (OtherComp :type "PrimitiveComponent Object Reference") (OtherBodyIndex :type Integer)))

(fn `UserConstructionScript`)