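; Player controller that owns the game's UI and handles pausing and the player's death.
; On BeginPlay it creates a UI_Interface widget and adds it to the viewport.
; The pause input toggles game pause, mouse cursor, input mode and the visible panel (in-game or pause).
; The Death event pauses the game, shows the cursor and clears the NotLose flag without switching UI panels itself.
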(event `self.ReceiveBeginPlay`
  (bind _returnvalue (`|CreateWidget` "/Game/UI/UI_Interface.UI_Interface_C"))
  (bind _output_get (set `self.Interface` _returnvalue))
  (`UserWidget.AddToViewport` _output_get 1))

(event `EnhancedInput|/Game/GeneralSettings/Input/IA_OpenPauseScreen`
  (params (ActionValue :type Boolean) (ElapsedSeconds :type "Float (double-precision)") (TriggeredSeconds :type "Float (double-precision)") (InputAction :type "InputAction Object Reference" :default "/Game/GeneralSettings/Input/IA_OpenPauseScreen.IA_OpenPauseScreen"))
  (bind _interface (`self.Interface`))
  (bind _interface_2 (`self.Interface`))
  (:`Triggered`
    (if (`GameplayStatics.IsGamePaused`)
      (set `self.bShowMouseCursor` false)
      (`WidgetBlueprintLibrary.SetInputMode_GameOnly` self)
      (`GameplayStatics.SetGamePaused` false)
      (`/Game/UI/UI_Interface.HideAll` _interface)
      (`Widget.SetVisibility` (`/Game/UI/UI_Interface.UI_InGame` _interface) "Visible")
      (else
        (set `self.bShowMouseCursor` true)
        (`WidgetBlueprintLibrary.SetInputMode_GameAndUIEx` self (`self.Interface`) "DoNotLock" false)
        (`/Game/UI/UI_Interface.HideAll` _interface_2)
        (`GameplayStatics.SetGamePaused` true)
        (`Widget.SetVisibility` (`/Game/UI/UI_Interface.UI_Pause` _interface_2) "Visible")
        (set `UserWidget.bIsFocusable` true _interface_2)))))

(event `Death`
  (set `self.bShowMouseCursor` true)
  (`GameplayStatics.SetGamePaused` true)
  (set `self.NotLose` false))

(fn `UserConstructionScript`)