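; Two-box trigger actor that switches the BP_SeaWatcher player's RemoveDashForPont flag according to which side they leave by, apparently disabling dash on one side.
; Overlap events on BOXA and BOXB drive a StateEntry enum that tracks whether the player is in A, B or both.
; A final exit through A calls GoA to clear the flag, while one through B calls GoB to set it.
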(event `self.BOXA.OnComponentBeginOverlap`
  (params (OverlappedComponent :type "PrimitiveComponent Object Reference") (OtherActor :type "Actor Object Reference") (OtherComp :type "PrimitiveComponent Object Reference") (OtherBodyIndex :type Integer) (bFromSweep :type Boolean) (SweepResult :type "HitResult Structure (by ref)"))
  (cast `/Game/Characters/SeaWatcher/BP_SeaWatcher` OtherActor)
  (switch `/Game/Levels/Enum_EntryType` (`self.StateEntry`)
    (:`NewEnumerator0`
      (set `self.StateEntry` "NewEnumerator1" :!label _label))
    (:`NewEnumerator2`
      (goto _label))
    (:`NewEnumerator3`
      (set `self.StateEntry` "NewEnumerator5"))
    (:`NewEnumerator4`
      (goto _label))))

(event `GoA`
  (params (PlayerRef :type "/Game/Characters/SeaWatcher/BP_SeaWatcher Object Reference"))
  (set `/Game/Characters/SeaWatcher/BP_SeaWatcher.RemoveDashForPont` false PlayerRef))

(event `self.BOXA.OnComponentEndOverlap`
  (params (OverlappedComponent :type "PrimitiveComponent Object Reference") (OtherActor :type "Actor Object Reference") (OtherComp :type "PrimitiveComponent Object Reference") (OtherBodyIndex :type Integer))
  (bind _asbp_sea_watcher (cast `/Game/Characters/SeaWatcher/BP_SeaWatcher` OtherActor))
  (switch `/Game/Levels/Enum_EntryType` (`self.StateEntry`)
    (:`NewEnumerator0`
      (set `self.StateEntry` "NewEnumerator2" :!label _label_2)
      (`self.GoA` _asbp_sea_watcher))
    (:`NewEnumerator1`
      (goto _label_2))
    (:`NewEnumerator5`
      (set `self.StateEntry` "NewEnumerator3"))))

(event `GoB`
  (params (PlayerRef :type "/Game/Characters/SeaWatcher/BP_SeaWatcher Object Reference"))
  (set `/Game/Characters/SeaWatcher/BP_SeaWatcher.RemoveDashForPont` true PlayerRef))

(event `self.BOXB.OnComponentBeginOverlap`
  (params (OverlappedComponent :type "PrimitiveComponent Object Reference") (OtherActor :type "Actor Object Reference") (OtherComp :type "PrimitiveComponent Object Reference") (OtherBodyIndex :type Integer) (bFromSweep :type Boolean) (SweepResult :type "HitResult Structure (by ref)"))
  (cast `/Game/Characters/SeaWatcher/BP_SeaWatcher` OtherActor)
  (switch `/Game/Levels/Enum_EntryType` (`self.StateEntry`)
    (:`NewEnumerator0`
      (set `self.StateEntry` "NewEnumerator3" :!label _label_3))
    (:`NewEnumerator1`
      (set `self.StateEntry` "NewEnumerator5"))
    (:`NewEnumerator2`
      (goto _label_3))
    (:`NewEnumerator4`
      (goto _label_3))))

(event `self.BOXB.OnComponentEndOverlap`
  (params (OverlappedComponent :type "PrimitiveComponent Object Reference") (OtherActor :type "Actor Object Reference") (OtherComp :type "PrimitiveComponent Object Reference") (OtherBodyIndex :type Integer))
  (bind _asbp_sea_watcher (cast `/Game/Characters/SeaWatcher/BP_SeaWatcher` OtherActor))
  (switch `/Game/Levels/Enum_EntryType` (`self.StateEntry`)
    (:`NewEnumerator0`
      (set `self.StateEntry` "NewEnumerator2")
      (`self.GoA` _asbp_sea_watcher))
    (:`NewEnumerator3`
      (set `self.StateEntry` "NewEnumerator4")
      (`self.GoB` _asbp_sea_watcher))
    (:`NewEnumerator5`
      (set `self.StateEntry` "NewEnumerator1"))))

(fn `ExitA`)

(fn `ExitB`)

(fn `UserConstructionScript`)