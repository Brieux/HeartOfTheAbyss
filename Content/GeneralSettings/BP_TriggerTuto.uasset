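; Tutorial trigger volume that shows an attack tutorial on a linked Blob when the BP_SeaWatcher actor enters its box.
; On BeginPlay it attaches itself to the Blob, keeping its world transform.
; The first overlap activates the Blob's combo-attack or basic-attack widget, whichever it holds, and flags the Blob's UI as on.
; DesactiveTuto tells the cached SeaWatcher's UI to despawn the tutorial.
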(event `self.ReceiveBeginPlay`
  (`/Engine/EditorBlueprintResources/StandardMacros.IsValid` (`self.blob`)
    (:`Is Valid`
      (`self.K2_AttachToActor` (`self.blob`) "None" "KeepWorld" "KeepWorld" "KeepWorld"))))

(event `self.Box.OnComponentBeginOverlap`
  (params (OverlappedComponent :type "PrimitiveComponent Object Reference") (OtherActor :type "Actor Object Reference") (OtherComp :type "PrimitiveComponent Object Reference") (OtherBodyIndex :type Integer) (bFromSweep :type Boolean) (SweepResult :type "HitResult Structure (by ref)"))
  (bind _blob (`self.blob`))
  (bind _returnvalue (`WidgetComponent.GetWidget` (`/Game/BP_BlopV2.Widget` _blob)))
  (bind _asbp_sea_watcher (cast `/Game/Characters/SeaWatcher/BP_SeaWatcher` OtherActor))
  (set `self.As BP Sea Watcher` _asbp_sea_watcher)
  (`/Engine/EditorBlueprintResources/StandardMacros.DoOnce` false
    (:`Completed`
      (`/Engine/EditorBlueprintResources/StandardMacros.IsValid` _blob
        (:`Is Valid`
          (bind _asui_combo_attack (cast `/Game/UI/UI_ComboAttack` _returnvalue)
            (:`then`
              (`/Game/UI/UI_ComboAttack.ApplyPushButton` _asui_combo_attack true))
            (:`CastFailed`
              (bind _asui_tuto_basic_attack (cast `/Game/UI/UI_TutoBasicAttack` _returnvalue))
              (`/Game/UI/UI_TutoBasicAttack.Appear` _asui_tuto_basic_attack true)))
          (set `/Game/BP_BlopV2.UIIsOn` true (`self.blob`)))))))

(event `DesactiveTuto`
  (bind _as_bp_sea_watcher (`self.As BP Sea Watcher`))
  (`/Engine/EditorBlueprintResources/StandardMacros.IsValid` _as_bp_sea_watcher
    (:`Is Valid`
      (`/Game/UI/UI_Interface.EventDispawnTuto` (`/Game/Characters/SeaWatcher/BP_SeaWatcher.UI_Ref` _as_bp_sea_watcher) (`self.Duration`)))))

(fn `UserConstructionScript`)