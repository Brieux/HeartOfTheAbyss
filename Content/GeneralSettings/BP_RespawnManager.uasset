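; Respawn manager that returns the sea watcher player to one of four fixed locations chosen by PartToRespawn.
; Respawn restores health, potions, state flags and game input, unpauses, and pops the Stunned sound mix.
; Part 0 resets crab triggers, deactivates barriers and sets two data layer lists to Activated and Loaded.
; Other parts switch off the camera manager, reset cached crab bosses' stagger and call Reset.
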(event `self.ReceiveBeginPlay`
  (bind _asbp_sea_watcher (cast `/Game/Characters/SeaWatcher/BP_SeaWatcher` (`GameplayStatics.GetPlayerCharacter` 0)))
  (set `self.Player` _asbp_sea_watcher)
  (bind _asbp_player_controller (cast `/Game/GeneralSettings/BP_PlayerController` (`GameplayStatics.GetPlayerController` 0)))
  (set `self.Controller` _asbp_player_controller)
  (bind _outactors (`GameplayStatics.GetAllActorsOfClass` "/Game/Characters/Enemy/Boss/Crabe/BP_Crabe.BP_Crabe_C"))
  (set `self.CrabeBoss` _outactors))

(event `Respawn`
  (bind _player (`self.Player`))
  (bind _player_2 (`self.Player`))
  (`GameplayStatics.PopSoundMixModifier` "/Game/Sound/Mix/Stunned.Stunned")
  (`WidgetBlueprintLibrary.SetInputMode_GameOnly` (`self.Controller`))
  (`self.K2_SetActorLocation` _player (select `int` (`self.PartToRespawn`) :`0` (-31270.0 -21230.0 1639.96228) :`1` (-10260.0 -496.0 1132.0) :`2` (7285.337402 -542.211182 146.208313) :`3` (16779.994116 -19597.058328 -3237.39238) :!type "Vector Structure") false false)
  (`/Game/GeneralSettings/BP_PlayerController.Unpause` (`self.Controller`))
  (set `/Game/Characters/SeaWatcher/BP_SeaWatcher.EnergyRefill` true _player)
  (set `/Game/Characters/SeaWatcher/BP_SeaWatcher.CanMove` true _player_2)
  (set `/Game/Characters/SeaWatcher/BP_SeaWatcher.InClam?` false _player_2)
  (set `/Game/Characters/SeaWatcher/BP_SeaWatcher.GetHitBack` false _player_2)
  (set `/Game/Characters/SeaWatcher/BP_SeaWatcher.isDead` false _player_2)
  (set `/Game/Characters/SeaWatcher/BP_SeaWatcher.Imune` false _player)
  (set `/Game/Characters/SeaWatcher/BP_SeaWatcher.Health` (`/Game/Characters/SeaWatcher/BP_SeaWatcher.MaxHealth` _player_2) _player_2)
  (set `/Game/Characters/SeaWatcher/BP_SeaWatcher.NbPotions` (`/Game/Characters/SeaWatcher/BP_SeaWatcher.NbPotionMax` _player_2) _player_2)
  (set `PlayerController.bShowMouseCursor` false (`self.Controller`))
  (switch `int` (`self.PartToRespawn`)
    (:`0`
      (bind _outactors (`GameplayStatics.GetAllActorsOfClass` "/Game/Characters/Enemy/TrashMob/BP_TriggerCrabe.BP_TriggerCrabe_C"))
      (for _array_element _outactors
        (`/Game/Characters/Enemy/TrashMob/BP_TriggerCrabe.Reset` _array_element))
      (bind _outactors_2 (`GameplayStatics.GetAllActorsOfClass` "/Game/GeneralSettings/BP_BarriereDeBebz.BP_BarriereDeBebz_C"))
      (for _array_element_2 _outactors_2
        (`/Game/GeneralSettings/BP_BarriereDeBebz.Deactivate` _array_element_2))
      (for _array_element_3 (`self.DataLayerReset01`)
        (`DataLayerSubsystem.SetDataLayerRuntimeState` (subsystem `DataLayerSubsystem`) _array_element_3 "Activated" false))
      (for _array_element_4 (`self.DataLayerReset02`)
        (`DataLayerSubsystem.SetDataLayerRuntimeState` (subsystem `DataLayerSubsystem`) _array_element_4 "Loaded" false)))
    (:`1`
      (bind _returnvalue (`GameplayStatics.GetActorOfClass` "/Game/GeneralSettings/BP_CamManager.BP_CamManager_C" :!label _label))
      (set `/Game/GeneralSettings/BP_CamManager.Activ?` false _returnvalue)
      (for _array_element_5 (`self.CrabeBoss`)
        (`/Game/Characters/Enemy/Boss/Crabe/BP_Crabe.ResetStagger` _array_element_5))
      (`self.Reset`))
    (:`2`
      (goto _label))
    (:`3`
      (goto _label))))

(fn `OnRep_Reset`)

(fn `UserConstructionScript`)