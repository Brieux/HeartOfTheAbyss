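; Menu player controller that drives the main menu, options and credits through Enhanced Input, with menu music and sound effects.
; Up and down wrap a selection index forwarded to the UIWidMenu2REF widget, whose current menu state decides what select and back do.
; Left and right cycle scalability levels with a short cooldown, including an overall preset.
; Values load from GameUserSettings, apply on confirmation, or come from a hardware benchmark.
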(event `ApplySettings`
  (bind _returnvalue (`GameUserSettings.GetGameUserSettings`))
  (`GameUserSettings.SetViewDistanceQuality` _returnvalue (`self.VDInt`))
  (`GameUserSettings.SetAntiAliasingQuality` _returnvalue (`self.AAInt`))
  (`GameUserSettings.SetPostProcessingQuality` _returnvalue (`self.PPInt`))
  (`GameUserSettings.SetShadowQuality` _returnvalue (`self.ShadowsInt`))
  (`GameUserSettings.SetGlobalIlluminationQuality` _returnvalue (`self.GIInt`))
  (`GameUserSettings.SetReflectionQuality` _returnvalue (`self.RInt`))
  (`GameUserSettings.SetTextureQuality` _returnvalue (`self.TInt`))
  (`GameUserSettings.SetVisualEffectQuality` _returnvalue (`self.EInt`))
  (`GameUserSettings.SetFoliageQuality` _returnvalue (`self.FInt`))
  (`GameUserSettings.SetShadingQuality` _returnvalue (`self.ShadingInt`))
  (`GameUserSettings.ApplySettings` _returnvalue true))

(event `GetSettings`
  (bind _returnvalue (`GameUserSettings.GetGameUserSettings` :!label _label))
  (set `self.VDInt` (`GameUserSettings.GetViewDistanceQuality` _returnvalue))
  (set `self.AAInt` (`GameUserSettings.GetAntiAliasingQuality` _returnvalue))
  (set `self.PPInt` (`GameUserSettings.GetPostProcessingQuality` _returnvalue))
  (set `self.ShadowsInt` (`GameUserSettings.GetShadowQuality` _returnvalue))
  (set `self.GIInt` (`GameUserSettings.GetGlobalIlluminationQuality` _returnvalue))
  (set `self.RInt` (`GameUserSettings.GetReflectionQuality` _returnvalue))
  (set `self.TInt` (`GameUserSettings.GetTextureQuality` _returnvalue))
  (set `self.EInt` (`GameUserSettings.GetVisualEffectQuality` _returnvalue))
  (set `self.FInt` (`GameUserSettings.GetFoliageQuality` _returnvalue))
  (set `self.ShadingInt` (`GameUserSettings.GetShadingQuality` _returnvalue))
  (set `self.GlobalInt` (`GameUserSettings.GetOverallScalabilityLevel` _returnvalue)))

(event `GetRef`
  (params (UI_Wid_Menu2_REF :type "/Game/UI/UI_InteractiveMainMenu Object Reference"))
  (bind _output_get (set `self.UI_Wid_Menu2_REF` UI_Wid_Menu2_REF))
  (`/Game/UI/UI_InteractiveMainMenu.ModuloMenu` _output_get "NewEnumerator5")
  (goto _label))

(event `EnhancedInput|/Game/GeneralSettings/Input/IA_InMenu/IA_MoveDown`
  (params (ActionValue :type Boolean) (ElapsedSeconds :type "Float (double-precision)") (TriggeredSeconds :type "Float (double-precision)") (InputAction :type "InputAction Object Reference" :default "/Game/GeneralSettings/Input/IA_InMenu/IA_MoveDown.IA_MoveDown"))
  (bind _modulomenu (`self.ModuloMenu`))
  (bind _ui_wid_menu2_ref (`self.UI_Wid_Menu2_REF`))
  (:`Completed`
    (if (`self.CanMovePosition`)
      (bind _output_get (set `self.JoystickPosition` (mod (+ (+ (`self.JoystickPosition`) 1) _modulomenu) _modulomenu)))
      (switch `/Game/UI/WhichMenu` (`/Game/UI/UI_InteractiveMainMenu.isInMenu` _ui_wid_menu2_ref) :!label _label_2
        (:`NewEnumerator5`
          (`/Game/UI/UI_InteractiveMainMenu.MoveSelectionPrincipal` _ui_wid_menu2_ref _output_get))
        (:`NewEnumerator6`
          (`/Game/UI/UI_InteractiveMainMenu.MoveSelectionOptionUp/Down` _ui_wid_menu2_ref (stale `EnhancedInput|/Game/GeneralSettings/Input/IA_InMenu/IA_MoveUp` _output_get))))
      (`KismetSystemLibrary.Delay` 0.3)
      (set `self.CanMovePosition` true))))

(event `EnhancedInput|/Game/GeneralSettings/Input/IA_InMenu/IA_MoveUp`
  (params (ActionValue :type Boolean) (ElapsedSeconds :type "Float (double-precision)") (TriggeredSeconds :type "Float (double-precision)") (InputAction :type "InputAction Object Reference" :default "/Game/GeneralSettings/Input/IA_InMenu/IA_MoveUp.IA_MoveUp"))
  (bind _modulomenu (`self.ModuloMenu`))
  (:`Completed`
    (if (`self.CanMovePosition`)
      (bind _output_get (set `self.JoystickPosition` (mod (+ (- (`self.JoystickPosition`) 1) _modulomenu) _modulomenu)))
      (goto _label_2))))

(event `EnhancedInput|/Game/GeneralSettings/Input/IA_InMenu/IA_MoveRight`
  (params (ActionValue :type "Float (double-precision)") (ElapsedSeconds :type "Float (double-precision)") (TriggeredSeconds :type "Float (double-precision)") (InputAction :type "InputAction Object Reference" :default "/Game/GeneralSettings/Input/IA_InMenu/IA_MoveRight.IA_MoveRight"))
  ;[1 1 1] SwitchSettings
  (:`Completed`
    (if (`|EnumEquality` (`/Game/UI/UI_InteractiveMainMenu.isInMenu` (`self.UI_Wid_Menu2_REF`)) "NewEnumerator6")
      ;;[0.9746 0.2451 1] Comment
      (`GameplayStatics.PlaySound2D` "/Game/Sound/UI/UI_SFX_ScrollBar_V3.UI_SFX_ScrollBar_V3" 1.0 1.0 0.0 null null)
      (if (`self.CanMovePosition`)
        (set `self.CanMovePosition` false)
        (switch `int` (`self.JoystickPosition`)
          (:`Default`
            _)
          (:`0`
            (bind _output_get (set `self.GlobalInt` (mod (+ (+ (`self.GlobalInt`) 1) 5) 5)))
            (bind _output_get_2 (set `self.VDInt` _output_get))
            (bind _output_get_3 (set `self.AAInt` _output_get_2))
            (bind _output_get_4 (set `self.PPInt` _output_get_3))
            (bind _output_get_5 (set `self.ShadowsInt` _output_get_4))
            (bind _output_get_6 (set `self.GIInt` _output_get_5))
            (bind _output_get_7 (set `self.RInt` _output_get_6))
            (bind _output_get_8 (set `self.TInt` _output_get_7))
            (bind _output_get_9 (set `self.EInt` _output_get_8))
            (bind _output_get_10 (set `self.FInt` _output_get_9))
            (set `self.ShadingInt` _output_get_10))
          (:`1`
            (set `self.VDInt` (mod (+ (+ (`self.VDInt`) 1) 5) 5)))
          (:`2`
            (set `self.AAInt` (mod (+ (+ (`self.AAInt`) 1) 5) 5)))
          (:`3`
            (set `self.PPInt` (mod (+ (+ (`self.PPInt`) 1) 5) 5)))
          (:`4`
            (set `self.ShadowsInt` (mod (+ (+ (`self.ShadowsInt`) 1) 5) 5)))
          (:`5`
            (set `self.GIInt` (mod (+ (+ (`self.GIInt`) 1) 5) 5)))
          (:`6`
            (set `self.RInt` (mod (+ (+ (`self.RInt`) 1) 5) 5)))
          (:`7`
            (set `self.TInt` (mod (+ (+ (`self.TInt`) 1) 5) 5)))
          (:`8`
            (set `self.EInt` (mod (+ (+ (`self.EInt`) 1) 5) 5)))
          (:`9`
            (set `self.FInt` (mod (+ (+ (`self.FInt`) 1) 5) 5)))
          (:`10`
            (set `self.ShadingInt` (mod (+ (+ (`self.ShadingInt`) 1) 5) 5))))
        (`KismetSystemLibrary.Delay` 0.3 :!label _label_3)
        (set `self.CanMovePosition` true)))))

(event `EnhancedInput|/Game/GeneralSettings/Input/IA_InMenu/IA_Select`
  (params (ActionValue :type Boolean) (ElapsedSeconds :type "Float (double-precision)") (TriggeredSeconds :type "Float (double-precision)") (InputAction :type "InputAction Object Reference" :default "/Game/GeneralSettings/Input/IA_InMenu/IA_Select.IA_Select"))
  (bind _ui_wid_menu2_ref (`self.UI_Wid_Menu2_REF`))
  (:`Completed`
    (switch `/Game/UI/WhichMenu` (`/Game/UI/UI_InteractiveMainMenu.isInMenu` (`self.UI_Wid_Menu2_REF`))
      (:`NewEnumerator5`
        (switch `int` (`self.JoystickPosition`)
          (:`0`
            (`/Game/UI/UI_InteractiveMainMenu.Play` _ui_wid_menu2_ref)
            ;[1 0.06621 0.8652] Comment
            (`GameplayStatics.PlaySound2D` "/Game/Sound/UI/UI_SFX_PlayButton.UI_SFX_PlayButton" 1.0 1.0 0.0 null null)
            (`AudioComponent.FadeOut` (`self.Music`) 3.0 0.0 "Linear"))
          (:`1`
            (`/Game/UI/UI_InteractiveMainMenu.GoOption` _ui_wid_menu2_ref)
            (`GameplayStatics.PlaySound2D` "/Game/Sound/UI/UI_SFX_Validation.UI_SFX_Validation" 1.0 1.0 0.0 null null :!label _label_4))
          (:`2`
            (`/Game/UI/UI_InteractiveMainMenu.Credit` _ui_wid_menu2_ref)
            (goto _label_4))
          (:`3`
            (`/Game/UI/UI_InteractiveMainMenu.Quit` _ui_wid_menu2_ref))))
      (:`NewEnumerator6`
        (switch `int` (`self.JoystickPosition`)
          (:`11`
            (`/Game/UI/UI_InteractiveMainMenu.GoBackMainMenu` (`self.UI_Wid_Menu2_REF`) :!label _label_5))
          (:`12`
            (`self.ApplySettings`)
            (goto _label_5))
          (:`13`
            (bind _returnvalue (`GameUserSettings.GetGameUserSettings`))
            (`GameUserSettings.RunHardwareBenchmark` _returnvalue 10 1.0 1.0)
            (`self.GetSettings`))))
      (:`NewEnumerator7`
        (`/Game/UI/UI_InteractiveMainMenu.StopAnimCredit` (`self.UI_Wid_Menu2_REF`))))))

(event `self.ReceiveBeginPlay`
  ;[1 0.06621 0.8652] Comment
  (`AudioComponent.Play` (`self.Music`) 0.0))

(event `EnhancedInput|/Game/GeneralSettings/Input/IA_InMenu/IA_MoveLeft`
  (params (ActionValue :type "Float (double-precision)") (ElapsedSeconds :type "Float (double-precision)") (TriggeredSeconds :type "Float (double-precision)") (InputAction :type "InputAction Object Reference" :default "/Game/GeneralSettings/Input/IA_InMenu/IA_MoveLeft.IA_MoveLeft"))
  ;[1 1 1] SwitchSettings
  (:`Completed`
    (if (`|EnumEquality` (`/Game/UI/UI_InteractiveMainMenu.isInMenu` (`self.UI_Wid_Menu2_REF`)) "NewEnumerator6")
      ;;[1 0.3176 0.9856] Comment
      (`GameplayStatics.PlaySound2D` "/Game/Sound/UI/UI_SFX_ScrollBar_V3.UI_SFX_ScrollBar_V3" 1.0 1.0 0.0 null null)
      (if (`self.CanMovePosition`)
        (set `self.CanMovePosition` false)
        (switch `int` (`self.JoystickPosition`)
          (:`Default`
            (goto _label_3))
          (:`0`
            (bind _output_get (set `self.GlobalInt` (mod (+ (- (`self.GlobalInt`) 1) 5) 5)))
            (bind _output_get_2 (set `self.VDInt` _output_get))
            (bind _output_get_3 (set `self.AAInt` _output_get_2))
            (bind _output_get_4 (set `self.PPInt` _output_get_3))
            (bind _output_get_5 (set `self.ShadowsInt` _output_get_4))
            (bind _output_get_6 (set `self.GIInt` _output_get_5))
            (bind _output_get_7 (set `self.RInt` _output_get_6))
            (bind _output_get_8 (set `self.TInt` _output_get_7))
            (bind _output_get_9 (set `self.EInt` _output_get_8))
            (bind _output_get_10 (set `self.FInt` _output_get_9))
            (set `self.ShadingInt` _output_get_10)
            (goto _label_3))
          (:`1`
            (set `self.VDInt` (mod (+ (- (`self.VDInt`) 1) 5) 5))
            (goto _label_3))
          (:`2`
            (set `self.AAInt` (mod (+ (- (`self.AAInt`) 1) 5) 5))
            (goto _label_3))
          (:`3`
            (set `self.PPInt` (mod (+ (- (`self.PPInt`) 1) 5) 5))
            (goto _label_3))
          (:`4`
            (set `self.ShadowsInt` (mod (+ (- (`self.ShadowsInt`) 1) 5) 5))
            (goto _label_3))
          (:`5`
            (set `self.GIInt` (mod (+ (- (`self.GIInt`) 1) 5) 5))
            (goto _label_3))
          (:`6`
            (set `self.RInt` (mod (+ (- (`self.RInt`) 1) 5) 5))
            (goto _label_3))
          (:`7`
            (set `self.TInt` (mod (+ (- (`self.TInt`) 1) 5) 5))
            (goto _label_3))
          (:`8`
            (set `self.EInt` (mod (+ (- (`self.EInt`) 1) 5) 5))
            (goto _label_3))
          (:`9`
            (set `self.FInt` (mod (+ (- (`self.FInt`) 1) 5) 5))
            (goto _label_3))
          (:`10`
            (set `self.ShadingInt` (mod (+ (- (`self.ShadingInt`) 1) 5) 5))
            (goto _label_3)))))))

(event `EnhancedInput|/Game/GeneralSettings/Input/IA_BackInMenu`
  (params (ActionValue :type Boolean) (ElapsedSeconds :type "Float (double-precision)") (TriggeredSeconds :type "Float (double-precision)") (InputAction :type "InputAction Object Reference" :default "/Game/GeneralSettings/Input/IA_BackInMenu.IA_BackInMenu"))
  (bind _ui_wid_menu2_ref (`self.UI_Wid_Menu2_REF`))
  (:`Completed`
    (switch `/Game/UI/WhichMenu` (`/Game/UI/UI_InteractiveMainMenu.isInMenu` (`self.UI_Wid_Menu2_REF`))
      (:`NewEnumerator6`
        (`/Game/UI/UI_InteractiveMainMenu.GoBackMainMenu` _ui_wid_menu2_ref))
      (:`NewEnumerator7`
        (`/Game/UI/UI_InteractiveMainMenu.StopAnimCredit` _ui_wid_menu2_ref)))))

(event `self.ReceivePossess`
  (params (PossessedPawn :type "Pawn Object Reference"))
  (`EnhancedInputSubsystemInterface.AddMappingContext` (subsystem `EnhancedInputLocalPlayerSubsystem`) "/Game/GeneralSettings/Input/IMC_Menu01.IMC_Menu01" 0 (struct)))

(fn `UserConstructionScript`)