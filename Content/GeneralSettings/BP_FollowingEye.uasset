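; BP_FollowingEye is an eye actor that watches the player and blinks at irregular moments.
; While IsActiv is set, Tick interpolates the Scene component's world rotation toward the player character.
; A looping timer fires CloseEye, which waits a random delay, then plays a timeline driving a morph target on OeilZlagCorps for the blink, independent of IsActiv.
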(event `self.ReceiveBeginPlay`
  (`KismetSystemLibrary.K2_SetTimerDelegate` (delegate `CloseEye`) 2.0 true))

(event `CloseEye`
  (`KismetSystemLibrary.Delay` (`KismetMathLibrary.RandomFloatInRange` 1.0 2.0))
  (bind (_direction _newtrack_0) (`Timeline|Timeline` :!via `PlayFromStart`)
    (:`Update`
      (`SkeletalMeshComponent.SetMorphTarget` (`self.oeil_zlag_corps`) "Zlagskin_low1" _newtrack_0 true))))

(event `self.ReceiveTick`
  (params (DeltaSeconds :type "Float (single-precision)"))
  (bind _scene (`self.Scene`))
  (if (`self.isActiv`)
    (`SceneComponent.K2_SetWorldRotation` _scene (`KismetMathLibrary.RInterpTo` (`SceneComponent.K2_GetComponentRotation` _scene) (`KismetMathLibrary.FindLookAtRotation` (`self.K2_GetActorLocation`) (`self.K2_GetActorLocation` (`GameplayStatics.GetPlayerCharacter` 0))) DeltaSeconds 50.0) false false)))

(fn `UserConstructionScript`)