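; Spline-based transition zone that blends the BP_SeaWatcher's global light between two zone colors as it travels along the spline.
; The construction script places paired enter/end overlap triggers at both spline ends, and a direction flag selects the active pair, flipping shortly after each exit.
; While active, Tick eases the blend alpha toward the watcher's closest spline input key, continuing after exit until it catches up.
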(event `self.ReceiveBeginPlay`)

(event `self.ReceiveTick`
  (params (DeltaSeconds :type "Float (single-precision)"))
  (bind _returnvalue (`SplineComponent.FindInputKeyClosestToWorldLocation` (`self.Spline`) (`self.K2_GetActorLocation` (`self.As BP Sea Watcher`))))
  (if (or (`self.isActiv?`) (`self.needToFinish`))
    (bind _output_get (set `self.ActualAlpha` (`KismetMathLibrary.FInterpTo_Constant` (`self.ActualAlpha`) _returnvalue DeltaSeconds 2.0)))
    (`/Game/Characters/SeaWatcher/BP_SeaWatcher.ChangeGlobalLight` (`self.As BP Sea Watcher`) (`KismetMathLibrary.LinearColorLerp` (`self.Zone1Color`) (`self.Zone2Color`) (`self.ActualAlpha`)))
    (if (== _output_get _returnvalue)
      (set `self.needToFinish` false))))

(event `self.Enter0-1.OnComponentBeginOverlap`
  (params (OverlappedComponent :type "PrimitiveComponent Object Reference") (OtherActor :type "Actor Object Reference") (OtherComp :type "PrimitiveComponent Object Reference") (OtherBodyIndex :type Integer) (bFromSweep :type Boolean) (SweepResult :type "HitResult Structure (by ref)"))
  (if (`self.0-1?`)
    (bind _asbp_sea_watcher (cast `/Game/Characters/SeaWatcher/BP_SeaWatcher` OtherActor))
    (set `self.isActiv?` true)
    (set `self.As BP Sea Watcher` _asbp_sea_watcher)))

(event `self.End0-1.OnComponentBeginOverlap`
  (params (OverlappedComponent :type "PrimitiveComponent Object Reference") (OtherActor :type "Actor Object Reference") (OtherComp :type "PrimitiveComponent Object Reference") (OtherBodyIndex :type Integer) (bFromSweep :type Boolean) (SweepResult :type "HitResult Structure (by ref)"))
  (if (`self.0-1?`)
    (cast `/Game/Characters/SeaWatcher/BP_SeaWatcher` OtherActor)
    (set `self.needToFinish` true)
    (set `self.isActiv?` false)
    (`KismetSystemLibrary.Delay` 0.2)
    (set `self.0-1?` (not (`self.0-1?`)))))

(event `self.Enter1-0.OnComponentBeginOverlap`
  (params (OverlappedComponent :type "PrimitiveComponent Object Reference") (OtherActor :type "Actor Object Reference") (OtherComp :type "PrimitiveComponent Object Reference") (OtherBodyIndex :type Integer) (bFromSweep :type Boolean) (SweepResult :type "HitResult Structure (by ref)"))
  (if (not (`self.0-1?`))
    (bind _asbp_sea_watcher (cast `/Game/Characters/SeaWatcher/BP_SeaWatcher` OtherActor))
    (set `self.isActiv?` true)
    (set `self.As BP Sea Watcher` _asbp_sea_watcher)))

(event `self.End1-0.OnComponentBeginOverlap`
  (params (OverlappedComponent :type "PrimitiveComponent Object Reference") (OtherActor :type "Actor Object Reference") (OtherComp :type "PrimitiveComponent Object Reference") (OtherBodyIndex :type Integer) (bFromSweep :type Boolean) (SweepResult :type "HitResult Structure (by ref)"))
  (if (not (`self.0-1?`))
    (cast `/Game/Characters/SeaWatcher/BP_SeaWatcher` OtherActor)
    (set `self.needToFinish` true)
    (set `self.isActiv?` false)
    (`KismetSystemLibrary.Delay` 0.2)
    (set `self.0-1?` (not (`self.0-1?`)))))

(fn `UserConstructionScript`
  (bind _spline (`self.Spline`))
  (bind _spline_2 (`self.Spline`))
  (`SceneComponent.K2_SetWorldLocationAndRotation` (`self.Enter0-1`) (`SplineComponent.GetLocationAtTime` _spline_2 0.0 "World" false) (`SplineComponent.GetRotationAtTime` _spline_2 0.0 "World" false) false false)
  (`SceneComponent.K2_SetWorldLocationAndRotation` (`self.End1-0`) (`SplineComponent.GetLocationAtTime` _spline_2 0.0 "World" false) (`SplineComponent.GetRotationAtTime` _spline_2 0.0 "World" false) false false)
  (`SceneComponent.K2_SetWorldLocationAndRotation` (`self.End0-1`) (`SplineComponent.GetLocationAtTime` _spline 1.0 "World" false) (`SplineComponent.GetRotationAtTime` _spline 1.0 "World" false) false false)
  (`SceneComponent.K2_SetWorldLocationAndRotation` (`self.Enter1-0`) (`SplineComponent.GetLocationAtTime` _spline 1.0 "World" false) (`SplineComponent.GetRotationAtTime` _spline 1.0 "World" false) false false))