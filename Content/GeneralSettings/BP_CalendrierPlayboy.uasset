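; BP_CalendrierPlayboy is a calendar point of interest that draws the SeaWatcher character's look toward it while inside its adjustable trigger sphere.
; It can attach to another actor on BeginPlay.
; While active, Tick eases the AnimBP's LookTo using dot products: side position when the calendar is in front, centred otherwise.
; Leaving the sphere stops this and applies only one interpolation step toward zero.
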(event `self.ReceiveBeginPlay`
  (bind _returnvalue (`GameplayStatics.GetActorOfClass` "/Game/Characters/SeaWatcher/BP_SeaWatcher.BP_SeaWatcher_C"))
  (set `self.SeaWatcherRef` _returnvalue)
  (`/Engine/EditorBlueprintResources/StandardMacros.IsValid` (`self.ActorAttach`)
    (:`Is Valid`
      (`self.K2_AttachToActor` (`self.ActorAttach`) "None" "KeepWorld" "KeepRelative" "KeepRelative"))))

(event `self.ReceiveTick`
  (params (DeltaSeconds :type "Float (single-precision)"))
  (bind _seawatcherref (`self.SeaWatcherRef`))
  (bind _returnvalue (`KismetMathLibrary.GetDirectionUnitVector` (`self.K2_GetActorLocation` _seawatcherref) (`self.K2_GetActorLocation`)))
  (if (`self.isActiv`)
    (bind _asabp_sea_watcher_nr (cast `/Game/Characters/SeaWatcher/Mesh/CharaVF/ABP_SeaWatcher_NR` (`SkeletalMeshComponent.GetAnimInstance` (`Character.Mesh` (`self.SeaWatcherRef`)))))
    (set `/Game/Characters/SeaWatcher/Mesh/CharaVF/ABP_SeaWatcher_NR.look to` (`KismetMathLibrary.FInterpTo` (`/Game/Characters/SeaWatcher/Mesh/CharaVF/ABP_SeaWatcher_NR.look to` _asabp_sea_watcher_nr) (`KismetMathLibrary.SelectFloat` (`KismetMathLibrary.MapRangeClamped` (`KismetMathLibrary.Dot_VectorVector` _returnvalue (`self.GetActorRightVector` _seawatcherref)) -1.0 1.0 0.0 100.0) 50.0 (and (`self.isActiv`) (>= (`KismetMathLibrary.Dot_VectorVector` _returnvalue (`self.GetActorForwardVector` _seawatcherref)) 0.45))) DeltaSeconds 1.0) _asabp_sea_watcher_nr)))

(event `self.Sphere.OnComponentBeginOverlap`
  (params (OverlappedComponent :type "PrimitiveComponent Object Reference") (OtherActor :type "Actor Object Reference") (OtherComp :type "PrimitiveComponent Object Reference") (OtherBodyIndex :type Integer) (bFromSweep :type Boolean) (SweepResult :type "HitResult Structure (by ref)"))
  (cast `/Game/Characters/SeaWatcher/BP_SeaWatcher` OtherActor)
  (set `self.isActiv` true))

(event `self.Sphere.OnComponentEndOverlap`
  (params (OverlappedComponent :type "PrimitiveComponent Object Reference") (OtherActor :type "Actor Object Reference") (OtherComp :type "PrimitiveComponent Object Reference") (OtherBodyIndex :type Integer))
  (bind _asbp_sea_watcher (cast `/Game/Characters/SeaWatcher/BP_SeaWatcher` OtherActor))
  (set `self.isActiv` false)
  (bind _asabp_sea_watcher_nr (cast `/Game/Characters/SeaWatcher/Mesh/CharaVF/ABP_SeaWatcher_NR` (`SkeletalMeshComponent.GetAnimInstance` (`Character.Mesh` _asbp_sea_watcher))))
  (set `/Game/Characters/SeaWatcher/Mesh/CharaVF/ABP_SeaWatcher_NR.look to` (`KismetMathLibrary.FInterpTo` (`/Game/Characters/SeaWatcher/Mesh/CharaVF/ABP_SeaWatcher_NR.look to` _asabp_sea_watcher_nr) 0.0 (`GameplayStatics.GetWorldDeltaSeconds`) 1.0) _asabp_sea_watcher_nr))

(fn `UserConstructionScript`
  (`SphereComponent.SetSphereRadius` (`self.Sphere`) (`self.In Sphere Radius`) true))