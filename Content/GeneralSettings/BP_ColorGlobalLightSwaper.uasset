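; BP_ColorGlobalLightSwaper is a trigger actor that changes the global light color when a BP_SeaWatcher enters its box.
; On overlap it passes ColorToSwap to the watcher's ChangeGlobalLight, deactivates itself and activates its linked twin, JumelleToActivate.
; Activate and Deactivate only set IsActiv, which the overlap never checks, so the trigger fires on every watcher entry.
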(event `Activate`
  (set `self.isActiv` true))

(event `Deactivate`
  (set `self.isActiv` false))

(event `self.Box.OnComponentBeginOverlap`
  (params (OverlappedComponent :type "PrimitiveComponent Object Reference") (OtherActor :type "Actor Object Reference") (OtherComp :type "PrimitiveComponent Object Reference") (OtherBodyIndex :type Integer) (bFromSweep :type Boolean) (SweepResult :type "HitResult Structure (by ref)"))
  (if true
    (bind _asbp_sea_watcher (cast `/Game/Characters/SeaWatcher/BP_SeaWatcher` OtherActor))
    (`/Game/Characters/SeaWatcher/BP_SeaWatcher.ChangeGlobalLight` _asbp_sea_watcher (`self.Color to Swap`))
    (`self.Deactivate`)
    (`self.Activate` (`self.JumelleToActivate`))))

(fn `UserConstructionScript`)