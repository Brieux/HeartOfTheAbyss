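; BP_DiscoLight is a disco light that keeps shifting its SpotLight between random colors.
; On BeginPlay it starts a looping timer with a randomized interval, picked once per instance.
; Each tick of that timer stores the current light color, picks a new one from a fixed palette, and restarts a Timeline that lerps the SpotLight from one to the other.
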(event `self.ReceiveBeginPlay`
  (`KismetSystemLibrary.K2_SetTimerDelegate` (delegate `ChangeLight`) (+ (`KismetMathLibrary.RandomFloat`) 0.3) true))

(event `ChangeLight`
  (set `self.NewVar` (`LightComponentBase.GetLightColor` (`self.SpotLight`)))
  (set `self.NewVar_0` (`KismetArrayLibrary.Array_Random` (`|MakeArray` (struct :`R` 0.768151 :`G` 0.064803 :`B` 0.031896 :`A` 1.0) (struct :`G` 0.066626 :`B` 0.57758 :`A` 1.0) (struct :`G` 1.0 :`B` 0.024158 :`A` 1.0) (struct :`R` 0.171441 :`G` 0.701102 :`B` 1.0 :`A` 1.0) (struct :`R` 1.0 :`G` 0.791298 :`A` 1.0) (struct :`R` 0.191202 :`G` 0.01096 :`B` 0.637597 :`A` 1.0) (struct :`R` 0.445201 :`G` 0.266355 :`B` 0.423267 :`A` 1.0) (struct :`G` 0.526042 :`B` 0.112347 :`A` 1.0) (struct :`R` 0.364583 :`G` 0.339376 :`B` 0.206977 :`A` 1.0) :!type "LinearColor Structure")))
  (bind (_direction _newtrack_0) (`Timeline|Timeline` :!via `PlayFromStart`)
    (:`Update`
      (`LightComponent.SetLightColor` (`self.SpotLight`) (`KismetMathLibrary.LinearColorLerp` (`self.NewVar`) (`self.NewVar_0`) _newtrack_0) false))))

(fn `UserConstructionScript`)