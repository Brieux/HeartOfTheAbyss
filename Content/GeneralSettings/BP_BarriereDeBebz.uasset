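; Combat barrier that walls off an area with a Niagara effect and a colliding box until every BP_LilCrab in the level is gone.
; It starts off, is raised by Activate, then after a short delay polls the crab count on Tick to lower itself.
; When flagged LastWall, lowering crossfades BP_Switch_Music_CalmToVnr from Vnr to calm music.
; StopFightMusic is an empty test event, with leftover unconnected fade logic.
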(event `self.ReceiveBeginPlay`
  (`ActorComponent.Deactivate` (`self.Niagara`))
  (`PrimitiveComponent.SetCollisionEnabled` (`self.Box`) "NoCollision"))

(event `Activate`
  (`ActorComponent.Activate` (`self.Niagara`) true)
  (`PrimitiveComponent.SetCollisionEnabled` (`self.Box`) "QueryAndPhysics")
  (`KismetSystemLibrary.Delay` 0.75)
  (set `self.Activ` true))

(event `Deactivate`
  (`ActorComponent.Deactivate` (`self.Niagara`))
  (`PrimitiveComponent.SetCollisionEnabled` (`self.Box`) "NoCollision")
  (`self.FadeMusic`))

(event `self.ReceiveTick`
  (params (DeltaSeconds :type "Float (single-precision)"))
  (if (`self.Activ`)
    (bind _outactors (`GameplayStatics.GetAllActorsOfClass` "/Game/Characters/Enemy/TrashMob/Ptit_Crab/BP_LilCrab.BP_LilCrab_C"))
    (if (<= (`KismetArrayLibrary.Array_Length` _outactors) 0)
      (set `self.Activ` false)
      (`self.Deactivate`))))

(event `FadeMusic`
  (bind _outactors (`GameplayStatics.GetAllActorsOfClass` "/Game/Sound/Music/BP_Switch_Music_CalmToVnr.BP_Switch_Music_CalmToVnr_C"))
  (set `self.Music` (`|GetArrayItem` _outactors))
  (if (`self.LastWall`)
    (`AudioComponent.FadeOut` (`/Game/Sound/Music/BP_Switch_Music_CalmToVnr.Music_Vnr_Test` (`self.Music`)) 4.0 0.0 "Linear")
    (`AudioComponent.FadeIn` (`/Game/Sound/Music/BP_Switch_Music_CalmToVnr.Music_Calm_Test` (`self.Music`)) 5.0 1.0 0.0 "Linear")))

(event `StopFightMusic`
  ;[1 0 0.07535] A TEST
)

(fn `UserConstructionScript`)