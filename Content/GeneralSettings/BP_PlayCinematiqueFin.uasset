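; BP_PlayCinematiqueFin plays the FinCombat end cinematic and handles the switch to the end credits.
; CinematiqueLaunch hides the crab, player and interface, disables input, plays the sequence as view target and destroys all spikes and crab waves.
; It also sets a timer for one second before the sequence ends.
; EndCinematique restores the interface, starts the credit music and calls CreditEnd after a short delay.
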(event `self.ReceiveBeginPlay`
  (bind _asbp_sea_watcher (cast `/Game/Characters/SeaWatcher/BP_SeaWatcher` (`GameplayStatics.GetPlayerCharacter` 0)))
  (bind _output_get (set `self.As BP Sea Watcher` _asbp_sea_watcher))
  (bind _asbp_player_controller (cast `/Game/GeneralSettings/BP_PlayerController` (`Pawn.GetController` _output_get)))
  (set `self.As BP Player Controller` _asbp_player_controller))

(event `CinematiqueLaunch`
  (bind _as_bp_sea_watcher (`self.As BP Sea Watcher`))
  ;[1 1 1] LaunchCinematic
  (`self.SetActorHiddenInGame` (`self.Bp_Crabe`) true)
  (`Widget.SetVisibility` (`/Game/GeneralSettings/BP_PlayerController.Interface` (`self.As BP Player Controller`)) "Hidden")
  (`self.DisableInput` (`self.As BP Sea Watcher`) (`self.As BP Player Controller`))
  (`self.SetActorHiddenInGame` (`self.As BP Sea Watcher`) true)
  (bind (_outactor _returnvalue) (`LevelSequencePlayer.CreateLevelSequencePlayer` "/Game/CUTSCENES/FinCombat/FinCombat.FinCombat"))
  (`PlayerController.SetViewTargetWithBlend` (`self.As BP Player Controller`) _outactor 0.0 "VTBlend_Linear" 0.0 false)
  (`MovieSceneSequencePlayer.Play` _returnvalue)
  (`self.Destroy&Clean`)
  (`/Game/Characters/SeaWatcher/BP_SeaWatcher.RemoveIdleCam` _as_bp_sea_watcher)
  (set `/Game/Characters/SeaWatcher/BP_SeaWatcher.InClam?` true _as_bp_sea_watcher)
  (`KismetSystemLibrary.K2_SetTimerDelegate` (`|CreateDelegate` :!event `EndCinematique`) (- (`TimeManagementBlueprintLibrary.Conv_QualifiedFrameTimeToSeconds` (`MovieSceneSequencePlayer.GetDuration` _returnvalue)) 1.0)))

(event `EndCinematique`
  (bind _interface (`/Game/GeneralSettings/BP_PlayerController.Interface` (`self.As BP Player Controller`)))
  ;[1 1 1] CreditEndCinePhase1
  (set `/Game/Characters/SeaWatcher/BP_SeaWatcher.InClam?` true (`self.As BP Sea Watcher`))
  (`Widget.SetVisibility` _interface "Visible")
  (`/Game/UI/UI_Interface.HideAll` _interface)
  (`GameplayStatics.SpawnSound2D` "/Game/Sound/Music/MS_Credit.MS_Credit" 1.0 1.0 0.0 null)
  (`KismetSystemLibrary.Delay` 1.0)
  (`/Game/UI/UI_Interface.CreditEnd` _interface))

(fn `Destroy&Clean`
  (bind _outactors (`GameplayStatics.GetAllActorsOfClass` "/Game/Characters/Enemy/Boss/Crabe/BP_Spike.BP_Spike_C"))
  (for _array_element _outactors
    (`self.K2_DestroyActor` _array_element))
  (bind _outactors_2 (`GameplayStatics.GetAllActorsOfClass` "/Game/VFX/Crab/BP_CrabWave.BP_CrabWave_C"))
  (for _array_element_2 _outactors_2
    (`self.K2_DestroyActor` _array_element_2)))

(fn `EndCreditPhase1`)

(fn `UserConstructionScript`)