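; BP_IdleCam is an idle camera actor for the player, filed under the SeaWatcher character.
; From BeginPlay, a slow timeline moves the camera along a spline while look-at rotation keeps it aimed at PlayerRef.
; GetIdleCam and LeaveIdleCam switch the player controller's view to this actor and back to PlayerRef with cubic blends, returning faster than entering.
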(event `self.ReceiveBeginPlay`
  (`self.CamTurn`))

(event `CamTurn`
  (bind _camera (`self.Camera`))
  (`TimelineComponent.SetPlayRate` (`self.Timeline_0`) 0.05)
  (bind (_direction _newtrack_0) (`Timeline|Timeline_0`)
    (:`Update`
      (`SceneComponent.K2_SetWorldLocation` _camera (`SplineComponent.GetLocationAtTime` (`self.Spline`) _newtrack_0 "World" false) false false)
      (`SceneComponent.K2_SetWorldRotation` _camera (`KismetMathLibrary.FindLookAtRotation` (`SceneComponent.K2_GetComponentLocation` _camera) (`self.K2_GetActorLocation` (`self.playerRef`))) false false))))

(event `GetIdleCam`
  (`PlayerController.SetViewTargetWithBlend` (`GameplayStatics.GetPlayerController` 0) self 1.0 "VTBlend_Cubic" 0.0 true))

(event `LeaveIdleCam`
  (`PlayerController.SetViewTargetWithBlend` (`GameplayStatics.GetPlayerController` 0) (`self.playerRef`) 0.4 "VTBlend_Cubic" 0.0 true))

(fn `UserConstructionScript`)