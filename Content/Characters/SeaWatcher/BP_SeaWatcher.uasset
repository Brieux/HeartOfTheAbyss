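; SeaWatcher player character: claw/tail combat, potion healing, energy-draining dash with immunity and an ultimate that spends Jauge to spawn missiles.
; Combos choose montages from the previous two attacks within a timer window.
; A detection sphere tracks BP_TestCamera targets for switchable lock-on, which turns the character and reframes the spring arm.
; Tick drives focus, Energy regeneration and sphere-trace fading of BP_Hiding occluders; MoveOrient derives movement-direction enums from velocity.
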(event `EnhancedInput|/Game/GeneralSettings/Input/IA_Heal`
  (params (ActionValue :type Boolean) (ElapsedSeconds :type "Float (double-precision)") (TriggeredSeconds :type "Float (double-precision)") (InputAction :type "InputAction Object Reference" :default "/Game/GeneralSettings/Input/IA_Heal.IA_Heal"))
  (bind _maxhealth (`self.MaxHealth`))
  (bind _returnvalue (* (`self.MaxHealth`) 0.6))
  ;[0 1 0.2334] CombatSystem
  (:`Started`
    (`/Engine/EditorBlueprintResources/StandardMacros.CompareFloat` (`self.Health`) (`self.MaxHealth`)
      (:`<`
        (`/Engine/EditorBlueprintResources/StandardMacros.CompareInt` (`self.NbPotions`)
          (:`>`
            (`KismetSystemLibrary.PrintString` "Heal" true true (struct :`R` 1.0 :`G` 0.043137 :`A` 1.0))
            (set `self.NbPotions` (+ (`self.NbPotions`) -1))
            (`KismetSystemLibrary.PrintString` (`KismetStringLibrary.Conv_DoubleToString` _returnvalue) true true (struct :`R` 1.0 :`G` 0.043137 :`A` 1.0))
            (bind _output_get (set `self.Health` (+ (`self.Health`) _returnvalue)))
            (`/Engine/EditorBlueprintResources/StandardMacros.CompareFloat` _output_get _maxhealth
              (:`>`
                (set `self.Health` _maxhealth))))
          (:`==`
            (`KismetSystemLibrary.PrintString` "Pas de Heal" true true (struct :`R` 1.0 :`G` 0.043137 :`A` 1.0))))))))

(event `AddAnimation`
  (params (MontageToPlay :type "AnimMontage Object Reference"))
  ;[0 1 0.2334] CombatSystem
  (bind _asabp_player (cast `/Game/Characters/SeaWatcher/Test/ABP_Player` (`SkeletalMeshComponent.GetAnimInstance` (`self.Mesh`))))
  (`/Game/Characters/SeaWatcher/Test/ABP_Player.MontageToPlayCombo` _asabp_player MontageToPlay))

(event `ResetCombo`
  ;[0 1 0.2334] CombatSystem
  (set `self.Can'tAttack` false)
  (set `self.PreviousAttack1` "NewEnumerator0")
  (set `self.PreviousAttack2` "NewEnumerator0")
  (`KismetSystemLibrary.K2_ClearAndInvalidateTimerHandle` (`self.TimerComboKeyHandle`)))

(event `EnhancedInput|/Game/GeneralSettings/Input/IA_SpecialAttackA`
  (params (ActionValue :type Boolean) (ElapsedSeconds :type "Float (double-precision)") (TriggeredSeconds :type "Float (double-precision)") (InputAction :type "InputAction Object Reference" :default "/Game/GeneralSettings/Input/IA_SpecialAttackA.IA_SpecialAttackA"))
  ;[1 0.8311 0] AttaqueSpé
  (:`Started`
    (set `self.SpecialA` true)
    (`self.SpecialAttack` :!label _label))
  (:`Completed`
    (set `self.SpecialA` false)))

(event `EnhancedInput|/Game/GeneralSettings/Input/IA_Claw`
  (params (ActionValue :type Boolean) (ElapsedSeconds :type "Float (double-precision)") (TriggeredSeconds :type "Float (double-precision)") (InputAction :type "InputAction Object Reference" :default "/Game/GeneralSettings/Input/IA_Claw.IA_Claw"))
  (bind _clawattack_ (`self.ClawAttack?`))
  (bind _clawattack__2 (`self.ClawAttack?`))
  (bind _clawattack__3 (`self.ClawAttack?`))
  ;[0 1 0.2334] CombatSystem
  (:`Started`
    (set `self.ClawAttack?` true)
    (if (`self.Can'tAttack`) :!label _label_2
      _
      (elif (or (`KismetSystemLibrary.K2_IsValidTimerHandle` (`self.TimerComboKeyHandle`)) (`|EnumEquality` (`self.PreviousAttack1`) "NewEnumerator0"))
        (`KismetSystemLibrary.K2_ClearAndInvalidateTimerHandle` (`self.TimerComboKeyHandle`))
        (bind _returnvalue (`KismetSystemLibrary.K2_SetTimerDelegate` (`|CreateDelegate` :!event `ResetCombo`) (`self.TimerCombo`)))
        (set `self.TimerComboKeyHandle` _returnvalue)
        (set `self.Can'tAttack` true)
        (`|ExecutionSequence`
          (:`then_0`
            (switch `/Game/Characters/SeaWatcher/Enum_Attack` (`self.PreviousAttack1`)
              (:`NewEnumerator0`
                (`self.AddAnimation` (select `bool` _clawattack_ :`false` "/Game/Characters/SeaWatcher/ComboX3/Q1_Montage.Q1_Montage" :`true` "/Game/Characters/SeaWatcher/ComboX3/G1_Montage.G1_Montage" :!type "AnimMontage Object Reference"))
                (set `self.PreviousAttack1` (select `bool` _clawattack_ :`false` "NewEnumerator2" :`true` "NewEnumerator1" :!type "/Game/Characters/SeaWatcher/Enum_Attack Enum")))
              (:`NewEnumerator1`
                (switch `/Game/Characters/SeaWatcher/Enum_Attack` (`self.PreviousAttack2`)
                  (:`NewEnumerator0`
                    (`self.AddAnimation` (select `bool` _clawattack__3 :`false` "/Game/Characters/SeaWatcher/ComboX3/GQ2_Montage.GQ2_Montage" :`true` "/Game/Characters/SeaWatcher/ComboX3/GG2_Montage.GG2_Montage" :!type "AnimMontage Object Reference"))
                    (set `self.PreviousAttack2` (select `bool` _clawattack__3 :`false` "NewEnumerator2" :`true` "NewEnumerator1" :!type "/Game/Characters/SeaWatcher/Enum_Attack Enum")))
                  (:`NewEnumerator1`
                    (`self.AddAnimation` (select `bool` (`self.ClawAttack?`) :`false` "/Game/Characters/SeaWatcher/ComboX3/GGQ3_Montage.GGQ3_Montage" :`true` "/Game/Characters/SeaWatcher/ComboX3/GGG3_Montage.GGG3_Montage" :!type "AnimMontage Object Reference")))
                  (:`NewEnumerator2`
                    (`self.AddAnimation` (select `bool` (`self.ClawAttack?`) :`false` "/Game/Characters/SeaWatcher/ComboX3/GQQ3_Montage.GQQ3_Montage" :`true` "/Game/Characters/SeaWatcher/ComboX3/GQG3_Montage.GQG3_Montage" :!type "AnimMontage Object Reference")))))
              (:`NewEnumerator2`
                (switch `/Game/Characters/SeaWatcher/Enum_Attack` (`self.PreviousAttack2`)
                  (:`NewEnumerator0`
                    (`self.AddAnimation` (select `bool` _clawattack__2 :`false` "/Game/Characters/SeaWatcher/ComboX3/QQ2_Montage.QQ2_Montage" :`true` "/Game/Characters/SeaWatcher/ComboX3/QG2_Montage.QG2_Montage" :!type "AnimMontage Object Reference"))
                    (set `self.PreviousAttack2` (select `bool` _clawattack__2 :`false` "NewEnumerator2" :`true` "NewEnumerator1" :!type "/Game/Characters/SeaWatcher/Enum_Attack Enum")))
                  (:`NewEnumerator1`
                    (`self.AddAnimation` (select `bool` (`self.ClawAttack?`) :`false` "/Game/Characters/SeaWatcher/ComboX3/QGQ3_Montage.QGQ3_Montage" :`true` "/Game/Characters/SeaWatcher/ComboX3/QGG3_Montage.QGG3_Montage" :!type "AnimMontage Object Reference")))
                  (:`NewEnumerator2`
                    (`self.AddAnimation` (select `bool` (`self.ClawAttack?`) :`false` "/Game/Characters/SeaWatcher/ComboX3/QQQ3_Montage.QQQ3_Montage" :`true` "/Game/Characters/SeaWatcher/ComboX3/QQG3_Montage.QQG3_Montage" :!type "AnimMontage Object Reference")))))))
          (:`then_1`
            (set `self.Energy` (- (`self.Energy`) (`KismetMathLibrary.SelectFloat` 10.0 25.0 (`self.ClawAttack?`))))))))))

(event `EnhancedInput|/Game/GeneralSettings/Input/IA_SpecialAttackE`
  (params (ActionValue :type Boolean) (ElapsedSeconds :type "Float (double-precision)") (TriggeredSeconds :type "Float (double-precision)") (InputAction :type "InputAction Object Reference" :default "/Game/GeneralSettings/Input/IA_SpecialAttackE.IA_SpecialAttackE"))
  ;[1 0.8311 0] AttaqueSpé
  (:`Started`
    (set `self.SpecialE` true)
    (goto _label))
  (:`Completed`
    (set `self.SpecialE` false)))

(event `EnhancedInput|/Game/GeneralSettings/Input/IA_Tail`
  (params (ActionValue :type Boolean) (ElapsedSeconds :type "Float (double-precision)") (TriggeredSeconds :type "Float (double-precision)") (InputAction :type "InputAction Object Reference" :default "/Game/GeneralSettings/Input/IA_Tail.IA_Tail"))
  ;[0 1 0.2334] CombatSystem
  (:`Started`
    (set `self.ClawAttack?` false)
    (goto _label_2)))

(event `SpecialAttack`
  ;[1 0.8311 0] AttaqueSpé
  (if (and (`self.SpecialA`) (`self.SpecialE`) (>= (`self.Jauge`) 100.0))
    (`|PlayMontage` (`self.Mesh`) "/Game/Characters/SeaWatcher/Test/AM_Ult.AM_Ult"
      (:`then`
        (bind _returnvalue (`KismetSystemLibrary.K2_SetTimerDelegate` (delegate `SpawnProjectil`) 0.05 true))
        (bind (_direction _newtrack_0) (`Timeline|Timeline_2` :!via `PlayFromStart`)
          (:`Update`
            (set `self.Jauge` (* _newtrack_0 100.0)))
          (:`Finished`
            (`KismetSystemLibrary.K2_ClearAndInvalidateTimerHandle` _returnvalue)))))))

(event `SpawnProjectil`
  ;[1 0.8311 0] AttaqueSpé
  (`|SpawnActorFromClass` "/Game/Characters/SeaWatcher/BP_Missile.BP_Missile_C" (`self.GetTransform`) "AdjustIfPossibleButAlwaysSpawn" "OverrideRootScale" null null))

(event `self.ReceiveAnyDamage`
  (params (Damage :type "Float (single-precision)") (DamageType :type "DamageType Object Reference") (InstigatedBy :type "Controller Object Reference") (DamageCauser :type "Actor Object Reference"))
  ;[1 0.02546 0] Dammage Systeme
  (if (not (`self.Imune`))
    (cast `/Game/AI/AIC_Crabe` DamageCauser
      (:`then`
        (`GameplayStatics.PlayWorldCameraShake` "/Game/GeneralSettings/BP_CamShakeLourd.BP_CamShakeLourd_C" (`SceneComponent.K2_GetComponentLocation` (`self.Camera`)) 0.0 10.0))
      (:`CastFailed`
        _))
    (`/Engine/EditorBlueprintResources/StandardMacros.DoOnce` false :!label _label_3
      (:`Completed`
        (bind _output_get (set `self.Health` (`KismetMathLibrary.FClamp` (- (`self.Health`) (* Damage 2.0)) 0.0 100.0)))
        (if (== _output_get 0.0)
          (`self.Die`)
          (else
            (`|SpawnActorFromClass` "/Game/VFX/Blueprint/BP_DamagedPlayerFeedback_001.BP_DamagedPlayerFeedback_001_C" (`KismetMathLibrary.MakeTransform` (`SceneComponent.K2_GetComponentLocation` (`self.Mesh`))) "Undefined" "OverrideRootScale" null null)
            (`ForceFeedbackComponent.Play` (`self.ForceFeedback`) 0.0)))))))

(event `ResetDammage`
  ;[1 0.02546 0] Dammage Systeme
  (goto _label_3 :!via `Reset`))

(event `Die`
  ;[1 0.02546 0] Dammage Systeme
  (bind _asbp_player_controller (cast `/Game/GeneralSettings/BP_PlayerController` (`self.GetController`)))
  (`/Game/GeneralSettings/BP_PlayerController.Death` _asbp_player_controller))

(event `DesactivateCollisionDash`
  (bind _capsulecomponent (`self.CapsuleComponent`))
  ;[1 0.1168 0] Dash
  (bind _isa (`/Engine/EditorBlueprintResources/StandardMacros.FlipFlop`)
    (:`A`
      _)
    (:`B`
      _))
  (bind _returnvalue (select `bool` _isa :`false` "ECR_Block" :`true` "ECR_Overlap" :!type "ECollisionResponse Enum"))
  (`PrimitiveComponent.SetCollisionResponseToChannel` _capsulecomponent "ECC_GameTraceChannel2" _returnvalue)
  (`PrimitiveComponent.SetCollisionResponseToChannel` _capsulecomponent "ECC_Destructible" _returnvalue)
  (`PrimitiveComponent.SetCollisionResponseToChannel` _capsulecomponent "ECC_Pawn" _returnvalue))

(event `EnhancedInput|/Game/GeneralSettings/Input/IA_Dash`
  (params (ActionValue :type Boolean) (ElapsedSeconds :type "Float (double-precision)") (TriggeredSeconds :type "Float (double-precision)") (InputAction :type "InputAction Object Reference" :default "/Game/GeneralSettings/Input/IA_Dash.IA_Dash"))
  (bind _returnvalue (`self.GetActorForwardVector`))
  (bind _returnvalue_2 (>= (`self.Energy`) (`self.DashEnergyCost`)))
  (bind _velocity (`MovementComponent.Velocity` (`self.CharacterMovement`)))
  (bind _returnvalue_3 (`KismetMathLibrary.VSize` _velocity))
  ;[1 0.1168 0] Dash
  (:`Started`
    (if (`self.DashAvailable`)
      (set `self.Imune` true)
      (`self.DesactivateCollisionDash`)
      (set `self.DashAvailable` false)
      (set `MovementComponent.Velocity` (* (`KismetMathLibrary.SelectVector` (`KismetMathLibrary.SelectVector` _returnvalue (/ _velocity _returnvalue_3) (== _returnvalue_3 0.0)) _returnvalue (`KismetSystemLibrary.IsValid` (`self.Actor to Focus`))) (* (/ (`self.DashLenght`) (`KismetMathLibrary.SelectFloat` 1.0 2.0 _returnvalue_2)) (`KismetMathLibrary.SelectFloat` 6.0 2.0 (`CharacterMovementComponent.IsWalking` (`self.CharacterMovement`))))) (`self.CharacterMovement`))
      (set `self.Energy` (- (`self.Energy`) (`self.DashEnergyCost`)))
      (`ActorComponent.Activate` (`self.DashFX`) false)
      (`|PlayMontage` (`self.Mesh`) "/Game/Characters/SeaWatcher/Test/AM_Dash.AM_Dash" (`KismetMathLibrary.SelectFloat` 0.9 1.2 _returnvalue_2)
        (:`then`
          (`Timeline|Timeline_0` :!via `PlayFromStart`
            (:`Finished`
              (set `self.Imune` false)
              (`self.DesactivateCollisionDash`)
              (`KismetSystemLibrary.Delay` (`self.DashCooldown`))
              (set `self.DashAvailable` true))))))))

(event `FocusToggle`
  (bind _actor_to_focus (`self.Actor to Focus`))
  ;[0 0.2583 1] FocusCam
  (`/Engine/EditorBlueprintResources/StandardMacros.IsValid` _actor_to_focus
    (:`Is Valid`
      (if (`self.ToggleFocusOn?`)
        (if (`self.AtLeastOneEnemyInRange`)
          (if (not (< (`KismetMathLibrary.Vector_Distance` (`self.K2_GetActorLocation`) (`self.K2_GetActorLocation` _actor_to_focus)) (`self.MaxDistanceToFocus`)))
            (`self.incrementIndex` 1)
            (`self.ShowWidgetAndvalidate`))
          (set `self.FocusOn?` true))
        (else
          (set `self.FocusOn?` false))))))

(event `EnhancedInput|/Game/GeneralSettings/Input/IA_ToggleFocus`
  (params (ActionValue :type Boolean) (ElapsedSeconds :type "Float (double-precision)") (TriggeredSeconds :type "Float (double-precision)") (InputAction :type "InputAction Object Reference" :default "/Game/GeneralSettings/Input/IA_ToggleFocus.IA_ToggleFocus"))
  ;[0 0.2583 1] FocusCam
  (:`Started`
    (bind _isa (`/Engine/EditorBlueprintResources/StandardMacros.FlipFlop`)
      (:`A`
        _)
      (:`B`
        _))
    (set `self.ToggleFocusOn?` _isa)))

(event `EnergyFill`
  (if (<= (`self.Energy`) 100.0)
    (set `self.Energy` (`KismetMathLibrary.FClamp` (+ (* 10.0 (`GameplayStatics.GetWorldDeltaSeconds`)) (`self.Energy`)) 0.0 100.0))))

(event `self.ReceiveBeginPlay`
  (`SphereComponent.SetSphereRadius` (`self.Sphere`) (`self.MaxDistanceToFocus`) true)
  (bind _returnvalue (`|CreateWidget` "/Game/UI/UI_Interface.UI_Interface_C"))
  (bind _output_get (set `self.UI_Ref` _returnvalue))
  (set `/Game/UI/UI_Interface.SeaWatcher` self _output_get)
  (`UserWidget.AddToViewport` (`self.UI_Ref`) 1)
  (bind _outactors (`GameplayStatics.GetAllActorsOfClass` "/Game/Characters/Enemy/Boss/BP_TestCamera.BP_TestCamera_C"))
  (for _array_element _outactors
    (`BlueprintMapLibrary.Map_Add` (`self.AllActorToFocus`) _array_element))
  (`ForceFeedbackComponent.Stop` (`self.ForceFeedback`))
  (`KismetSystemLibrary.ExecuteConsoleCommand` "stat fps" null)
  (`PlayerController.SetAudioListenerOverride` :`self` (`GameplayStatics.GetPlayerController` 0) :`AttachToComponent` (`self.SpringArm`))
  (message `EnhancedInputSubsystemInterface.RemoveMappingContext` (pcsubsystem `EnhancedInputLocalPlayerSubsystem` (`GameplayStatics.GetPlayerController` 0)) "/Game/GeneralSettings/Input/IMC_SeaWatcher.IMC_SeaWatcher" (struct)))

(event `SpawnBenit`
  (bind _returnvalue (pcsubsystem `EnhancedInputLocalPlayerSubsystem` (`GameplayStatics.GetPlayerController` 0)))
  (`/Engine/EditorBlueprintResources/StandardMacros.IsValid` _returnvalue
    (:`Is Valid`
      (`EnhancedInputSubsystemInterface.AddMappingContext` _returnvalue "/Game/GeneralSettings/Input/IMC_SeaWatcher.IMC_SeaWatcher" 0 (struct)))))

(event `Focus`
  (bind _springarm (`self.SpringArm`))
  (bind _charactermovement (`self.CharacterMovement`))
  (bind _springarm_2 (`self.SpringArm`))
  (bind _springarm_3 (`self.SpringArm`))
  (bind _returnvalue (`KismetMathLibrary.Vector_Distance` (`self.K2_GetActorLocation`) (`self.K2_GetActorLocation` (`self.Actor to Focus`))))
  (bind _returnvalue_2 (+ (`self.CamDistance`) (/ _returnvalue 5.0)))
  ;[0 0.2583 1] FocusCam
  (if (`self.FocusOn?`)
    (`|ExecutionSequence`
      (:`then_0`
        (`/Engine/EditorBlueprintResources/StandardMacros.DoOnce` false :!label _label_4
          (:`Completed`
            (set `CharacterMovementComponent.bUseControllerDesiredRotation` false _charactermovement)
            (goto _label_5 :!via `Reset`))))
      (:`then_1`
        (`self.K2_SetActorRotation` (`KismetMathLibrary.FindLookAtRotation` (`self.K2_GetActorLocation`) (`self.K2_GetActorLocation` (`self.Actor to Focus`))))
        (`SceneComponent.K2_SetWorldLocation` (`self.SpringArm`) (+ (`self.K2_GetActorLocation`) (* (`self.GetActorForwardVector`) (`self.RayonFocus`))) false false)
        (set `SpringArmComponent.TargetArmLength` _returnvalue_2 _springarm_2)
        (set `SpringArmComponent.SocketOffset` (`KismetMathLibrary.MakeVector` 0.0 0.0 _returnvalue_2) _springarm_2)
        (set `self.FocusOn?` (not (> _returnvalue (`self.MaxDistanceToFocus`))))))
    (else
      (`/Engine/EditorBlueprintResources/StandardMacros.DoOnce` false :!label _label_5
        (:`Completed`
          (set `CharacterMovementComponent.bUseControllerDesiredRotation` true _charactermovement)
          (`SceneComponent.K2_SetRelativeLocation` _springarm (0.0 0.0 0.0) false false)
          (`|ExecutionSequence`
            (:`then_0`
              (set `self.Target Arm Length` (`SpringArmComponent.TargetArmLength` _springarm))
              (bind (_direction _newtrack_0) (`Timeline|Timeline_1` :!via `PlayFromStart`)
                (:`Update`
                  (bind _returnvalue_3 (`KismetMathLibrary.Lerp` (`self.Target Arm Length`) (`self.CamDistance`) _newtrack_0))
                  (set `SpringArmComponent.TargetArmLength` _returnvalue_3 _springarm_3)
                  (set `SpringArmComponent.SocketOffset` (`KismetMathLibrary.MakeVector` 0.0 0.0 _returnvalue_3) _springarm_3))))
            (:`then_1`
              (goto _label_4 :!via `Reset`))))))))

(event `ClearCam`
  (bind _camera (`self.Camera`))
  ;[0.3359 1 0] Detect BP_Hiding in front of cam
  (bind (_outhits _returnvalue) (`KismetSystemLibrary.SphereTraceMultiForObjects` :`Start` (`SceneComponent.K2_GetComponentLocation` _camera) :`End` (+ (* (`KismetMathLibrary.NegateVector` (`SceneComponent.GetForwardVector` _camera)) 20.0) (`SceneComponent.K2_GetComponentLocation` (`self.Mesh`))) :`Radius` 25.0 :`ObjectTypes` (`|MakeArray` "ObjectTypeQuery7" :!type "EObjectTypeQuery Enum") :`DrawTime` 0.0))
  (bind _output_get (set `self.HitToHide` _outhits))
  (for _array_element _output_get
    (bind _asbp_hiding (cast `/Game/Props/BP/BP_Hiding` (`.HitActor` (`GameplayStatics.BreakHitResult` _array_element))))
    (`KismetArrayLibrary.Array_AddUnique` (`self.HindingObject`) _asbp_hiding)
    (`/Game/Props/BP/BP_Hiding.FadeOut` _asbp_hiding))
  (if (not _returnvalue)
    (for _array_element_2 (`self.HindingObject`)
      (`/Game/Props/BP/BP_Hiding.FadeIn` _array_element_2))
    (`KismetArrayLibrary.Array_Clear` (`self.HindingObject`))))

(event `self.ReceiveTick`
  (params (DeltaSeconds :type "Float (single-precision)"))
  (`self.Focus`)
  ;[1 1 1] CanBeSwitchOrUnSwitch
  (`self.FocusToggle`)
  (`self.ClearCam`)
  (`self.EnergyFill`)
  (if (> (`self.Jauge`) 100.0)
    (`/Engine/EditorBlueprintResources/StandardMacros.DoOnce` false
      (:`Completed`
        (`/Game/UI/UI_Interface.ToolTip Tuto` (`self.UI_Ref`) "Appuie sur RT et LT pour utiliser ton ulti" 3.0)))))

(event `self.Sphere.OnComponentBeginOverlap`
  (params (OverlappedComponent :type "PrimitiveComponent Object Reference") (OtherActor :type "Actor Object Reference") (OtherComp :type "PrimitiveComponent Object Reference") (OtherBodyIndex :type Integer) (bFromSweep :type Boolean) (SweepResult :type "HitResult Structure (by ref)"))
  ;[0 0.2583 1] FocusCam
  ;;[0 0.3023 1] DetectLockRange
  (bind _asbp_test_camera (cast `/Game/Characters/Enemy/Boss/BP_TestCamera` OtherActor))
  (`BlueprintMapLibrary.Map_Add` (`self.AllActorToFocus`) _asbp_test_camera true)
  (set `self.AtLeastOneEnemyInRange` true)
  (`self.ShowWidgetAndvalidate`))

(event `ShowWidgetAndValidate`
  ;[0 0.2583 1] FocusCam
  ;;[0 0.2208 1] ShowWidget
  (bind _keys (`BlueprintMapLibrary.Map_Keys` (`self.AllActorToFocus`)))
  (for _array_element _keys
    (`/Engine/EditorBlueprintResources/StandardMacros.IsValid` _array_element
      (:`Is Valid`
        (`/Game/Characters/Enemy/Boss/BP_TestCamera.HideWid` _array_element true))))
  (bind _keys_2 (`BlueprintMapLibrary.Map_Keys` (`self.AllActorToFocus`)))
  (bind _output (`|GetArrayItem` _keys_2 (`self.ActorToFocusIndex`)))
  (if (`BlueprintMapLibrary.Map_Find` (`self.AllActorToFocus`) _output)
    (`/Game/Characters/Enemy/Boss/BP_TestCamera.HideWid` _output false)
    (set `self.Actor to Focus` _output)))

(event `EnhancedInput|/Game/GeneralSettings/Input/IA_Move`
  (params (ActionValue :type "Vector2D Structure") (ElapsedSeconds :type "Float (double-precision)") (TriggeredSeconds :type "Float (double-precision)") (InputAction :type "InputAction Object Reference" :default "/Game/GeneralSettings/Input/IA_Move.IA_Move"))
  (:`Triggered`
    (`self.AddMovementInput` (0.5 0.5 0.0) (`KismetMathLibrary.NormalizeToRange` (* ActionValue_X 1.0) 0.0 0.7))
    (`self.AddMovementInput` (0.5 -0.5 0.0) (`KismetMathLibrary.NormalizeToRange` (* ActionValue_Y 1.0) 0.0 0.7))
    (`self.MoveOrient` (`MovementComponent.Velocity` (`self.CharacterMovement`))))
  (:`Completed`
    (`self.MoveOrient` (0.0 0.0 0.0))))

(event `self.Sphere.OnComponentEndOverlap`
  (params (OverlappedComponent :type "PrimitiveComponent Object Reference") (OtherActor :type "Actor Object Reference") (OtherComp :type "PrimitiveComponent Object Reference") (OtherBodyIndex :type Integer))
  (bind _allactortofocus (`self.AllActorToFocus`))
  ;[0 0.2583 1] FocusCam
  ;;[0 0.3023 1] DetectLockRange
  (bind _asbp_test_camera (cast `/Game/Characters/Enemy/Boss/BP_TestCamera` OtherActor))
  (`BlueprintMapLibrary.Map_Add` _allactortofocus _asbp_test_camera)
  (bind _values (`BlueprintMapLibrary.Map_Values` _allactortofocus))
  (for _array_element _values :!label _label_6
    (if _array_element
      (set `self.AtLeastOneEnemyInRange` true)
      (`self.BreakLoopDetection`)
      (else
        (set `self.AtLeastOneEnemyInRange` false))))
  (`self.ShowWidgetAndvalidate`))

(event `EnhancedInput|/Game/GeneralSettings/Input/IA_ChangeFocus`
  (params (ActionValue :type "Float (double-precision)") (ElapsedSeconds :type "Float (double-precision)") (TriggeredSeconds :type "Float (double-precision)") (InputAction :type "InputAction Object Reference" :default "/Game/GeneralSettings/Input/IA_ChangeFocus.IA_ChangeFocus"))
  ;[0 0.2583 1] FocusCam
  (:`Started`
    (if (`self.AtLeastOneEnemyInRange`)
      (`self.incrementIndex` (`KismetMathLibrary.SelectInt` 1 -1 (> ActionValue 0.0))))))

(event `BreakLoopDetection`
  ;[0 0.2583 1] FocusCam
  ;;[0 0.3023 1] DetectLockRange
  (goto _label_6 :!via `Break`))

(event `IncrementIndex`
  (params (`+` :type Integer))
  (bind _returnvalue (`BlueprintMapLibrary.Map_Length` (`self.AllActorToFocus`)))
  ;[0 0.2583 1] FocusCam
  ;;[0 0.1805 1] IncrementIndex
  (set `self.ActorToFocusIndex` (mod (`KismetMathLibrary.Abs_Int` (+ `+` (+ (`self.ActorToFocusIndex`) _returnvalue))) _returnvalue))
  (bind _keys (`BlueprintMapLibrary.Map_Keys` (`self.AllActorToFocus`)))
  (if (`BlueprintMapLibrary.Map_Find` (`self.AllActorToFocus`) (`|GetArrayItem` _keys (`self.ActorToFocusIndex`)))
    (`self.ShowWidgetAndvalidate`)
    (else
      (`self.incrementIndex` `+`))))

(fn `MoveOrient`
  (params (A :type "Vector Structure"))
  (bind _velocity (`MovementComponent.Velocity` (`self.CharacterMovement`)))
  (bind _velocity_2 (`MovementComponent.Velocity` (`self.CharacterMovement`)))
  (bind _velocity_3 (`MovementComponent.Velocity` (`self.CharacterMovement`)))
  (bind _velocity_4 (`MovementComponent.Velocity` (`self.CharacterMovement`)))
  (`|ExecutionSequence`
    (:`then_0`
      (if (== (`self.GetActorForwardVector`) (/ _velocity_2 (`KismetMathLibrary.VSize` _velocity_2)) :`ErrorTolerance` 0.8)
        (set `self.MoveOrientationForward` "NewEnumerator0")
        (elif (== (`KismetMathLibrary.NegateVector` (`self.GetActorForwardVector`)) (/ _velocity_3 (`KismetMathLibrary.VSize` _velocity_3)) :`ErrorTolerance` 0.8)
          (set `self.MoveOrientationForward` "NewEnumerator1")
          (else
            (set `self.MoveOrientationForward` "NewEnumerator4")))))
    (:`then_1`
      (if (== (`self.GetActorRightVector`) (/ _velocity_4 (`KismetMathLibrary.VSize` _velocity_4)) :`ErrorTolerance` 0.8)
        (set `self.MoveOrientationRight` "NewEnumerator3")
        (elif (== (`KismetMathLibrary.NegateVector` (`self.GetActorRightVector`)) (/ _velocity (`KismetMathLibrary.VSize` _velocity)) :`ErrorTolerance` 0.8)
          (set `self.MoveOrientationRight` "NewEnumerator2")
          (else
            (set `self.MoveOrientationRight` "NewEnumerator4")))))
    (:`then_2`
      (if (== (`KismetMathLibrary.VSize` A) 0.0)
        (set `self.MoveOrientationForward` "NewEnumerator4")
        (set `self.MoveOrientationRight` "NewEnumerator4")))))

(fn `UserConstructionScript`)