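; Homing missile for the SeaWatcher character that flies a randomized arc to its assigned target.
; On BeginPlay it builds a three-point spline with an upward-biased random midpoint, and a Timeline moves and rotates the missile along it.
; Tick keeps the spline's endpoint on the moving target.
; When the Timeline finishes, it applies radial damage and sends a hit message using the player's damage balancer, then destroys itself.
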(event `self.ReceiveBeginPlay`
  (bind _returnvalue_location (`KismetMathLibrary.BreakTransform` (`self.GetTransform`)))
  (bind (_returnvalue_x _returnvalue_y _returnvalue_z) (`KismetMathLibrary.BreakVector` (`KismetMathLibrary.RandomUnitVector`)))
  (bind _target (`self.Target`))
  (bind _returnvalue (`self.K2_GetActorLocation` (`self.Target`)))
  (bind _dammagebalancerref_dammagebalancer (break `/Game/GeneralSettings/Struct_DammageBalancer` (`/Game/Characters/SeaWatcher/BP_SeaWatcher.DammageBalancerRef` (cast `/Game/Characters/SeaWatcher/BP_SeaWatcher` (`GameplayStatics.GetPlayerCharacter` 0) :!pure true))))
  (bind _value (`BlueprintMapLibrary.Map_Find` _dammagebalancerref_dammagebalancer "NewEnumerator13"))
  (bind _returnvalue_2 (`AddComponent|NODE_AddSplineComponent-0` :`RelativeTransform` (`KismetMathLibrary.MakeTransform` _returnvalue_location (`KismetMathLibrary.Conv_VectorToRotator` (`self.GetActorForwardVector`)))))
  (set `self.FollowSpline` _returnvalue_2)
  (`SplineComponent.SetLocationAtSplinePoint` _returnvalue_2 1 (+ (`KismetMathLibrary.VLerp` _returnvalue_location _returnvalue 0.5) (* (`KismetMathLibrary.MakeVector` _returnvalue_x _returnvalue_y (`KismetMathLibrary.Abs` _returnvalue_z)) (`self.lenghrandom`))) "World" true)
  (`SplineComponent.AddSplinePoint` _returnvalue_2 _returnvalue "World" true)
  ;[1 1 1] vitesse de déplacement des missiles
  (bind (_direction _newtrack_0) (`Timeline|Timeline_0`)
    (:`Update`
      (`self.K2_SetActorLocationAndRotation` (`SplineComponent.GetLocationAtTime` _returnvalue_2 _newtrack_0 "World" false) (`SplineComponent.GetRotationAtTime` _returnvalue_2 _newtrack_0 "World" false))
      (`SceneComponent.K2_SetRelativeLocationAndRotation` :`self` (`self.Niagara`)))
    (:`Finished`
      (`/Engine/EditorBlueprintResources/StandardMacros.IsValid` _target
        (:`Is Valid`
          (`GameplayStatics.ApplyRadialDamage` :`BaseDamage` (* _value 0.5) :`Origin` (`self.K2_GetActorLocation`) :`DamageRadius` 350.0 :`DamageCauser` null :`InstigatedByController` null)
          (message `/Game/GeneralSettings/Int_Hittable.GetHit` _target _value (0.0 0.0 0.0) false true false)
          (set `self.Target` null))
        (:`Is Not Valid`
          _))
      (`self.K2_DestroyActor`))))

(event `self.ReceiveTick`
  (params (DeltaSeconds :type "Float (single-precision)"))
  (bind _followspline (`self.FollowSpline`))
  (bind _target (`self.Target`))
  (`/Engine/EditorBlueprintResources/StandardMacros.IsValid` _followspline
    (:`Is Valid`
      (`/Engine/EditorBlueprintResources/StandardMacros.IsValid` _target
        (:`Is Valid`
          (`SplineComponent.SetLocationAtSplinePoint` _followspline 2 (`self.K2_GetActorLocation` _target) "World" true))))))

(fn `UserConstructionScript`)