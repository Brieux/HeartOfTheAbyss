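; BP_LilCrab is a small trash-mob crab enemy that attacks BP_SeaWatcher in melee and dies in one hit.
; While the player overlaps its box, a looping timer plays the attack montage, which applies damage on completion.
; The first hit flashes a dynamic material glow, unpossesses the crab and spawns impact FX.
; A death montage then triggers death FX on notify and, on blend out, spawns a BP_ZlagBall and destroys the actor.
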(event `self.ReceiveBeginPlay`
  (bind _asbp_sea_watcher (cast `/Game/Characters/SeaWatcher/BP_SeaWatcher` (`GameplayStatics.GetPlayerCharacter` 0)))
  (set `self.As BP Sea Watcher` _asbp_sea_watcher)
  (bind _returnvalue (`KismetMaterialLibrary.CreateDynamicMaterialInstance` "/Game/Characters/Enemy/TrashMob/Ptit_Crab/Materials/M_Ptit_Crab_Inst.M_Ptit_Crab_Inst"))
  (bind _output_get (set `self.Mat` _returnvalue))
  (`PrimitiveComponent.SetMaterial` (`self.SkeletalMesh`) 0 _output_get))

(event `HitPlayer`
  (bind _as_bp_sea_watcher (`self.As BP Sea Watcher`))
  (`/Engine/EditorBlueprintResources/StandardMacros.IsValid` _as_bp_sea_watcher
    (:`Is Valid`
      (`|PlayMontage` (`self.SkeletalMesh`) "/Game/Characters/Enemy/TrashMob/Ptit_Crab/Anim/LilCrabAttack.LilCrabAttack"
        (:`OnCompleted`
          (`GameplayStatics.ApplyDamage` _as_bp_sea_watcher 2.0)
          (`/Game/Characters/SeaWatcher/BP_SeaWatcher.ResetDammage` _as_bp_sea_watcher))))))

(event `self.Box.OnComponentBeginOverlap`
  (params (OverlappedComponent :type "PrimitiveComponent Object Reference") (OtherActor :type "Actor Object Reference") (OtherComp :type "PrimitiveComponent Object Reference") (OtherBodyIndex :type Integer) (bFromSweep :type Boolean) (SweepResult :type "HitResult Structure (by ref)"))
  (bind _asbp_sea_watcher (cast `/Game/Characters/SeaWatcher/BP_SeaWatcher` OtherActor))
  (set `self.As BP Sea Watcher` _asbp_sea_watcher)
  (bind _returnvalue (`KismetSystemLibrary.K2_SetTimerDelegate` (delegate `HitPlayer`) 1.0 true))
  (set `self.Handler` _returnvalue))

(event `self.Box.OnComponentEndOverlap`
  (params (OverlappedComponent :type "PrimitiveComponent Object Reference") (OtherActor :type "Actor Object Reference") (OtherComp :type "PrimitiveComponent Object Reference") (OtherBodyIndex :type Integer))
  (cast `/Game/Characters/SeaWatcher/BP_SeaWatcher` OtherActor)
  (set `self.As BP Sea Watcher` null)
  (if (`KismetSystemLibrary.K2_IsValidTimerHandle` (`self.Handler`))
    (`KismetSystemLibrary.K2_ClearAndInvalidateTimerHandle` (`self.Handler`))))

(event `Die`
  (params (V3 :type "Vector Structure"))
  (`|SpawnActorFromClass` "/Game/Characters/Enemy/TrashMob/BP_ZlagBall.BP_ZlagBall_C" (`KismetMathLibrary.MakeTransform` V3) "Undefined" "OverrideRootScale" null null)
  (`self.K2_DestroyActor`))

(event `/Game/GeneralSettings/Int_Hittable.GetHit`
  (params (Dammage :type "Float (double-precision)") (PositionHited :type "Vector Structure") (ComboEnd :type Boolean) (`Missile?` :type Boolean))
  (bind _returnvalue (`SceneComponent.GetSocketLocation` (`self.SkeletalMesh`) "Bind_BodySocket"))
  (`/Engine/EditorBlueprintResources/StandardMacros.DoOnce` false
    (:`Completed`
      (`MaterialInstanceDynamic.SetScalarParameterValue` (`self.Mat`) "Glow" 50.0)
      (`Controller.UnPossess` (`self.GetController`))
      (`NiagaraFunctionLibrary.SpawnSystemAtLocation` "/Game/VFX/NiagaraSystem/NS_Impact_01.NS_Impact_01" PositionHited)
      (`KismetSystemLibrary.Delay` 0.15)
      (`|PlayMontage` (`self.SkeletalMesh`) (`|GetArrayItem` (`self.Montage to Play`) 1)
        (:`OnBlendOut`
          (`self.Die` _returnvalue))
        (:`OnNotifyBegin`
          (`NiagaraFunctionLibrary.SpawnSystemAtLocation` "/Game/VFX/NiagaraSystem/Mick/LilCrab/NS_LitlCrab_Death.NS_LitlCrab_Death" _returnvalue))))))

(fn `UserConstructionScript`)