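; BP_LilCrabCreeper is a small crab trash-mob enemy that attacks BP_SeaWatcher up close and dies in one hit.
; Box overlap runs a looping timer that plays random attack montages, applying BalancerRef damage on their notify.
; A non-missile hit or radial damage fires a DoOnce death: glow, controller detach and montage.
; That montage's notify calls Die, which spawns a randomly scaled BP_ZlagBall and destroys the crab; missile hits only spawn impact effects.
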(event `self.ReceiveBeginPlay`
  (bind _asbp_sea_watcher (cast `/Game/Characters/SeaWatcher/BP_SeaWatcher` (`GameplayStatics.GetPlayerCharacter` 0)))
  (set `self.As BP Sea Watcher` _asbp_sea_watcher)
  (bind _returnvalue (`KismetMaterialLibrary.CreateDynamicMaterialInstance` "/Game/Characters/Enemy/TrashMob/Ptit_Crab/Materials/M_Ptit_Crab_Inst.M_Ptit_Crab_Inst"))
  (bind _output_get (set `self.Mat` _returnvalue))
  (`PrimitiveComponent.SetMaterial` (`self.SkeletalMesh`) 0 _output_get))

(event `HitPlayer`
  (bind _balancerref_dammageapply (break `/Game/GeneralSettings/Struct_DammageApplyOnPlayer` (`self.BalancerRef`)))
  (bind _as_bp_sea_watcher (`self.As BP Sea Watcher`))
  (`/Engine/EditorBlueprintResources/StandardMacros.IsValid` _as_bp_sea_watcher
    (:`Is Valid`
      (if (not (`self.IsAttacking`))
        (set `self.IsAttacking` true)
        (`/Game/Characters/SeaWatcher/BP_SeaWatcher.ResetDammage` _as_bp_sea_watcher)
        (`|PlayMontage` (`self.SkeletalMesh`) (`KismetArrayLibrary.Array_Random` (`|MakeArray` "/Game/Characters/Enemy/TrashMob/Ptit_Crab/Anim/AM_Attack01.AM_Attack01" "/Game/Characters/Enemy/TrashMob/Ptit_Crab/Anim/AM_Attack02.AM_Attack02" :!type "AnimMontage Object Reference"))
          (:`OnNotifyBegin`
            (`GameplayStatics.ApplyDamage` _as_bp_sea_watcher (`BlueprintMapLibrary.Map_Find` _balancerref_dammageapply "NewEnumerator1"))
            (set `self.IsAttacking` false)))))))

(event `Die`
  (bind _skeletalmesh (`self.SkeletalMesh`))
  (bind _asbp_sea_watcher (cast `/Game/Characters/SeaWatcher/BP_SeaWatcher` (`GameplayStatics.GetPlayerCharacter` 0)))
  (set `/Game/Characters/SeaWatcher/BP_SeaWatcher.WhoIsHit` "CrabDeath" _asbp_sea_watcher)
  (`|SpawnActorFromClass` "/Game/VFX/Blueprint/BP_ZlagBall.BP_ZlagBall_C" (`KismetMathLibrary.MakeTransform` (`SceneComponent.GetSocketLocation` (`self.SkeletalMesh`) "Bind_Body") (`KismetMathLibrary.MakeRotator` 0.0 0.0 (`KismetMathLibrary.RandomFloatInRange` 0.0 360.0)) (`KismetMathLibrary.VLerp` (0.3 0.3 0.3) (0.6 0.6 0.6) (`KismetMathLibrary.RandomFloat`))) "AdjustIfPossibleButAlwaysSpawn" "OverrideRootScale" null null)
  (`|ExecutionSequence`
    (:`then_0`
      (goto _label :!via `Reset`))
    (:`then_1`
      (`SkeletalMeshComponent.Stop` (`self.SkeletalMesh`))
      (`KismetSystemLibrary.DelayUntilNextTick`)
      (`self.K2_DestroyActor`))))

(event `self.Box.OnComponentBeginOverlap`
  (params (OverlappedComponent :type "PrimitiveComponent Object Reference") (OtherActor :type "Actor Object Reference") (OtherComp :type "PrimitiveComponent Object Reference") (OtherBodyIndex :type Integer) (bFromSweep :type Boolean) (SweepResult :type "HitResult Structure (by ref)"))
  (if (`self.NotDead`)
    (bind _asbp_sea_watcher (cast `/Game/Characters/SeaWatcher/BP_SeaWatcher` OtherActor))
    (set `self.As BP Sea Watcher` _asbp_sea_watcher)
    (bind _returnvalue (`KismetSystemLibrary.K2_SetTimerDelegate` (delegate `HitPlayer`) (`KismetMathLibrary.RandomFloatInRange` 0.6 0.7) true))
    (set `self.Handler` _returnvalue)))

(event `self.Box.OnComponentEndOverlap`
  (params (OverlappedComponent :type "PrimitiveComponent Object Reference") (OtherActor :type "Actor Object Reference") (OtherComp :type "PrimitiveComponent Object Reference") (OtherBodyIndex :type Integer))
  (if (`self.NotDead`)
    (cast `/Game/Characters/SeaWatcher/BP_SeaWatcher` OtherActor)
    (set `self.As BP Sea Watcher` null)
    (if (`KismetSystemLibrary.K2_IsValidTimerHandle` (`self.Handler`))
      (`KismetSystemLibrary.K2_ClearAndInvalidateTimerHandle` (`self.Handler`))
      (set `self.IsAttacking` false))))

(event `/Game/GeneralSettings/Int_Hittable.GetHit`
  (params (Dammage :type "Float (double-precision)") (PositionHited :type "Vector Structure") (ComboEnd :type Boolean) (`Missile?` :type Boolean) (ClawAttack :type Boolean))
  (bind (_returnvalue_x _returnvalue_y _returnvalue_z) (`KismetMathLibrary.BreakVector` (`self.K2_GetActorLocation`)))
  (bind _skeletalmesh (`self.SkeletalMesh`))
  (if `Missile?`
    (`NiagaraFunctionLibrary.SpawnSystemAtLocation` "/Game/VFX/SeaWatcher/ULTI/NS_ImpactUlti.NS_ImpactUlti" (`KismetMathLibrary.MakeVector` (+ _returnvalue_x (`KismetMathLibrary.RandomFloatInRange` 0.0 50.0)) (+ _returnvalue_y (`KismetMathLibrary.RandomFloatInRange` 0.0 50.0)) (+ _returnvalue_z 25.0)))
    (else
      (`/Engine/EditorBlueprintResources/StandardMacros.DoOnce` false :!label _label
        (:`Completed`
          (`/Game/Characters/SeaWatcher/BP_SeaWatcher.PlayPlayerHitCameraShake` (cast `/Game/Characters/SeaWatcher/BP_SeaWatcher` (`GameplayStatics.GetPlayerCharacter` 0) :!pure true))
          (if (`KismetSystemLibrary.K2_IsValidTimerHandle` (`self.Handler`))
            (`KismetSystemLibrary.K2_ClearAndInvalidateTimerHandle` (`self.Handler`))
            (set `self.IsAttacking` false))
          (`MaterialInstanceDynamic.SetScalarParameterValue` (`self.Mat`) "Glow" 50.0)
          (`self.DetachFromControllerPendingDestroy`)
          (set `self.NotDead` false)
          (`PrimitiveComponent.SetCollisionResponseToChannel` (`self.CapsuleComponent`) "ECC_Pawn" "ECR_Ignore")
          (`NiagaraFunctionLibrary.SpawnSystemAtLocation` "/Game/VFX/NS_Impact_Leger.NS_Impact_Leger" PositionHited)
          (`SkeletalMeshComponent.Stop` _skeletalmesh)
          (`KismetSystemLibrary.Delay` 0.15)
          (`|PlayMontage` _skeletalmesh (`|GetArrayItem` (`self.Montage to Play`) 1)
            (:`then`
              (if (`KismetSystemLibrary.K2_IsValidTimerHandle` (`self.Handler`))
                (`KismetSystemLibrary.K2_ClearAndInvalidateTimerHandle` (`self.Handler`))
                (set `self.IsAttacking` false)))
            (:`OnNotifyBegin`
              (`NiagaraFunctionLibrary.SpawnSystemAtLocation` "/Game/VFX/NiagaraSystem/Mick/LilCrab/NS_LitlCrab_Death.NS_LitlCrab_Death" (`SceneComponent.GetSocketLocation` (`self.SkeletalMesh`) "Bind_BodySocket"))
              (`self.Die`))))))))

(event `self.ReceiveRadialDamage`
  (params (DamageReceived :type "Float (single-precision)") (DamageType :type "DamageType Object Reference") (Origin :type "Vector Structure") (HitInfo :type "HitResult Structure (by ref)") (InstigatedBy :type "Controller Object Reference") (DamageCauser :type "Actor Object Reference"))
  (goto _label))

(fn `UserConstructionScript`)