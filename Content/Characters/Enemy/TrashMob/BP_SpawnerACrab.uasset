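; BP_SpawnerACrab is an enemy spawner that releases batches of BP_LilCrab at its own transform.
; AddSpawn stores the requested count, spawns immediately, then repeats Spawn on a short looping timer.
; Spawn decrements the counter before checking it, so a batch yields one fewer than requested, and clears the timer at zero.
; Each crab's AIC_IntelligentCrab is triggered unless the level's BP_Crabe has NeedToFlew set.
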(event `Spawn`
  (bind _result (`/Engine/EditorBlueprintResources/StandardMacros.DecrementInt` (`self.Counter`))
    (:`  `
      (bind _output_get (set `self.Counter` _result))
      (if (> _output_get 0)
        (bind _returnvalue (`|SpawnActorFromClass` "/Game/Characters/Enemy/TrashMob/Ptit_Crab/BP_LilCrab.BP_LilCrab_C" (`self.GetTransform`) "AdjustIfPossibleButAlwaysSpawn" "OverrideRootScale" null null))
        (bind _asaic_intelligent_crab (cast `/Game/AI/AIC_IntelligentCrab` (`Pawn.GetController` _returnvalue)))
        (bind _returnvalue_2 (`GameplayStatics.GetActorOfClass` "/Game/Characters/Enemy/Boss/Crabe/BP_Crabe.BP_Crabe_C"))
        (if (not (`/Game/Characters/Enemy/Boss/Crabe/BP_Crabe.needToFlew` _returnvalue_2))
          (`/Game/AI/AIC_IntelligentCrab.Trigger` _asaic_intelligent_crab))
        (else
          (`KismetSystemLibrary.K2_ClearAndInvalidateTimerHandle` (`self.Timer`)))))))

(event `AddSpawn`
  (params (Counter :type Integer))
  (set `self.Counter` Counter)
  (`self.Spawn`)
  (bind _returnvalue (`KismetSystemLibrary.K2_SetTimerDelegate` (delegate `Spawn`) 0.3 true))
  (set `self.Timer` _returnvalue))

(fn `UserConstructionScript`)