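; BP_ZlagBall is a trash-mob actor that floats in place until a BP_SeaWatcher touches it.
; On BeginPlay a timeline lerps it vertically from its start location, with randomized height and play rate to vary each instance's motion.
; Overlapping its sphere stops the timeline, adds to the SeaWatcher's Jauge gauge, spawns BP_Zlag_test_2 at its transform and destroys the ball.
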(event `self.ReceiveBeginPlay`
  (bind _output_get (set `self.NewVar_0` (`self.K2_GetActorLocation`)))
  (`TimelineComponent.SetPlayRate` (`self.Timeline_0`) (`KismetMathLibrary.RandomFloatInRange` 0.4 0.6))
  (set `self.NewVar_1` (`KismetMathLibrary.RandomFloatInRange` 90.0 110.0))
  (bind (_direction _newtrack_0) (`Timeline|Timeline_0` :!label _label)
    (:`Update`
      (`self.K2_SetActorLocation` (`KismetMathLibrary.VLerp` _output_get (+ _output_get (`KismetMathLibrary.MakeVector` 0.0 0.0 (`self.NewVar_1`))) _newtrack_0)))))

(event `self.Sphere1.OnComponentBeginOverlap`
  (params (OverlappedComponent :type "PrimitiveComponent Object Reference") (OtherActor :type "Actor Object Reference") (OtherComp :type "PrimitiveComponent Object Reference") (OtherBodyIndex :type Integer) (bFromSweep :type Boolean) (SweepResult :type "HitResult Structure (by ref)"))
  (bind _asbp_sea_watcher (cast `/Game/Characters/SeaWatcher/BP_SeaWatcher` OtherActor))
  (`|ExecutionSequence`
    (:`then_0`
      (goto _label :!via `Stop`))
    (:`then_1`
      (set `/Game/Characters/SeaWatcher/BP_SeaWatcher.Jauge` (+ (`/Game/Characters/SeaWatcher/BP_SeaWatcher.Jauge` _asbp_sea_watcher) 10.0) _asbp_sea_watcher)
      (`|SpawnActorFromClass` "/Game/VFX/Blueprint/BP_Zlag_test_2.BP_Zlag_test_2_C" (`self.GetTransform`) "AlwaysSpawn" "OverrideRootScale" null null)
      (`self.K2_DestroyActor`))))

(fn `UserConstructionScript`)