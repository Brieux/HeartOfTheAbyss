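; BP_TriggerCrabe is a box trigger that starts crab spawning when a BP_SeaWatcher overlaps it.
; It calls AddSpawn on every entry in EachCrab with a random amount between Min and Max, then activates the linked BPTriggerPorte if valid.
; The DoOnce runs before the cast, so the first overlap by any actor uses up the trigger.
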(event `self.Box.OnComponentBeginOverlap`
  (params (OverlappedComponent :type "PrimitiveComponent Object Reference") (OtherActor :type "Actor Object Reference") (OtherComp :type "PrimitiveComponent Object Reference") (OtherBodyIndex :type Integer) (bFromSweep :type Boolean) (SweepResult :type "HitResult Structure (by ref)"))
  (`/Engine/EditorBlueprintResources/StandardMacros.DoOnce` false
    (:`Completed`
      (cast `/Game/Characters/SeaWatcher/BP_SeaWatcher` OtherActor)
      (for _array_element (`self.EachCrab`)
        (`/Game/Characters/Enemy/TrashMob/BP_SpawnerACrab.AddSpawn` _array_element (`KismetMathLibrary.RandomIntegerInRange` (`self.Min`) (`self.Max`))))
      (`/Engine/EditorBlueprintResources/StandardMacros.IsValid` (`self.BP_TriggerPorte`)
        (:`Is Valid`
          (`/Game/BP_BarriereBebeTuto.Activate` (`self.BP_TriggerPorte`)))))))

(fn `UserConstructionScript`)