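; Hittable blob enemy that dies only to the attack pattern set by its Type: Attack, Combo or Ulti.
; Each gated hit spawns an actor, fills the player's gauge, then runs that type's check, which tracks claw sequence, timed combo finishers or missile hits.
; A camera-facing widget shows input prompts and combo feedback.
; Death fades the widget and uses Niagara bursts with a timeline squash and material swap.
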(event `Die`
  (`/Engine/EditorBlueprintResources/StandardMacros.DoOnce` false
    (:`Completed`
      (`NiagaraFunctionLibrary.SpawnSystemAtLocation` "/Game/VFX/NiagaraSystem/Mick/LilCrab/NS_LitlCrab_Death.NS_LitlCrab_Death" (`SceneComponent.K2_GetComponentLocation` (`self.Mesh`)) (struct) (10.0 10.0 10.0))
      (bind (_direction _newtrack_0) (`Timeline|Timeline_0` :!via `PlayFromStart`)
        (:`Update`
          (`SceneComponent.SetWorldScale3D` (`self.Mesh`) (`KismetMathLibrary.VLerp` (47.5 47.5 47.5) (12.0 6.0 6.0) _newtrack_0))
          (if (>= _newtrack_0 0.5)
            (`/Engine/EditorBlueprintResources/StandardMacros.DoOnce` false
              (:`Completed`
                (`NiagaraFunctionLibrary.SpawnSystemAtLocation` "/Game/VFX/NiagaraSystem/Mick/LilCrab/NS_LitlCrab_Death.NS_LitlCrab_Death" (`SceneComponent.K2_GetComponentLocation` (`self.Mesh`)) (struct) (10.0 10.0 10.0))
                (`PrimitiveComponent.SetMaterial` (`self.Mesh`) 0 "/Game/Characters/Enemy/TrashMob/Blob/Textures/NiceBlob/M_NiceBlob.M_NiceBlob")))))))))

(event `self.ReceiveBeginPlay`
  (bind _returnvalue (`KismetMaterialLibrary.CreateDynamicMaterialInstance` "/Game/Characters/Enemy/TrashMob/Blob/Mesh/M_Blob_Inst.M_Blob_Inst"))
  (bind _output_get (set `self.Materiau` _returnvalue))
  (`PrimitiveComponent.SetMaterial` (`self.Mesh`) 0 _output_get))

(event `self.ReceiveTick`
  (params (DeltaSeconds :type "Float (single-precision)"))
  (bind _asbp_sea_watcher (cast `/Game/Characters/SeaWatcher/BP_SeaWatcher` (`GameplayStatics.GetPlayerCharacter` 0)))
  (`SceneComponent.K2_SetWorldRotation` (`self.Widget`) (`KismetMathLibrary.Conv_VectorToRotator` (`KismetMathLibrary.NegateVector` (`SceneComponent.GetForwardVector` (`/Game/Characters/SeaWatcher/BP_SeaWatcher.Camera` _asbp_sea_watcher)))) false false))

(event `ResetHit`
  (goto _label :!via `Reset`))

(event `/Game/GeneralSettings/Int_Hittable.GetHit`
  (params (Dammage :type "Float (double-precision)") (PositionHited :type "Vector Structure") (ComboEnd :type Boolean) (`Missile?` :type Boolean) (ClawAttack :type Boolean))
  (`/Engine/EditorBlueprintResources/StandardMacros.DoOnce` false :!label _label
    (:`Completed`
      (`|SpawnActorFromClass` "/Game/VFX/Blueprint/BP_Zlag_test_2.BP_Zlag_test_2_C" (`KismetMathLibrary.MakeTransform` (`SceneComponent.K2_GetComponentLocation` (`self.Mesh`))) "Undefined" "OverrideRootScale" null null)
      (bind _asbp_sea_watcher (cast `/Game/Characters/SeaWatcher/BP_SeaWatcher` (`GameplayStatics.GetPlayerCharacter` 0)))
      (set `/Game/Characters/SeaWatcher/BP_SeaWatcher.Jauge` (+ (`/Game/Characters/SeaWatcher/BP_SeaWatcher.Jauge` _asbp_sea_watcher) 5.0) _asbp_sea_watcher)
      (`/Game/UI/UI_Interface.PlayFlip` (`/Game/Characters/SeaWatcher/BP_SeaWatcher.UI_Ref` _asbp_sea_watcher))
      (switch `/Game/Characters/Enemy/TrashMob/E_TutorialType` (`self.Type`)
        (:`NewEnumerator0`
          (`self.CheckAttack` ClawAttack)
          (bind (_direction _newtrack_0) (`Timeline|Timeline_1` :!via `PlayFromStart` :!label _label_2)
            (:`Update`
              (`MaterialInstanceDynamic.SetScalarParameterValue` (`self.Materiau`) "Glow" _newtrack_0))))
        (:`NewEnumerator1`
          (`self.CheckCombo` ComboEnd)
          (goto _label_2 :!via `PlayFromStart`))
        (:`NewEnumerator2`
          (`self.CheckUlti` `Missile?`)
          (goto _label_2 :!via `PlayFromStart`))))))

(event `ResetWid`
  (set `self.NewVar_1` false)
  (bind _aswid_hpblob_afrappe_1 (cast `/Game/UI/WID_HPBlobAFrappe1` (`WidgetComponent.GetWidget` (`self.Widget`)) :!label _label_3))
  (bind _image (`/Game/UI/WID_HPBlobAFrappe1.Image` _aswid_hpblob_afrappe_1))
  (`Widget.SetRenderOpacity` _image 0.3)
  (`Widget.SetRenderOpacity` (`/Game/UI/WID_HPBlobAFrappe1.Image_1` _aswid_hpblob_afrappe_1) 0.3)
  (`Image.SetBrushTintColor` _image (make `SlateColor` (`KismetMathLibrary.SelectColor` (struct :`R` 0.40625 :`G` 0.078818 :`B` 0.0586 :`A` 1.0) (struct :`R` 0.310215 :`G` 1.0 :`B` 0.560211 :`A` 1.0) (not (`self.NewVar_1`)))))
  (`Image.SetBrushTintColor` (`/Game/UI/WID_HPBlobAFrappe1.Image_1` _aswid_hpblob_afrappe_1) (make `SlateColor` (`KismetMathLibrary.SelectColor` (struct :`R` 0.40625 :`G` 0.078818 :`B` 0.0586 :`A` 1.0) (struct :`R` 0.310215 :`G` 1.0 :`B` 0.560211 :`A` 1.0) (not (`self.NewVar_1`)))))
  (`Image.SetBrushTintColor` (`/Game/UI/WID_HPBlobAFrappe1.Image_0` _aswid_hpblob_afrappe_1) (make `SlateColor` (`KismetMathLibrary.SelectColor` (struct :`R` 0.40625 :`G` 0.078818 :`B` 0.0586 :`A` 1.0) (struct :`R` 0.310215 :`G` 1.0 :`B` 0.560211 :`A` 1.0) (not (`self.NewVar_1`)))))
  (`KismetSystemLibrary.Delay` 0.2)
  (`Image.SetBrushTintColor` _image (make `SlateColor` (struct :`R` 1.0 :`G` 1.0 :`B` 1.0 :`A` 1.0)))
  (`Image.SetBrushTintColor` (`/Game/UI/WID_HPBlobAFrappe1.Image_1` _aswid_hpblob_afrappe_1) (make `SlateColor` (struct :`R` 1.0 :`G` 1.0 :`B` 1.0 :`A` 1.0)))
  (`Image.SetBrushTintColor` (`/Game/UI/WID_HPBlobAFrappe1.Image_0` _aswid_hpblob_afrappe_1) (make `SlateColor` (struct :`R` 1.0 :`G` 1.0 :`B` 1.0 :`A` 1.0))))

(event `GoodWid`
  (set `self.NewVar_1` true)
  (goto _label_3))

(fn `CheckAttack`
  (params (AttackType :type Boolean))
  (if (and AttackType (== (`self.Count`) 0))
    (set `self.Count` 1)
    (bind _aswid_hpblob_afrappe (cast `/Game/UI/WID_HPBlobAFrappe` (`WidgetComponent.GetWidget` (`self.Widget`))))
    (`Image.SetBrushFromTexture` (`/Game/UI/WID_HPBlobAFrappe.Image_0` _aswid_hpblob_afrappe) "/Game/UI/Texture/XboxSeriesX_Y.XboxSeriesX_Y" false)
    (elif (and (not AttackType) (== (`self.Count`) 1))
      (`self.Die`)
      (bind _aswid_hpblob_afrappe_2 (cast `/Game/UI/WID_HPBlobAFrappe` (`WidgetComponent.GetWidget` (`self.Widget`))))
      (`UserWidget.PlayAnimationForward` _aswid_hpblob_afrappe_2 (`/Game/UI/WID_HPBlobAFrappe.FadeOut` _aswid_hpblob_afrappe_2) 1.0 false))))

(fn `CheckCombo`
  (params (EndCombo :type Boolean))
  (bind _newvar_0 (`self.NewVar_0`))
  (if EndCombo
    (bind _result (`/Engine/EditorBlueprintResources/StandardMacros.IncrementInt` (`self.Count`))
      (:`  `
        (`KismetSystemLibrary.K2_ClearAndInvalidateTimerHandle` (`self.NewVar_0`))
        (`self.GoodWid`)
        (if (>= _result 3)
          (`self.Die`)
          (bind _aswid_hpblob_afrappe_1 (cast `/Game/UI/WID_HPBlobAFrappe1` (`WidgetComponent.GetWidget` (`self.Widget`))))
          (`UserWidget.PlayAnimationForward` _aswid_hpblob_afrappe_1 (`/Game/UI/WID_HPBlobAFrappe1.FadeOut` _aswid_hpblob_afrappe_1) 1.0 false))))
    (else
      (bind _aswid_hpblob_afrappe_1_2 (cast `/Game/UI/WID_HPBlobAFrappe1` (`WidgetComponent.GetWidget` (`self.Widget`))))
      (if (`KismetSystemLibrary.K2_IsValidTimerHandle` _newvar_0)
        (`KismetSystemLibrary.K2_ClearAndInvalidateTimerHandle` _newvar_0))
      (bind _returnvalue (`KismetSystemLibrary.K2_SetTimerDelegate` (`|CreateDelegate` :!event `ResetWid`) 0.7))
      (set `self.NewVar_0` _returnvalue)
      (if (== (`Widget.GetRenderOpacity` (`/Game/UI/WID_HPBlobAFrappe1.Image` _aswid_hpblob_afrappe_1_2)) 1.0)
        (`Widget.SetRenderOpacity` (`/Game/UI/WID_HPBlobAFrappe1.Image_1` _aswid_hpblob_afrappe_1_2) 1.0)
        (else
          (`Widget.SetRenderOpacity` (`/Game/UI/WID_HPBlobAFrappe1.Image` _aswid_hpblob_afrappe_1_2) 1.0))))))

(fn `CheckUlti`
  (params (Ulti :type Boolean))
  (if Ulti
    (`self.Die`)
    (bind _aswid_hpblob_afrappe_2 (cast `/Game/UI/WID_HPBlobAFrappe2` (`WidgetComponent.GetWidget` (`self.Widget`))))
    (`UserWidget.PlayAnimationForward` _aswid_hpblob_afrappe_2 (`/Game/UI/WID_HPBlobAFrappe2.FadeOut` _aswid_hpblob_afrappe_2) 1.0 false)))

(fn `UserConstructionScript`)