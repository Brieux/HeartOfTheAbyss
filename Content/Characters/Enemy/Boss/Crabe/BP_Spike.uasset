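; BP_Spike is a Crab boss hazard that rises as a Niagara effect, hurts BP_SeaWatcher on contact and can later explode.
; Spawning staggers the effect, enables capsule collision in timed stages, then pauses Niagara mid-animation.
; xplodeZlag resumes it and sphere-traces for the player, applying balancer-driven damage.
; Otherwise it shakes the camera and has a coin-flip chance to spawn a triggered LilCrab before destroying itself.
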(event `xplodeZlag`
  (bind _returnvalue (`self.K2_GetActorLocation`))
  (bind _balancerref_dammageapply (break `/Game/GeneralSettings/Struct_DammageApplyOnPlayer` (`self.balancerRef`)))
  (`NiagaraComponent.SetPaused` (`self.Niagara`) false)
  (`KismetSystemLibrary.Delay` (`KismetMathLibrary.RandomFloatInRange` 0.4 0.55))
  (bind (_outhit _returnvalue_2) (`KismetSystemLibrary.SphereTraceSingleForObjects` _returnvalue _returnvalue 750.0 (`|MakeArray` "ObjectTypeQuery3" :!type "EObjectTypeQuery Enum")))
  (if _returnvalue_2
    (bind _asbp_sea_watcher (cast `/Game/Characters/SeaWatcher/BP_SeaWatcher` (`.HitActor` (`GameplayStatics.BreakHitResult` _outhit)))
      (:`then`
        (`GameplayStatics.ApplyDamage` _asbp_sea_watcher (`BlueprintMapLibrary.Map_Find` _balancerref_dammageapply "NewEnumerator15"))
        (`/Game/Characters/SeaWatcher/BP_SeaWatcher.ResetDammage` _asbp_sea_watcher)
        (`KismetSystemLibrary.Delay` 2.5)
        (`self.K2_DestroyActor`))
      (:`CastFailed`
        (`self.SpawnOneCrab` :!label _label)
        (`/Game/Characters/SeaWatcher/BP_SeaWatcher.PlayXplosionCameraShake` (cast `/Game/Characters/SeaWatcher/BP_SeaWatcher` (`GameplayStatics.GetPlayerCharacter` 0) :!pure true))
        (`self.K2_DestroyActor`)))
    (else
      (`KismetSystemLibrary.Delay` 2.5)
      (goto _label))))

(event `self.ReceiveBeginPlay`
  (`KismetSystemLibrary.K2_SetTimerDelegate` (delegate `spawn`) (`KismetMathLibrary.RandomFloatInRange` 0.0 0.7)))

(event `spawn`
  (bind _capsule (`self.Capsule`))
  (`ActorComponent.Activate` (`self.Niagara`) false)
  (`PrimitiveComponent.SetCollisionEnabled` _capsule "NoCollision")
  (`KismetSystemLibrary.Delay` 2.75)
  (`PrimitiveComponent.SetCollisionEnabled` _capsule "QueryOnly")
  (`KismetSystemLibrary.Delay` 2.25)
  (`PrimitiveComponent.SetCollisionResponseToChannel` (`self.Capsule`) "ECC_GameTraceChannel5" "ECR_Block")
  (`NiagaraComponent.SetPaused` (`self.Niagara`) true))

(event `SpawnOneCrab`
  (if (`KismetMathLibrary.RandomBool`)
    (bind _returnvalue (`|SpawnActorFromClass` "/Game/Characters/Enemy/TrashMob/Ptit_Crab/BP_LilCrab.BP_LilCrab_C" (`KismetMathLibrary.MakeTransform` (`self.K2_GetActorLocation`)) "AdjustIfPossibleButAlwaysSpawn" "OverrideRootScale" null null))
    (bind _asaic_intelligent_crab (cast `/Game/AI/AIC_IntelligentCrab` (`Pawn.GetController` _returnvalue)))
    (`/Game/AI/AIC_IntelligentCrab.Trigger` _asaic_intelligent_crab)))

(event `self.Capsule.OnComponentBeginOverlap`
  (params (OverlappedComponent :type "PrimitiveComponent Object Reference") (OtherActor :type "Actor Object Reference") (OtherComp :type "PrimitiveComponent Object Reference") (OtherBodyIndex :type Integer) (bFromSweep :type Boolean) (SweepResult :type "HitResult Structure (by ref)"))
  (bind _balancerref_dammageapply (break `/Game/GeneralSettings/Struct_DammageApplyOnPlayer` (`self.balancerRef`)))
  (bind _asbp_sea_watcher (cast `/Game/Characters/SeaWatcher/BP_SeaWatcher` OtherActor))
  (`GameplayStatics.ApplyDamage` _asbp_sea_watcher (`BlueprintMapLibrary.Map_Find` _balancerref_dammageapply "NewEnumerator16"))
  (`KismetSystemLibrary.DelayUntilNextTick`)
  (`/Game/Characters/SeaWatcher/BP_SeaWatcher.ResetDammage` _asbp_sea_watcher))

(fn `UserConstructionScript`)