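; Falling bomb from the Crabe boss folder that explodes on landscape or static mesh contact and self-destructs on a timeout.
; On spawn it randomizes gravity and, if set to follow, repositions high above the player after a delay with random offset.
; Each tick, a downward trace places a warning decal, scaling its dynamic material's brightness and radius by ground distance.
; Explosion sphere-traces for BP_SeaWatcher, applying damage from that actor's balancing data.
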(event `self.ReceiveBeginPlay`
  (bind (_returnvalue_x _returnvalue_y) (`KismetMathLibrary.BreakVector` (`self.K2_GetActorLocation` (`GameplayStatics.GetPlayerPawn` 0))))
  (`|ExecutionSequence`
    (:`then_0`
      (set `self.Condition` false)
      (bind _returnvalue (`DecalComponent.CreateDynamicMaterialInstance` (`self.Decal`)))
      (set `self.NewVar` _returnvalue)
      (`self.K2_SetActorLocation` (`self.New Location`))
      (`KismetSystemLibrary.Delay` 0.2)
      (set `ProjectileMovementComponent.ProjectileGravityScale` (`KismetMathLibrary.RandomFloatInRange` 1.4 1.6) (`self.ProjectileMovement`))
      (if (`self.needToBeFollowing`)
        (`KismetSystemLibrary.Delay` (+ (`KismetMathLibrary.RandomFloat`) (/ 2.0 (`self.int`))))
        (`self.K2_SetActorLocation` (`KismetMathLibrary.MakeVector` (+ _returnvalue_x (`KismetMathLibrary.RandomFloatInRange` -50.0 50.0)) (+ _returnvalue_y (`KismetMathLibrary.RandomFloatInRange` -50.0 50.0)) (`KismetMathLibrary.RandomFloatInRange` 2850.0 2950.0)))
        (set `self.Condition` true)
        (else
          (set `self.Condition` true))))
    (:`then_1`
      (`KismetSystemLibrary.Delay` 4.0)
      (`self.K2_DestroyActor`))))

(event `self.ReceiveTick`
  (params (DeltaSeconds :type "Float (single-precision)"))
  (bind _returnvalue (`self.K2_GetActorLocation`))
  ;[0.116 1 0] SPAWN DECAL PREVISUALISATION
  (if (`self.Condition`)
    (bind (_outhit _returnvalue_2) (`KismetSystemLibrary.LineTraceSingle` _returnvalue (+ _returnvalue (* (0.0 0.0 -1.0) 10000.0)) "TraceTypeQuery1"))
    (if _returnvalue_2
      (`SceneComponent.K2_SetWorldLocation` (`self.Decal`) (`.Location` (`GameplayStatics.BreakHitResult` _outhit)) false false)
      (set `self.DistanceToSol` (`KismetMathLibrary.NormalizeToRange` (`.Distance` (`GameplayStatics.BreakHitResult` _outhit)) 0.0 9000.0))
      (`self.VFXDecalMATERIAL`))))

(event `self.Sphere.OnComponentHit`
  (params (HitComponent :type "PrimitiveComponent Object Reference") (OtherActor :type "Actor Object Reference") (OtherComp :type "PrimitiveComponent Object Reference") (NormalImpulse :type "Vector Structure") (Hit :type "HitResult Structure (by ref)"))
  ;[1 0.7109 0] COLLISION WITH GROUND
  (cast `/Game/Characters/Enemy/Boss/Crabe/BP_BombeInTheSky` OtherActor
    (:`CastFailed`
      (cast `LandscapeProxy` OtherActor
        (:`then`
          _)
        (:`CastFailed`
          (cast `LandscapeComponent` OtherComp
            (:`then`
              _)
            (:`CastFailed`
              (cast `Landscape` OtherActor
                (:`then`
                  _)
                (:`CastFailed`
                  (cast `StaticMeshActor` OtherActor
                    (:`then`
                      _)
                    (:`CastFailed`
                      (cast `StaticMeshComponent` OtherComp)))))))))
      (`self.Explosion`))))

(event `VFXDecalMATERIAL`
  (bind _newvar (`self.NewVar`))
  ;[0.5 0 1] VFX DECAL PREVISUALISATION
  (`MaterialInstanceDynamic.SetScalarParameterValue` _newvar "BrightnessBT" (`KismetMathLibrary.MapRangeClamped` (`self.DistanceToSol`) 0.0 1.0 10.0 1.0))
  (`MaterialInstanceDynamic.SetScalarParameterValue` _newvar "BrightnessRGE" (`KismetMathLibrary.MapRangeClamped` (`self.DistanceToSol`) 0.0 1.0 2.0 1.0))
  (`MaterialInstanceDynamic.SetScalarParameterValue` _newvar "Radius" (`KismetMathLibrary.MapRangeClamped` (`self.DistanceToSol`) 0.0 1.0 0.5)))

(event `Explosion`
  (bind _returnvalue (`self.K2_GetActorLocation`))
  ;[1 0 0] EXPLOSION DAMAGE
  (bind _outhits (`KismetSystemLibrary.SphereTraceMultiForObjects` :`Start` _returnvalue :`End` _returnvalue :`Radius` 738.0 :`ObjectTypes` (`|MakeArray` "ObjectTypeQuery11" :!type "EObjectTypeQuery Enum") :`DrawTime` 2.0))
  (for _array_element _outhits
    (bind _asbp_sea_watcher (cast `/Game/Characters/SeaWatcher/BP_SeaWatcher` (`.HitActor` (`GameplayStatics.BreakHitResult` _array_element))))
    (bind _balancergethit_dammageapply (break `/Game/GeneralSettings/Struct_DammageApplyOnPlayer` (`/Game/Characters/SeaWatcher/BP_SeaWatcher.BalancerGetHit` _asbp_sea_watcher)))
    (`GameplayStatics.ApplyDamage` _asbp_sea_watcher (`BlueprintMapLibrary.Map_Find` _balancergethit_dammageapply "NewEnumerator20"))
    (`/Game/Characters/SeaWatcher/BP_SeaWatcher.ResetDammage` _asbp_sea_watcher)
    (`KismetSystemLibrary.Delay` 0.3 :!label _label)
    (`self.K2_DestroyActor`))
  (goto _label))

(fn `UserConstructionScript`)