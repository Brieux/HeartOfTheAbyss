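; Crab boss "Eugene": tracks health and provides projectile, hammer wave, spike and rush-damage attacks, coordinated with AIC_Crabe through range and phase state.
; Hits play VFX and camera shake, mapping the nearest bone or its parents to AnimBP hit-zone flags.
; At zero health it summons timed little-crab waves, refills, then alternates between restarting AI in a new phase and a placeholder flee.
; Tick smooths facing and feeds player positions to Niagara.
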(event `LifeUp`
  (bind (_direction _newtrack_0) (`Timeline|Timeline_1` :!via `PlayFromStart`)
    (:`Update`
      (set `self.PV` (`KismetMathLibrary.Lerp` 0.0 (`self.PVMax`) _newtrack_0)))))

(event `self.ReceiveBeginPlay`
  (bind _returnvalue (`KismetMaterialLibrary.CreateDynamicMaterialInstance` "/Game/Characters/Enemy/Boss/Crabe/Materials/M_Eugene_Inst.M_Eugene_Inst"))
  (bind _output_get (set `self.Mat` _returnvalue))
  (`PrimitiveComponent.SetMaterial` (`self.SkeletalMesh`) 0 _output_get))

(event `ZlagMatEffect`
  (bind _skeletalmesh (`self.SkeletalMesh`))
  ;[1 1 1] Désactivé pour le moment (modifs sur le matériau crabe 02)
  (`MeshComponent.SetScalarParameterValueOnMaterials` _skeletalmesh "Quantity" (/ (`self.PV`) 500.0))
  (`MeshComponent.SetScalarParameterValueOnMaterials` _skeletalmesh "Weigth" (/ (`self.PV`) 250.0)))

(event `self.ReceiveTick`
  (params (DeltaSeconds :type "Float (single-precision)"))
  (`self.Smooth Rotation`)
  (`self.TargetPosition`)
  (`self.SpawnPosition`)
  (`|ExecutionSequence`
    (:`then_0`
      (for _array_element (`self.NS`)
        (bind _asbp_sea_watcher (cast `/Game/Characters/SeaWatcher/BP_SeaWatcher` (`GameplayStatics.GetPlayerCharacter` 0)))
        (`/Engine/EditorBlueprintResources/StandardMacros.IsValid` _array_element
          (:`Is Valid`
            (`NiagaraComponent.SetVariablePosition` _array_element "User.Attractor Position" (`SceneComponent.GetSocketLocation` (`Character.Mesh` _asbp_sea_watcher) "Bind_PearlSocket"))))))
    (:`then_1`
      (set `self.PV_Buffer` (`KismetMathLibrary.FInterpTo_Constant` (`self.PV_Buffer`) (`self.PV`) (`GameplayStatics.GetWorldDeltaSeconds`) 30.0)))))

(event `Fuite`
  (`KismetSystemLibrary.PrintString` "Hello"))

(event `Summon`
  ;[0.4453 1 0] Inovcation
  (set `self.CanDie` false)
  (set `self.Phase` "NewEnumerator3")
  (set `self.CompteurInvoq` 0)
  (bind _returnvalue (`KismetSystemLibrary.K2_SetTimerDelegate` (delegate `Invocation`) 2.0 true))
  (set `self.SummonHandler` _returnvalue)
  (for _array_element (`self.SpawnToActive`)
    (`/Game/Characters/Enemy/TrashMob/BP_SpawnerACrab.AddSpawn` _array_element (`KismetMathLibrary.RandomIntegerInRange` 2 7))))

(event `Invocation`
  ;[0.4453 1 0] Inovcation
  (if (< (`self.CompteurInvoq`) 6)
    (bind _result (`/Engine/EditorBlueprintResources/StandardMacros.IncrementInt` (`self.CompteurInvoq`))
      (:`  `
        (set `self.CompteurInvoq` _result)
        (`|PlayMontage` (`self.SkeletalMesh`) "/Game/Characters/Enemy/Boss/Crabe/Anim/AM_Invocation.AM_Invocation"
          (:`then`
            (for _index (range 5)
              (bind (_returnvalue_location _returnvalue_rotation) (`KismetMathLibrary.BreakTransform` (`SceneComponent.K2_GetComponentToWorld` (`|GetArrayItem` (`|MakeArray` (`self.Scene`) (`self.Scene1`) (`self.Scene2`) (`self.Scene3`) (`self.Scene4`)) _index))))
              (bind _returnvalue (`|SpawnActorFromClass` "/Game/Characters/Enemy/TrashMob/Ptit_Crab/BP_LilCrab.BP_LilCrab_C" (`KismetMathLibrary.MakeTransform` _returnvalue_location _returnvalue_rotation) "AdjustIfPossibleButAlwaysSpawn" "OverrideRootScale" null null))
              (bind _asaic_enemy (cast `/Game/AI/AIC_Enemy` (`self.GetController` _returnvalue)))
              (`/Game/AI/AIC_Enemy.Trigger` _asaic_enemy))))))
    (else
      (`KismetSystemLibrary.K2_ClearAndInvalidateTimerHandle` (`self.SummonHandler`))
      (bind (_direction _newtrack_0) (`Timeline|Timeline_2` :!via `PlayFromStart`)
        (:`Update`
          (set `self.PV` (`KismetMathLibrary.Lerp` 0.0 (`self.PVMax`) _newtrack_0)))
        (:`Finished`
          (`/Engine/EditorBlueprintResources/StandardMacros.FlipFlop`
            (:`A`
              (set `self.Phase` "NewEnumerator1")
              (bind _asaic_crabe (cast `/Game/AI/AIC_Crabe` (`self.GetController`)))
              (set `/Game/AI/AIC_Crabe.Phase&Comportement` "NewEnumerator1" _asaic_crabe)
              (`/Game/AI/AIC_Crabe.SetPhase` _asaic_crabe)
              (`/Game/AI/AIC_Crabe.Triggering` _asaic_crabe)
              (set `self.CanDie` true))
            (:`B`
              (`self.Fuite`))))))))

(event `GlowingAttacking`
  ;[1 1 1] GLOWING ATTACKING
  (set `self.Attack?` true)
  (bind (_direction _glowingattack_value) (`Timeline|Timeline_GlowingAttacking` :!label _label)
    (:`Update`
      (`MeshComponent.SetScalarParameterValueOnMaterials` (`self.SkeletalMesh`) "EmissivPic" _glowingattack_value))
    (:`Finished`
      (if (`self.Attack?`)
        (set `self.Attack?` false)
        (`KismetSystemLibrary.Delay` 2.0)
        (`self.StopGlowingAttacking`)))))

(event `StopGlowingAttacking`
  ;[1 1 1] GLOWING ATTACKING
  (goto _label :!via `Reverse`))

(event `VFXZlagClaw`
  (bind (_returnvalue_x _returnvalue_y _returnvalue_z) (`KismetMathLibrary.BreakVector` (`SceneComponent.GetSocketLocation` (`self.SkeletalMesh`) "Bind_Dactyle_End_RSocket")))
  ;[0.6213 0 1] VFX ACTIVATION
  (`NiagaraFunctionLibrary.SpawnSystemAtLocation` "/Game/VFX/NiagaraSystem/Mick/BossCrab/NS_SpikeClaw_SandEffect.NS_SpikeClaw_SandEffect" (`KismetMathLibrary.MakeVector` _returnvalue_x _returnvalue_y (+ _returnvalue_z 130.0))))

(event `Spike`
  ;[1 1 1] Spike
  (`|ExecutionSequence`
    (:`then_0`
      (bind _asbp_sea_watcher (cast `/Game/Characters/SeaWatcher/BP_SeaWatcher` (`GameplayStatics.GetPlayerCharacter` 0)))
      (for _array_element (`|MakeArray` (+ (`SceneComponent.K2_GetComponentLocation` (`/Game/Characters/SeaWatcher/BP_SeaWatcher.PlacementRoche01` _asbp_sea_watcher)) (`self.Random in Z Location Spike`)) (+ (`SceneComponent.K2_GetComponentLocation` (`/Game/Characters/SeaWatcher/BP_SeaWatcher.PlacementRoche02` _asbp_sea_watcher)) (`self.Random in Z Location Spike`)) (+ (`SceneComponent.K2_GetComponentLocation` (`/Game/Characters/SeaWatcher/BP_SeaWatcher.PlacementRoche03` _asbp_sea_watcher)) (`self.Random in Z Location Spike`)) (+ (`SceneComponent.K2_GetComponentLocation` (`/Game/Characters/SeaWatcher/BP_SeaWatcher.PlacementRoche04` _asbp_sea_watcher)) (`self.Random in Z Location Spike`)))
        (`|SpawnActorFromClass` "/Game/Characters/Enemy/Boss/Crabe/BP_Spike.BP_Spike_C" (`KismetMathLibrary.MakeTransform` _array_element) "Undefined" "OverrideRootScale" null null)))
    (:`then_1`
      (for _array_element_2 (`|MakeArray` (+ (`SceneComponent.K2_GetComponentLocation` (`self.PlacementRocheCrabe1`)) (`self.Random in Z Location Spike`)) (+ (`SceneComponent.K2_GetComponentLocation` (`self.PlacementRocheCrabe2`)) (`self.Random in Z Location Spike`)) (+ (`SceneComponent.K2_GetComponentLocation` (`self.PlacementRocheCrabe3`)) (`self.Random in Z Location Spike`)) (+ (`SceneComponent.K2_GetComponentLocation` (`self.PlacementRocheCrabe4`)) (`self.Random in Z Location Spike`)))
        (`|SpawnActorFromClass` "/Game/Characters/Enemy/Boss/Crabe/BP_Spike.BP_Spike_C" (`KismetMathLibrary.MakeTransform` _array_element_2) "Undefined" "OverrideRootScale" null null)))))

(event `self.MidRange.OnComponentBeginOverlap`
  (params (OverlappedComponent :type "PrimitiveComponent Object Reference") (OtherActor :type "Actor Object Reference") (OtherComp :type "PrimitiveComponent Object Reference") (OtherBodyIndex :type Integer) (bFromSweep :type Boolean) (SweepResult :type "HitResult Structure (by ref)"))
  ;[0 0.4617 1] RangeDetection
  (cast `/Game/Characters/SeaWatcher/BP_SeaWatcher` OtherActor)
  (set `self.RangeToPlayer` "NewEnumerator1"))

(event `self.MidRange.OnComponentEndOverlap`
  (params (OverlappedComponent :type "PrimitiveComponent Object Reference") (OtherActor :type "Actor Object Reference") (OtherComp :type "PrimitiveComponent Object Reference") (OtherBodyIndex :type Integer))
  ;[0 0.4617 1] RangeDetection
  (cast `/Game/Characters/SeaWatcher/BP_SeaWatcher` OtherActor)
  (set `self.RangeToPlayer` "NewEnumerator2"))

(event `Shoot`
  (bind _returnvalue (`self.K2_GetActorLocation`))
  (bind _returnvalue_2 (`KismetMathLibrary.FindLookAtRotation` _returnvalue (`self.K2_GetActorLocation` (`GameplayStatics.GetPlayerCharacter` 0))))
  ;[1 0.1393 0] Attaque
  (`Controller.SetControlRotation` (`self.GetController`) _returnvalue_2)
  (bind _returnvalue_3 (`|SpawnActorFromClass` "/Game/Characters/Enemy/Boss/Crabe/BP_Pistolet.BP_Pistolet_C" (`KismetMathLibrary.MakeTransform` _returnvalue _returnvalue_2 (20.0 20.0 20.0)) "Undefined" "OverrideRootScale" null self null))
  (set `MovementComponent.Velocity` (* (`KismetMathLibrary.GetDirectionUnitVector` (`self.K2_GetActorLocation` _returnvalue_3) (`self.K2_GetActorLocation` (`GameplayStatics.GetPlayerCharacter` 0))) 10000.0) (`/Game/Characters/Enemy/Boss/Crabe/BP_Pistolet.ProjectileMovement` _returnvalue_3)))

(event `self.Cac.OnComponentBeginOverlap`
  (params (OverlappedComponent :type "PrimitiveComponent Object Reference") (OtherActor :type "Actor Object Reference") (OtherComp :type "PrimitiveComponent Object Reference") (OtherBodyIndex :type Integer) (bFromSweep :type Boolean) (SweepResult :type "HitResult Structure (by ref)"))
  ;[0 0.4617 1] RangeDetection
  (cast `/Game/Characters/SeaWatcher/BP_SeaWatcher` OtherActor)
  (set `self.RangeToPlayer` "NewEnumerator0"))

(event `CoupDeMarteau`
  (bind (_returnvalue_x _returnvalue_y _returnvalue_z) (`KismetMathLibrary.BreakVector` (`SceneComponent.GetSocketLocation` (`self.SkeletalMesh`) "Martro")))
  (bind (_returnvalue_x_2 _returnvalue_y_2 _returnvalue_z_2) (`KismetMathLibrary.BreakVector` (`SceneComponent.GetSocketLocation` (`self.SkeletalMesh`) "Martro")))
  (bind _returnvalue (+ _returnvalue_z_2 130.0))
  ;[1 0.1393 0] Attaque
  (`NiagaraFunctionLibrary.SpawnSystemAtLocation` "/Game/VFX/NiagaraSystem/Mick/BossCrab/NS_Hammer_SandEffect.NS_Hammer_SandEffect" (`KismetMathLibrary.MakeVector` _returnvalue_x_2 _returnvalue_y_2 _returnvalue))
  (`NiagaraFunctionLibrary.SpawnSystemAtLocation` "/Game/VFX/NiagaraSystem/Mick/BossCrab/NS_Hammer_Zlag.NS_Hammer_Zlag" (`KismetMathLibrary.MakeVector` _returnvalue_x_2 _returnvalue_y_2 _returnvalue))
  (bind _returnvalue_2 (`|SpawnActorFromClass` "/Game/VFX/Crab/BP_CrabWave.BP_CrabWave_C" (`KismetMathLibrary.MakeTransform` (`KismetMathLibrary.MakeVector` _returnvalue_x _returnvalue_y (+ _returnvalue_z 130.0))) "AlwaysSpawn" "OverrideRootScale" null self null))
  (`/Game/VFX/Crab/BP_CrabWave.Wave_3` _returnvalue_2))

(event `self.Cac.OnComponentEndOverlap`
  (params (OverlappedComponent :type "PrimitiveComponent Object Reference") (OtherActor :type "Actor Object Reference") (OtherComp :type "PrimitiveComponent Object Reference") (OtherBodyIndex :type Integer))
  ;[0 0.4617 1] RangeDetection
  (cast `/Game/Characters/SeaWatcher/BP_SeaWatcher` OtherActor)
  (set `self.RangeToPlayer` "NewEnumerator1"))

(event `Tremblement`
  (params (TestLocation :type "Vector Structure"))
  (bind (_bonelocation _returnvalue) (`SkinnedMeshComponent.FindClosestBone_K2` (`self.SkeletalMesh`) TestLocation 0.0 false))
  (bind _returnvalue_2 (`SkinnedMeshComponent.GetParentBone` (`self.SkeletalMesh`) _returnvalue))
  (bind _returnvalue_3 (`SkinnedMeshComponent.GetParentBone` (`self.SkeletalMesh`) _returnvalue_2))
  ;[0 1 0.8115] Dammage System
  (bind _asapb_definitive_edition_eugene (cast `/Game/Characters/Enemy/Boss/Crabe/APB_DefinitiveEditionEugene` (`SkeletalMeshComponent.GetAnimInstance` (`self.SkeletalMesh`))))
  (`/Game/Characters/Enemy/Boss/Crabe/APB_DefinitiveEditionEugene.GetHit` _asapb_definitive_edition_eugene)
  (if (`KismetArrayLibrary.Array_Contains` (`self.SkeletalToMove`) _returnvalue)
    (`self.ValidateHitShake` _returnvalue)
    (elif (`KismetArrayLibrary.Array_Contains` (`self.SkeletalToMove`) _returnvalue_2)
      (`self.ValidateHitShake` _returnvalue_2)
      (elif (`KismetArrayLibrary.Array_Contains` (`self.SkeletalToMove`) _returnvalue_3)
        (`self.ValidateHitShake` _returnvalue_3)))))

(event `self.ReceiveAnyDamage`
  (params (Damage :type "Float (single-precision)") (DamageType :type "DamageType Object Reference") (InstigatedBy :type "Controller Object Reference") (DamageCauser :type "Actor Object Reference"))
  ;[0 1 0.8115] Dammage System
  (bind _output_get (set `self.PV` (- (`self.PV`) Damage)))
  (if (<= _output_get 0.0)
    (bind _asaic_crabe (cast `/Game/AI/AIC_Crabe` (`self.GetController`) :!label _label_2))
    (set `/Game/AI/AIC_Crabe.Phase&Comportement` "NewEnumerator3" _asaic_crabe)
    (`self.Summon`)))

(event `self.ReceiveRadialDamage`
  (params (DamageReceived :type "Float (single-precision)") (DamageType :type "DamageType Object Reference") (Origin :type "Vector Structure") (HitInfo :type "HitResult Structure (by ref)") (InstigatedBy :type "Controller Object Reference") (DamageCauser :type "Actor Object Reference"))
  ;[0 1 0.8115] Dammage System
  (`NiagaraFunctionLibrary.SpawnSystemAtLocation` "/Game/VFX/NS_Impact.NS_Impact" (stale `/Game/GeneralSettings/Int_Hittable.GetHit` PositionHited) :!label _label_3)
  (`self.Tremblement` (stale `/Game/GeneralSettings/Int_Hittable.GetHit` PositionHited))
  (bind _asbp_sea_watcher (cast `/Game/Characters/SeaWatcher/BP_SeaWatcher` (`GameplayStatics.GetPlayerCharacter` 0)))
  (`GameplayStatics.PlayWorldCameraShake` "/Game/GeneralSettings/BP_CamShake.BP_CamShake_C" (`SceneComponent.K2_GetComponentLocation` (`/Game/Characters/SeaWatcher/BP_SeaWatcher.Camera` _asbp_sea_watcher)) 0.0 1.0)
  (bind _returnvalue (- (`self.PV`) (stale `/Game/GeneralSettings/Int_Hittable.GetHit` Dammage)))
  (bind _output_get (set `self.PV` _returnvalue))
  (`|ExecutionSequence`
    (:`then_0`
      (if (<= _output_get 0.0)
        (goto _label_2)
        (else
          (cast `/Game/Characters/SeaWatcher/BP_SeaWatcher` (`GameplayStatics.GetPlayerCharacter` 0))
          (if (stale `/Game/GeneralSettings/Int_Hittable.GetHit` `Missile?`)
            (`NiagaraFunctionLibrary.SpawnSystemAtLocation` "/Game/VFX/SeaWatcher/ULTI/NS_ImpactUlti.NS_ImpactUlti" (`self.FindHitNSLocation`))
            (`ActorComponent.SetActive` (`self.NS Ulti Explosion`) true true)
            (bind (_direction _newtrack_0) (`Timeline|Timeline_0` :!via `PlayFromStart` :!label _label_4)
              (:`Update`
                (`MaterialInstanceDynamic.SetScalarParameterValue` (`self.Mat`) "Glow" (`KismetMathLibrary.Lerp` 1.0 22.0 _newtrack_0))))
            (else
              (`self.SpawnZlagBall`)
              (goto _label_4 :!via `PlayFromStart`))))))
    (:`then_1`
      (`KismetSystemLibrary.RetriggerableDelay` 1.5)
      (set `self.PV_Buffer` _returnvalue))))

(event `/Game/GeneralSettings/Int_Hittable.GetHit`
  (params (Dammage :type "Float (double-precision)") (PositionHited :type "Vector Structure") (ComboEnd :type Boolean) (`Missile?` :type Boolean) (ClawAttack :type Boolean))
  ;[0 1 0.8115] Dammage System
  (if `Missile?`
    (goto _label_3)
    (else
      (`/Engine/EditorBlueprintResources/StandardMacros.DoOnce` false :!label _label_5
        (:`Completed`
          (goto _label_3))))))

(event `ResetDamage`
  ;[0 1 0.8115] Dammage System
  (goto _label_5 :!via `Reset`))

(event `TargetPosition`
  ;[0 1 0.8115] Dammage System
  (bind _returnvalue (`GameplayStatics.GetActorOfClass` "/Game/Characters/SeaWatcher/BP_SeaWatcher.BP_SeaWatcher_C"))
  (`NiagaraComponent.SetVariableVec3` (`self.NS Zlag Abso`) "Aim_Position" (`SceneComponent.GetSocketLocation` (`Character.Mesh` _returnvalue) "Bind_PearlSocket")))

(event `Die`
  ;[0 1 0.8115] Dammage System
  (set `self.iSDead` true)
  (`self.DetachFromControllerPendingDestroy`)
  (`SceneComponent.SetVisibility` (`self.SkeletalMesh`) false false))

(event `SpawnPosition`
  ;[0 1 0.8115] Dammage System
  (`NiagaraComponent.SetVariableVec3` (`self.NS Zlag Abso`) "Spawn_Position" (`self.K2_GetActorLocation`)))

(event `ValidateHitShake`
  (params (BoneDetected :type Name))
  ;[0 1 0.8115] Dammage System
  (bind _asapb_definitive_edition_eugene (cast `/Game/Characters/Enemy/Boss/Crabe/APB_DefinitiveEditionEugene` (`SkeletalMeshComponent.GetAnimInstance` (`self.SkeletalMesh`))))
  (switch `/Game/Characters/Enemy/Boss/Crabe/Anim/ZoneHit` (enumliteral `/Game/Characters/Enemy/Boss/Crabe/Anim/ZoneHit` (select `int` (`KismetArrayLibrary.Array_Find` (`self.SkeletalToMove`) BoneDetected) :`0` "NewEnumerator6" :`1` "NewEnumerator7" :`2` "NewEnumerator6" :`3` "NewEnumerator7" :`4` "NewEnumerator4" :`5` "NewEnumerator4" :`6` "NewEnumerator5" :`7` "NewEnumerator5" :`8` "NewEnumerator0" :`9` "NewEnumerator0" :`10` "NewEnumerator1" :`11` "NewEnumerator1" :`12` "NewEnumerator2" :`13` "NewEnumerator2" :`14` "NewEnumerator3" :`15` "NewEnumerator3" :!type "/Game/Characters/Enemy/Boss/Crabe/Anim/ZoneHit Enum"))
    (:`NewEnumerator0`
      (set `/Game/Characters/Enemy/Boss/Crabe/APB_DefinitiveEditionEugene.LFL` true _asapb_definitive_edition_eugene))
    (:`NewEnumerator1`
      (set `/Game/Characters/Enemy/Boss/Crabe/APB_DefinitiveEditionEugene.LFR` true _asapb_definitive_edition_eugene))
    (:`NewEnumerator2`
      (set `/Game/Characters/Enemy/Boss/Crabe/APB_DefinitiveEditionEugene.LML` true _asapb_definitive_edition_eugene))
    (:`NewEnumerator3`
      (set `/Game/Characters/Enemy/Boss/Crabe/APB_DefinitiveEditionEugene.LMR` true _asapb_definitive_edition_eugene))
    (:`NewEnumerator4`
      (set `/Game/Characters/Enemy/Boss/Crabe/APB_DefinitiveEditionEugene.LBL` true _asapb_definitive_edition_eugene))
    (:`NewEnumerator5`
      (set `/Game/Characters/Enemy/Boss/Crabe/APB_DefinitiveEditionEugene.LBR` true _asapb_definitive_edition_eugene))
    (:`NewEnumerator6`
      (set `/Game/Characters/Enemy/Boss/Crabe/APB_DefinitiveEditionEugene.HR` true _asapb_definitive_edition_eugene))
    (:`NewEnumerator7`
      (set `/Game/Characters/Enemy/Boss/Crabe/APB_DefinitiveEditionEugene.HL` true _asapb_definitive_edition_eugene))))

(event `SpawnZlagBall`
  ;[0 1 0.8115] Dammage System
  (bind _returnvalue (`GameplayStatics.GetActorOfClass` "/Game/Characters/SeaWatcher/BP_SeaWatcher.BP_SeaWatcher_C"))
  (bind _output_get (set `self.BP SeaWatcher Ref` _returnvalue))
  (set `/Game/Characters/SeaWatcher/BP_SeaWatcher.WhoIsHit` "Eugene" _output_get)
  (`|SpawnActorFromClass` "/Game/VFX/Blueprint/BP_ZlagBall.BP_ZlagBall_C" (`KismetMathLibrary.MakeTransform` (`self.K2_GetActorLocation`) (`KismetMathLibrary.RandomRotator` false) (`KismetMathLibrary.Conv_DoubleToVector` (`KismetMathLibrary.RandomFloatInRange` 0.3 0.6))) "Undefined" "OverrideRootScale" null null))

(event `self.DegatRush.OnComponentBeginOverlap`
  (params (OverlappedComponent :type "PrimitiveComponent Object Reference") (OtherActor :type "Actor Object Reference") (OtherComp :type "PrimitiveComponent Object Reference") (OtherBodyIndex :type Integer) (bFromSweep :type Boolean) (SweepResult :type "HitResult Structure (by ref)"))
  (bind _returnvalue (`self.GetController`))
  (if (`self.ActivAttackRush?`)
    (bind _asbp_sea_watcher (cast `/Game/Characters/SeaWatcher/BP_SeaWatcher` OtherActor)
      (:`then`
        (bind _asaic_crabe (cast `/Game/AI/AIC_Crabe` _returnvalue))
        (`/Game/AI/Ability/AC_Rush.StopRush` (`/Game/AI/AIC_Crabe.AC_Rush` _asaic_crabe))
        (`GameplayStatics.ApplyDamage` _asbp_sea_watcher 20.0 null _asaic_crabe))
      (:`CastFailed`
        (cast `StaticMeshActor` OtherActor
          (:`then`
            _)
          (:`CastFailed`
            (cast `StaticMeshComponent` OtherComp)))
        (bind _asaic_crabe_2 (cast `/Game/AI/AIC_Crabe` _returnvalue))
        (`/Game/AI/Ability/AC_Rush.StopRush` (`/Game/AI/AIC_Crabe.AC_Rush` _asaic_crabe_2))))))

(fn `FindHitNSLocation`
  (returns (Location :type "Vector Structure"))
  (bind (_returnvalue_x _returnvalue_y _returnvalue_z) (`KismetMathLibrary.BreakVector` (`self.K2_GetActorLocation`)))
  (return (`KismetMathLibrary.MakeVector` (+ _returnvalue_x (`KismetMathLibrary.RandomFloatInRange` 0.0 300.0)) (+ _returnvalue_y (`KismetMathLibrary.RandomFloatInRange` 0.0 300.0)) (+ _returnvalue_z 300.0))))

(fn `Random in Z Location Spike`
  (returns (Vector :type "Vector Structure"))
  (bind (_x _y) (`KismetMathLibrary.BreakVector3f` (`KismetMathLibrary.RandomUnitVector`)))
  (return (* (`KismetMathLibrary.MakeVector` _x _y) (`KismetMathLibrary.RandomFloatInRange` (`self.Min`) (`self.Max`)))))

(fn `Smooth Rotation`
  (bind (_returnvalue_roll _returnvalue_pitch _returnvalue_yaw) (`KismetMathLibrary.BreakRotator` (`KismetMathLibrary.RInterpTo` (`self.K2_GetActorRotation`) (`self.GetControlRotation`) (`GameplayStatics.GetWorldDeltaSeconds`) (select `bool` (> (`CharacterMovementComponent.MaxWalkSpeed` (`self.CharacterMovement`)) 601.0) :`false` 2.0 :`true` 4.0 :!type "Float (single-precision)"))))
  (if (`self.IsFocusing?`)
    (`Controller.SetControlRotation` (`self.GetController`) (`KismetMathLibrary.FindLookAtRotation` (`self.K2_GetActorLocation`) (`self.K2_GetActorLocation` (`GameplayStatics.GetPlayerCharacter` 0))))
    (`self.K2_SetActorRotation` (`KismetMathLibrary.MakeRotator` _returnvalue_roll 0.0 _returnvalue_yaw))))

(fn `UserConstructionScript`)