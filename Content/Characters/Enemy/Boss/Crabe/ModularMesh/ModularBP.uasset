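; Modular mesh Blueprint in the crab boss folder that periodically swaps the skeletal mesh of a pincer component.
; The construction script adds PinceMesh and sets the main SkeletalMesh as its master pose component, so it follows that pose.
; On BeginPlay, a looping timer drives a FlipFlop that alternates PinceMesh between Pince_Sans_Eugene_2 and Eugene_V2_Rig_04, reinitializing the pose on each swap.
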(event `self.ReceiveBeginPlay`
  (`KismetSystemLibrary.K2_SetTimerDelegate` (delegate `CustomEvent_0`) 6.0 true))

(event `CustomEvent_0`
  (bind _isa (`/Engine/EditorBlueprintResources/StandardMacros.FlipFlop`)
    (:`A`
      _)
    (:`B`
      _))
  (`SkinnedMeshComponent.SetSkinnedAssetAndUpdate` (`self.PinceMesh`) (select `bool` _isa :`false` "/Game/Characters/Enemy/Boss/Crabe/ModularMesh/Eugene_V2_Rig_04.Eugene_V2_Rig_04" :`true` "/Game/Characters/Enemy/Boss/Crabe/ModularMesh/Pince_Sans_Eugene_2.Pince_Sans_Eugene_2" :!type "SkeletalMesh Object Reference") true))

(fn `UserConstructionScript`
  (bind _returnvalue (`AddComponent|NODE_AddSkeletalMeshComponent-0`))
  (bind _output_get (set `self.PinceMesh` _returnvalue))
  (`SkinnedMeshComponent.SetLeaderPoseComponent` _output_get (`self.SkeletalMesh`) true))