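; Tutorial Blop enemy that teaches basic/heavy attacks, combos or the ultimate, depending on its Type.
; Hits pass a Hittable gate, spawn a Zlag ball, flash a material glow and advance that Type's check, with morph-target squash on non-missile hits.
; The checks update a camera-facing prompt widget, using a timer for combo input, and trigger Die on success.
; Death plays a montage, timeline-driven dissolve and VFX, drops another ball, then destroys the actor.
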(event `DeathVfx`
  (bind _ns_blob_death (`self.NS Blob Death`))
  ;[1 0 1] VFX DEATH BLOB - Intégration Presque parfaite non? :)
  (`SceneComponent.K2_SetWorldLocation` _ns_blob_death (`SceneComponent.GetSocketLocation` (`self.Mesh`) "Bind_BodySocket_DeathVFX") false false)
  (`/Engine/EditorBlueprintResources/StandardMacros.DoOnce` false
    (:`Completed`
      (`MeshComponent.SetScalarParameterValueOnMaterials` (`self.Mesh`) "Dissolve0on1off" 0.0)
      (`GameplayStatics.PlaySoundAtLocation` "/Game/Sound/Characters/Blob/Die_01.Die_01" (0.0 0.0 0.0) (struct) 1.0 1.0 0.0 null null null null)
      (`GameplayStatics.PlaySoundAtLocation` "/Game/Sound/Characters/Blob/Die_02.Die_02" (0.0 0.0 0.0) (struct) 1.0 1.0 0.0 null null null null)
      (`KismetSystemLibrary.Delay` 1.0)
      (`ActorComponent.Activate` _ns_blob_death false))))

(event `SpawnZlagBall`
  ;[1 1 1] SPAWN ZLAG BALL
  (bind _returnvalue (`GameplayStatics.GetActorOfClass` "/Game/Characters/SeaWatcher/BP_SeaWatcher.BP_SeaWatcher_C"))
  (bind _output_get (set `self.BP SeaWatcher Ref` _returnvalue))
  (set `/Game/Characters/SeaWatcher/BP_SeaWatcher.WhoIsHit` "Blop" _output_get)
  (`|SpawnActorFromClass` "/Game/VFX/Blueprint/BP_ZlagBall.BP_ZlagBall_C" (`KismetMathLibrary.MakeTransform` (`self.K2_GetActorLocation`) (`KismetMathLibrary.MakeRotator` 0.0 0.0 (`KismetMathLibrary.RandomFloatInRange` 0.0 360.0)) (`KismetMathLibrary.VLerp` (0.3 0.3 0.3) (0.6 0.6 0.6) (`KismetMathLibrary.RandomFloat`))) "Undefined" "OverrideRootScale" null null))

(event `Die`
  (bind (_returnvalue_x _returnvalue_y) (`KismetMathLibrary.BreakVector` (`self.K2_GetActorLocation`)))
  (bind _capsulecomponent (`self.CapsuleComponent`))
  (`self.DetachFromControllerPendingDestroy`)
  ;[0 0 0] DEATH BLOB
  (`/Engine/EditorBlueprintResources/StandardMacros.DoOnce` false
    (:`Completed`
      (`|PlayMontage` (`self.Mesh`) "/Game/Characters/Enemy/TrashMob/Blob/Mesh/Blob_VF/Blob_Anim_Ded_Montage.Blob_Anim_Ded_Montage"
        (:`then`
          (set `CharacterMovementComponent.MaxWalkSpeed` 0.0 (`self.CharacterMovement`))
          (`PrimitiveComponent.SetCollisionResponseToChannel` _capsulecomponent "ECC_GameTraceChannel5" "ECR_Ignore")
          (`PrimitiveComponent.SetCollisionResponseToChannel` _capsulecomponent "ECC_Pawn" "ECR_Ignore")
          (`AudioComponent.FadeOut` (`self.Audio`) 1.0 0.0 "Linear")
          (bind (_direction _newtrack_0 _coefdissolve) (`Timeline|Timeline_0`)
            (:`Update`
              (`MeshComponent.SetScalarParameterValueOnMaterials` (`self.Mesh`) "Dissolve" _coefdissolve)
              ;;[1 0 1] VFX
              (`self.DeathVfx`)
              (if (>= _newtrack_0 0.5)
                (`/Engine/EditorBlueprintResources/StandardMacros.DoOnce` false
                  (:`Completed`
                    (set `/Game/Characters/SeaWatcher/BP_SeaWatcher.WhoIsHit` "BlopDeath" (`self.BP SeaWatcher Ref`))
                    (`|SpawnActorFromClass` "/Game/VFX/Blueprint/BP_ZlagBall.BP_ZlagBall_C" (`KismetMathLibrary.MakeTransform` (`KismetMathLibrary.MakeVector` _returnvalue_x _returnvalue_y 1000.0) (struct) (`KismetMathLibrary.VLerp` (0.3 0.3 0.3) (0.6 0.6 0.6) (`KismetMathLibrary.RandomFloat`))) "Undefined" "OverrideRootScale" null null)))))
            (:`Finished`
              (`self.K2_DestroyActor`))))))))

(event `self.ReceiveBeginPlay`
  (bind _returnvalue (`KismetMaterialLibrary.CreateDynamicMaterialInstance` "/Game/Characters/Enemy/TrashMob/Blob/Mesh/M_Blob_Inst.M_Blob_Inst"))
  (bind _output_get (set `self.Materiau` _returnvalue))
  (`PrimitiveComponent.SetMaterial` (`self.Mesh`) 0 _output_get)
  (bind _asbp_sea_watcher (cast `/Game/Characters/SeaWatcher/BP_SeaWatcher` (`GameplayStatics.GetPlayerCharacter` 0)))
  (set `self.Camera` (`/Game/Characters/SeaWatcher/BP_SeaWatcher.Camera` _asbp_sea_watcher))
  (`GameplayStatics.SpawnSoundAttached` "/Game/Sound/Ambs/Fish/AMB_FishTuto_LP_Cue.AMB_FishTuto_LP_Cue" (`self.Audio`) "None" (0.0 0.0 0.0) (struct) "KeepRelativeOffset" false 1.0 1.0 0.0 null null))

(event `checkAtt`
  (params (A :type Boolean))
  (if A
    (if (not (>= (`self.Count`) 2))
      (bind _result (`/Engine/EditorBlueprintResources/StandardMacros.IncrementInt` (`self.Count`))
        (:`  `
          (if (== _result 2)
            (bind _asui_tuto_basic_attack (cast `/Game/UI/UI_TutoBasicAttack` (`WidgetComponent.GetWidget` (`self.Widget`))))
            (`/Game/UI/UI_TutoBasicAttack.Appear` _asui_tuto_basic_attack false)
            (`KismetSystemLibrary.Delay` 1.0)
            (`Image.SetBrushFromTexture` (`/Game/UI/UI_TutoBasicAttack.Bouton` _asui_tuto_basic_attack) "/Game/UI/Texture/UI_Y.UI_Y" false)
            (`TextBlock.SetText` (`/Game/UI/UI_TutoBasicAttack.TextBlock_28` _asui_tuto_basic_attack) "Heavy attack")
            (`/Game/UI/UI_TutoBasicAttack.Appear` _asui_tuto_basic_attack true)))))
    (elif (not (<= (`self.Count`) 1))
      (bind _result_2 (`/Engine/EditorBlueprintResources/StandardMacros.IncrementInt` (`self.Count`))
        (:`  `
          (if (>= _result_2 4)
            (`self.Die`)
            (bind _asui_tuto_basic_attack_2 (cast `/Game/UI/UI_TutoBasicAttack` (`WidgetComponent.GetWidget` (`self.Widget`))))
            (`/Game/UI/UI_TutoBasicAttack.Appear` _asui_tuto_basic_attack_2 false)))))))

(event `self.ReceiveTick`
  (params (DeltaSeconds :type "Float (single-precision)"))
  (if (`self.UIIsOn`)
    (`SceneComponent.K2_SetWorldRotation` (`self.Widget`) (`KismetMathLibrary.Conv_VectorToRotator` (`KismetMathLibrary.NegateVector` (`SceneComponent.GetForwardVector` (`self.Camera`)))) false false)))

(event `self.ReceiveRadialDamage`
  (params (DamageReceived :type "Float (single-precision)") (DamageType :type "DamageType Object Reference") (Origin :type "Vector Structure") (HitInfo :type "HitResult Structure (by ref)") (InstigatedBy :type "Controller Object Reference") (DamageCauser :type "Actor Object Reference"))
  (set `self.isMissile` true)
  (if (`self.Hittable?`) :!label _label
    (`GameplayStatics.SpawnSoundAtLocation` "/Game/Sound/Characters/Blob/Impact/SFX_Blob_GetHit_Cue.SFX_Blob_GetHit_Cue" (`SceneComponent.K2_GetComponentLocation` (`self.Audio`)) (struct) 1.0 1.0 0.0 null null)
    (if (not (`self.isMissile`))
      (`/Engine/EditorBlueprintResources/StandardMacros.DoOnce` false :!label _label_2
        (:`Completed`
          (`/Game/Characters/SeaWatcher/BP_SeaWatcher.PlayPlayerHitCameraShake` (cast `/Game/Characters/SeaWatcher/BP_SeaWatcher` (`GameplayStatics.GetPlayerCharacter` 0) :!pure true))
          (`self.ApplyBlend` (stale `/Game/GeneralSettings/Int_Hittable.GetHit` PositionHited)))))
    ;[1 1 1] zlag ball
    (`self.SpawnZlagBall`)
    (set `self.Hittable?` false)
    (switch `/Game/GeneralSettings/Enum_TutorialType` (`self.Type`)
      (:`NewEnumerator0`
        (`self.checkAtt` (stale `/Game/GeneralSettings/Int_Hittable.GetHit` ClawAttack))
        (bind (_direction _newtrack_0) (`Timeline|Timeline_1` :!via `PlayFromStart` :!label _label_3)
          (:`Update`
            (`MaterialInstanceDynamic.SetScalarParameterValue` (`self.Materiau`) "Glow" _newtrack_0))))
      (:`NewEnumerator1`
        (`self.CheckCombo` (stale `/Game/GeneralSettings/Int_Hittable.GetHit` ComboEnd))
        (goto _label_3 :!via `PlayFromStart`))
      (:`NewEnumerator2`
        (`self.CheckUlti` (`self.isMissile`))
        (goto _label_3 :!via `PlayFromStart`)))))

(event `/Game/GeneralSettings/Int_Hittable.GetHit`
  (params (Dammage :type "Float (double-precision)") (PositionHited :type "Vector Structure") (ComboEnd :type Boolean) (`Missile?` :type Boolean) (ClawAttack :type Boolean) (ComboAttackValue :type "/Game/GeneralSettings/Enum_ComboType Enum" :default "NewEnumerator0"))
  (set `self.isMissile` `Missile?`)
  (goto _label))

(event `ResetHit`
  (set `self.Hittable?` true)
  (goto _label_2 :!via `Reset`))

(event `ApplyBlend`
  (params (Dammage :type "Vector Structure"))
  ;[1 0.7372 0] BLEND
  (`TimelineComponent.SetPlayRate` (`self.Timeline_2`) 0.5)
  (bind (_direction _newtrack_0 _newtrack_1) (`Timeline|Timeline_2` :!via `PlayFromStart`)
    (:`Update`
      (`SkeletalMeshComponent.SetMorphTarget` (`self.Mesh`) "Body_Choc_Front_R" _newtrack_0 true)
      (`SkeletalMeshComponent.SetMorphTarget` (`self.Mesh`) "Body_Choc_Front_L" _newtrack_1 true))))

(event `ResetWid`
  (bind _newvar_1 (`self.NewVar_1`))
  (set `self.NewVar_1` false)
  (bind _asui_combo_attack (cast `/Game/UI/UI_ComboAttack` (`WidgetComponent.GetWidget` (`self.Widget`)) :!label _label_4))
  (`/Game/UI/UI_ComboAttack.SetText` _asui_combo_attack (select `int` (`self.Count`) :`0` "3" :`1` "2" :`2` "1" :`3` "0" :!type "Text"))
  (bind _image (`/Game/UI/UI_ComboAttack.Image` _asui_combo_attack))
  (`Widget.SetRenderOpacity` _image 0.6)
  (`Widget.SetRenderOpacity` (`/Game/UI/UI_ComboAttack.Image_1` _asui_combo_attack) 0.6)
  (`Widget.SetRenderOpacity` (`/Game/UI/UI_ComboAttack.Image_3` _asui_combo_attack) 0.6)
  (`Widget.SetRenderOpacity` (`/Game/UI/UI_ComboAttack.Image_4` _asui_combo_attack) 0.6)
  (`Widget.SetRenderOpacity` (`/Game/UI/UI_ComboAttack.Image_0` _asui_combo_attack) 0.6)
  (`Widget.SetRenderOpacity` (`/Game/UI/UI_ComboAttack.Image_2` _asui_combo_attack) 0.6)
  (`Image.SetBrushTintColor` _image (make `SlateColor` (`KismetMathLibrary.SelectColor` (struct :`R` 0.40625 :`G` 0.078818 :`B` 0.0586 :`A` 1.0) (struct :`R` 0.310215 :`G` 1.0 :`B` 0.560211 :`A` 1.0) (not _newvar_1))))
  (`Image.SetBrushTintColor` (`/Game/UI/UI_ComboAttack.Image_1` _asui_combo_attack) (make `SlateColor` (`KismetMathLibrary.SelectColor` (struct :`R` 0.40625 :`G` 0.078818 :`B` 0.0586 :`A` 1.0) (struct :`R` 0.310215 :`G` 1.0 :`B` 0.560211 :`A` 1.0) (not _newvar_1))))
  (`Image.SetBrushTintColor` (`/Game/UI/UI_ComboAttack.Image_0` _asui_combo_attack) (make `SlateColor` (`KismetMathLibrary.SelectColor` (struct :`R` 0.40625 :`G` 0.078818 :`B` 0.0586 :`A` 1.0) (struct :`R` 0.310215 :`G` 1.0 :`B` 0.560211 :`A` 1.0) (not _newvar_1))))
  (`Image.SetBrushTintColor` (`/Game/UI/UI_ComboAttack.Image_4` _asui_combo_attack) (make `SlateColor` (`KismetMathLibrary.SelectColor` (struct :`R` 0.40625 :`G` 0.078818 :`B` 0.0586 :`A` 1.0) (struct :`R` 0.310215 :`G` 1.0 :`B` 0.560211 :`A` 1.0) (not _newvar_1))))
  (`Image.SetBrushTintColor` (`/Game/UI/UI_ComboAttack.Image_3` _asui_combo_attack) (make `SlateColor` (`KismetMathLibrary.SelectColor` (struct :`R` 0.40625 :`G` 0.078818 :`B` 0.0586 :`A` 1.0) (struct :`R` 0.310215 :`G` 1.0 :`B` 0.560211 :`A` 1.0) (not _newvar_1))))
  (`Image.SetBrushTintColor` (`/Game/UI/UI_ComboAttack.Image_2` _asui_combo_attack) (make `SlateColor` (`KismetMathLibrary.SelectColor` (struct :`R` 0.40625 :`G` 0.078818 :`B` 0.0586 :`A` 1.0) (struct :`R` 0.310215 :`G` 1.0 :`B` 0.560211 :`A` 1.0) (not _newvar_1))))
  (`/Game/UI/UI_ComboAttack.UI FeedBack` _asui_combo_attack _newvar_1)
  (`KismetSystemLibrary.Delay` 0.4)
  (`Image.SetBrushTintColor` _image (make `SlateColor` (struct :`R` 1.0 :`G` 1.0 :`B` 1.0 :`A` 1.0)))
  (`Image.SetBrushTintColor` (`/Game/UI/UI_ComboAttack.Image_1` _asui_combo_attack) (make `SlateColor` (struct :`R` 1.0 :`G` 1.0 :`B` 1.0 :`A` 1.0)))
  (`Image.SetBrushTintColor` (`/Game/UI/UI_ComboAttack.Image_0` _asui_combo_attack) (make `SlateColor` (struct :`R` 1.0 :`G` 1.0 :`B` 1.0 :`A` 1.0)))
  (`Image.SetBrushTintColor` (`/Game/UI/UI_ComboAttack.Image_3` _asui_combo_attack) (make `SlateColor` (struct :`R` 1.0 :`G` 1.0 :`B` 1.0 :`A` 1.0)))
  (`Image.SetBrushTintColor` (`/Game/UI/UI_ComboAttack.Image_2` _asui_combo_attack) (make `SlateColor` (struct :`R` 1.0 :`G` 1.0 :`B` 1.0 :`A` 1.0)))
  (`Image.SetBrushTintColor` (`/Game/UI/UI_ComboAttack.Image_4` _asui_combo_attack) (make `SlateColor` (struct :`R` 1.0 :`G` 1.0 :`B` 1.0 :`A` 1.0))))

(event `GoodWid`
  (set `self.NewVar_1` true)
  (bind _asui_combo_attack (cast `/Game/UI/UI_ComboAttack` (`WidgetComponent.GetWidget` (`self.Widget`))))
  (`Widget.SetRenderOpacity` (`/Game/UI/UI_ComboAttack.Image_4` _asui_combo_attack) 1.0)
  (`Widget.SetRenderOpacity` (`/Game/UI/UI_ComboAttack.Image_3` _asui_combo_attack) 1.0)
  (`KismetSystemLibrary.Delay` 0.2)
  (goto _label_4))

(fn `CheckCombo`
  (params (EndCombo :type Boolean))
  (bind _newvar_0 (`self.NewVar_0`))
  (if EndCombo
    (bind _result (`/Engine/EditorBlueprintResources/StandardMacros.IncrementInt` (`self.Count`))
      (:`  `
        (`KismetSystemLibrary.K2_ClearAndInvalidateTimerHandle` (`self.NewVar_0`))
        (`self.GoodWid`)
        (if (>= _result 3)
          (`self.Die`)
          (bind _asui_combo_attack (cast `/Game/UI/UI_ComboAttack` (`WidgetComponent.GetWidget` (`self.Widget`))))
          (`/Game/UI/UI_ComboAttack.ApplyPushButton` _asui_combo_attack false))))
    (else
      (bind _asui_combo_attack_2 (cast `/Game/UI/UI_ComboAttack` (`WidgetComponent.GetWidget` (`self.Widget`))))
      (if (`KismetSystemLibrary.K2_IsValidTimerHandle` _newvar_0)
        (`KismetSystemLibrary.K2_ClearAndInvalidateTimerHandle` _newvar_0))
      (bind _returnvalue (`KismetSystemLibrary.K2_SetTimerDelegate` (`|CreateDelegate` :!event `ResetWid`) 0.7))
      (set `self.NewVar_0` _returnvalue)
      (bind _image_0 (`/Game/UI/UI_ComboAttack.Image_0` _asui_combo_attack_2))
      (if (== (`Widget.GetRenderOpacity` _image_0) 1.0)
        (`Widget.SetRenderOpacity` (`/Game/UI/UI_ComboAttack.Image_1` _asui_combo_attack_2) 1.0)
        (`Widget.SetRenderOpacity` (`/Game/UI/UI_ComboAttack.Image` _asui_combo_attack_2) 1.0)
        (else
          (`Widget.SetRenderOpacity` _image_0 1.0)
          (`Widget.SetRenderOpacity` (`/Game/UI/UI_ComboAttack.Image_2` _asui_combo_attack_2) 1.0))))))

(fn `CheckUlti`
  (params (Ulti :type Boolean))
  (if Ulti
    (`self.Die`)
    (bind _asui_ultimate (cast `/Game/UI/UI_Ultimate` (`WidgetComponent.GetWidget` (`self.Widget`))))
    (`/Game/UI/UI_Ultimate.ApplyPushButton` _asui_ultimate false)))

(fn `UserConstructionScript`)