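; Crab AI ability that makes the crab strafe in a randomly chosen direction for a short burst, unless it is doing stagger security.
; Activation raises walk speed, writes direction and movement flag to the Blackboard, and boosts the weights of three pincer and hammer attacks in the AI controller's Backpack.
; A timer then clears the movement flag, lowers the speed and finishes the skill.
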(event `self.ReceiveBeginPlay`
  (`parent.ReceiveBeginPlay`))

(event `self.ReceiveTick`
  (params (DeltaSeconds :type "Float (single-precision)"))
  (`parent.ReceiveTick` DeltaSeconds))

(event `self.Activation`
  (params (IsMovementAbility :type Boolean))
  (bind _returnvalue (`AIBlueprintHelperLibrary.GetBlackboard` (`self.AIC Crabe`)))
  (if (not (`/Game/Characters/Enemy/Boss/Crabe/BP_Crabe.isDoingStagger_Security` (`self.Crabe`)))
    (`parent.Activation` true)
    (set `CharacterMovementComponent.MaxWalkSpeed` 1400.0 (`Character.CharacterMovement` (`self.Crabe`)))
    (`BlackboardComponent.SetValueAsEnum` _returnvalue "Direction" (select `bool` (`KismetMathLibrary.RandomBool`) :`false` "NewEnumerator1" :`true` "NewEnumerator0" :!type "/Game/AI/Enum_Direction Enum"))
    (`BlackboardComponent.SetValueAsBool` _returnvalue "InMove" true)
    (set `self.inMove` true)
    (for _array_element (`/Game/AI/AIC_Crabe.Backpack` (`self.AIC Crabe`))
      (bind _returnvalue_2 (`GameplayStatics.GetObjectClass` _array_element))
      (if (or (== _returnvalue_2 "/Game/AI/Ability/OKAC_PinceZlag.OKAC_PinceZlag_C") (== _returnvalue_2 "/Game/AI/Ability/OKAC_CoupDeMarteau.OKAC_CoupDeMarteau_C") (== _returnvalue_2 "/Game/AI/Ability/OKAC_CoupDePince.OKAC_CoupDePince_C"))
        (`self.MoreWeight` _array_element 0.1 0.2)))
    (bind _returnvalue_3 (`KismetSystemLibrary.K2_SetTimerDelegate` (delegate `StopMove`) 3.0))
    (set `self.Handler` _returnvalue_3)))

(event `StopMove`
  (`BlackboardComponent.SetValueAsBool` (`AIBlueprintHelperLibrary.GetBlackboard` (`self.AIC Crabe`)) "InMove" false)
  (set `self.inMove` false)
  (set `CharacterMovementComponent.MaxWalkSpeed` 800.0 (`Character.CharacterMovement` (`self.Crabe`)))
  (`self.FinishedSkill`))