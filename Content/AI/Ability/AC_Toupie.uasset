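; AC_Toupie is an AI ability component that makes the Crabe enemy perform its Toupie montage attack.
; Activation is skipped during stagger security; otherwise it triggers the attack glow and plays the montage, faster when staggered and at slightly randomized speed otherwise.
; On completion it finishes the skill and adds weight to the controller's backward and strafe abilities, including NewStrafe when valid.
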(event `self.ReceiveBeginPlay`
  (`parent.ReceiveBeginPlay`))

(event `self.ReceiveTick`
  (params (DeltaSeconds :type "Float (single-precision)"))
  (`parent.ReceiveTick` DeltaSeconds))

(event `self.Activation`
  (params (IsMovementAbility :type Boolean))
  (bind _aic_crabe (`self.AIC Crabe`))
  (bind _crabe (`self.Crabe`))
  (bind _ac_backward (`/Game/AI/AIC_Crabe.AC_Backward` _aic_crabe))
  (if (not (`/Game/Characters/Enemy/Boss/Crabe/BP_Crabe.isDoingStagger_Security` (`self.Crabe`)))
    (`parent.Activation` false)
    (`/Game/Characters/Enemy/Boss/Crabe/BP_Crabe.GlowingAttacking` (`self.Crabe`))
    (`|PlayMontage` (`Character.Mesh` _crabe) "/Game/Characters/Enemy/Boss/Crabe/Anim/Toupie_V001_Montage.Toupie_V001_Montage" (select `bool` (`/Game/Characters/Enemy/Boss/Crabe/BP_Crabe.IsStagger` _crabe) :`false` (`KismetMathLibrary.RandomFloatInRange` 0.9 1.1) :`true` 1.4 :!type "Float (single-precision)")
      (:`OnCompleted`
        (`self.FinishedSkill`)
        (bind _ac_newstrafe (`/Game/AI/AIC_Crabe.AC_NewStrafe` _aic_crabe)
          (:`then`
            (`self.MoreWeight` _ac_backward 0.1 0.2)
            (`self.MoreWeight` (`/Game/AI/AIC_Crabe.OKAC_StrafeWithoutFocus` _aic_crabe) 0.1 0.2)
            (`self.MoreWeight` _ac_newstrafe 0.1 0.2))
          (:`else`
            (`self.MoreWeight` _ac_backward 0.1 0.2)
            (`self.MoreWeight` (`/Game/AI/AIC_Crabe.OKAC_StrafeWithoutFocus` _aic_crabe) 0.1 0.2)))))))