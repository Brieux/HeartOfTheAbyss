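; AI ability component that makes the crab burrow through sand to a fixed destination, skipped when it is already within range of it.
; Activation turns on the attack glow, disables collision and plays the dig montage, whose notify starts Tick-driven interpolated movement, with timed Niagara sand effects.
; On arrival, an exit montage's blend-out restores collision, stops the glow, raises backward and strafe ability weights, and finishes the skill.
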(event `DesactivateCollision`
  (params (Index :type Boolean))
  (`PrimitiveComponent.SetCollisionEnabled` (`/Game/Characters/Enemy/Boss/Crabe/BP_Crabe.SkeletalMesh` (`self.Crabe`)) (select `bool` Index :`false` "QueryAndPhysics" :`true` "NoCollision" :!type "ECollisionEnabled Enum"))
  (`PrimitiveComponent.SetCollisionEnabled` (`Character.CapsuleComponent` (`self.Crabe`)) (select `bool` Index :`false` "QueryAndPhysics" :`true` "NoCollision" :!type "ECollisionEnabled Enum")))

(event `self.ReceiveBeginPlay`
  (`parent.ReceiveBeginPlay`)
  (bind _returnvalue (`GameplayStatics.GetActorOfClass` "/Game/Characters/Enemy/Boss/Crabe/BP_Crabe.BP_Crabe_C"))
  (set `self.BP Crabe Ref` _returnvalue))

(event `self.ReceiveTick`
  (params (DeltaSeconds :type "Float (single-precision)"))
  (bind _crabe (`self.Crabe`))
  (bind _crabe_2 (`self.Crabe`))
  (`parent.ReceiveTick` DeltaSeconds)
  (if (`self.InMove`)
    (`Actor.K2_SetActorLocation` _crabe (`KismetMathLibrary.VInterpTo` (`Actor.K2_GetActorLocation` (`self.Crabe`)) (-1375.0 143.0 412.805481) DeltaSeconds 3.0) false false)
    (if (== (`Actor.K2_GetActorLocation` _crabe) (`self.AimDestination`) :`ErrorTolerance` 30.0)
      (`/Engine/EditorBlueprintResources/StandardMacros.DoOnce` false :!label _label
        (:`Completed`
          (set `self.InMove` false)
          (`|PlayMontage` (`/Game/Characters/Enemy/Boss/Crabe/BP_Crabe.SkeletalMesh` _crabe_2) "/Game/Characters/Enemy/Boss/Crabe/Anim/AM_FinTunnel.AM_FinTunnel"
            (:`OnBlendOut`
              (`/Game/Characters/Enemy/Boss/Crabe/BP_Crabe.StopGlowingAttacking` _crabe_2)
              (`self.DesactivateCollision` false)
              (`self.MoreWeight` (`/Game/AI/AIC_Crabe.AC_Backward` (`self.AIC Crabe`)) 0.1 0.2)
              (`self.MoreWeight` (`/Game/AI/AIC_Crabe.AC_Straf` (`self.AIC Crabe`)) 0.1 0.2)
              (`self.MoreWeight` (`/Game/AI/AIC_Crabe.OKAC_StrafeWithoutFocus` (`self.AIC Crabe`)) 0.1 0.2)
              (`self.FinishedSkill`))))))))

(event `self.Activation`
  (params (IsMovementAbility :type Boolean))
  (bind _crabe (`self.Crabe`))
  (`parent.Activation` false)
  (if (<= (`KismetMathLibrary.Vector_Distance` (`Actor.K2_GetActorLocation` (`self.Crabe`)) (`self.AimDestination`)) 2500.0)
    (`self.FinishedSkill`)
    (else
      (`/Game/Characters/Enemy/Boss/Crabe/BP_Crabe.GlowingAttacking` _crabe)
      (`self.VFXEnterTunnel`)
      (`self.DesactivateCollision` true)
      (`|PlayMontage` (`/Game/Characters/Enemy/Boss/Crabe/BP_Crabe.SkeletalMesh` _crabe) "/Game/Characters/Enemy/Boss/Crabe/Anim/AM_DebTunnel.AM_DebTunnel"
        (:`then`
          (`KismetSystemLibrary.Delay` 3.5)
          (`self.VFXLeaveTunnel`))
        (:`OnNotifyBegin`
          (set `self.InMove` true)
          (goto _label :!via `Reset`))))))

(event `VFXEnterTunnel`
  (bind _returnvalue (`SceneComponent.K2_GetComponentToWorld` (`/Game/Characters/Enemy/Boss/Crabe/BP_Crabe.SkeletalMesh` (`self.BP Crabe Ref`))))
  ;[1 1 1] VFX CRAB TUNNEL
  (`NiagaraFunctionLibrary.SpawnSystemAtLocation` "/Game/VFX/NiagaraSystem/Mick/BossCrab/NS_TunnelDeb_SandEffect.NS_TunnelDeb_SandEffect" (`KismetMathLibrary.MakeVector` (.x (.location _returnvalue)) (.y (.location _returnvalue)) (- (.z (.location _returnvalue)) 30.0)) (.rotation _returnvalue)))

(event `VFXLeaveTunnel`
  (bind _returnvalue (`SceneComponent.K2_GetComponentToWorld` (`/Game/Characters/Enemy/Boss/Crabe/BP_Crabe.SkeletalMesh` (`self.BP Crabe Ref`))))
  ;[1 1 1] VFX CRAB TUNNEL
  (`NiagaraFunctionLibrary.SpawnSystemAtLocation` "/Game/VFX/NiagaraSystem/Mick/BossCrab/NS_TunnelEnd_SandEffect.NS_TunnelEnd_SandEffect" (`KismetMathLibrary.MakeVector` (.x (.location _returnvalue)) (.y (.location _returnvalue)) (.z (.location _returnvalue))) (.rotation _returnvalue)))