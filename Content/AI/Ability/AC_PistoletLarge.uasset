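; AC_PistoletLarge is an AI ability for the crab (BP_Crabe) that relocates it through a tunnel move, then plays the PistoletLarge attack.
; On activation it turns off focusing, starts the attack glow and plays the tunnel-start montage.
; It then moves the crab to one of two hardcoded locations at random and, after a short delay, plays the tunnel-end montage.
; Focusing resumes for the PistoletLarge montage, whose blend-out stops the glow and finishes the skill.
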(event `self.ReceiveBeginPlay`
  (`parent.ReceiveBeginPlay`))

(event `self.ReceiveTick`
  (params (DeltaSeconds :type "Float (single-precision)"))
  (`parent.ReceiveTick` DeltaSeconds))

(event `self.Activation`
  (params (IsMovementAbility :type Boolean))
  (bind _crabe (`self.Crabe`))
  (bind _mesh (`Character.Mesh` _crabe))
  (`parent.Activation` false)
  (bind _returnvalue (`GameplayStatics.GetActorOfClass` "/Game/Characters/Enemy/Boss/Crabe/BP_Crabe.BP_Crabe_C"))
  (set `/Game/Characters/Enemy/Boss/Crabe/BP_Crabe.IsFocusing?` false _returnvalue)
  (`/Game/Characters/Enemy/Boss/Crabe/BP_Crabe.GlowingAttacking` _returnvalue)
  (`|PlayMontage` _mesh "/Game/Characters/Enemy/Boss/Crabe/ModularMesh/AnimRetarget/AM_DebTunnel_Retargeted.AM_DebTunnel_Retargeted"
    (:`OnCompleted`
      (`Actor.K2_SetActorLocation` (`self.Crabe`) (`KismetMathLibrary.SelectVector` (15846.0 -30866.0 -4518.0) (20549.0 -30879.0 -4518.0) (`KismetMathLibrary.RandomBool`)) false false)
      (`KismetSystemLibrary.Delay` 0.2)
      (`|PlayMontage` _mesh "/Game/Characters/Enemy/Boss/Crabe/ModularMesh/AnimRetarget/AM_FinTunnel_Retargeted.AM_FinTunnel_Retargeted"
        (:`OnBlendOut`
          (set `/Game/Characters/Enemy/Boss/Crabe/BP_Crabe.IsFocusing?` true _crabe)
          (`|PlayMontage` _mesh "/Game/Characters/Enemy/Boss/Crabe/ModularMesh/AnimRetarget/AM_PistoletLarge.AM_PistoletLarge"
            (:`OnBlendOut`
              (`/Game/Characters/Enemy/Boss/Crabe/BP_Crabe.StopGlowingAttacking` _crabe)
              (`self.FinishedSkill`))))))))