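; AI ability component that makes the Crabe enemy block for a random few seconds.
; Activation resets hit tracking, plays the block VFX and montage, and sets a timer to Unblock.
; Unblock either plays a glowing block-bash counter when TooMuchHit is set or a plain unblock montage, then restores focus and finishes the skill.
; A DoOnce, re-armed on each activation, keeps Unblock from running twice.
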(event `self.ReceiveBeginPlay`
  (`parent.ReceiveBeginPlay`))

(event `self.ReceiveTick`
  (params (DeltaSeconds :type "Float (single-precision)"))
  (`parent.ReceiveTick` DeltaSeconds))

(event `self.Activation`
  (params (IsMovementAbility :type Boolean))
  (bind _crabe (`self.Crabe`))
  (bind _crabe_2 (`self.Crabe`))
  (set `self.TooMuchHit` false)
  (set `/Game/Characters/Enemy/Boss/Crabe/BP_Crabe.NbOfHit` 0.0 (`self.Crabe`))
  (set `self.BlockingDelay` (`KismetMathLibrary.RandomFloatInRange` 3.0 7.0))
  (`/Game/Characters/Enemy/Boss/Crabe/BP_Crabe.VFXBlock` _crabe_2)
  (`|PlayMontage` (`Character.Mesh` _crabe_2) "/Game/Characters/Enemy/Boss/Crabe/ModularMesh/Anim_Retarget_VF/AM_Block.AM_Block"
    (:`then`
      (set `/Game/Characters/Enemy/Boss/Crabe/BP_Crabe.IsFocusing?` false _crabe)
      (set `/Game/Characters/Enemy/Boss/Crabe/BP_Crabe.IsBlocking` true _crabe)
      (bind _returnvalue (`KismetSystemLibrary.K2_SetTimerDelegate` (delegate `Unblock`) (`self.BlockingDelay`)))
      (set `self.Handler` _returnvalue)
      (`self.AllowUnblock`))))

(event `Unblock`
  (bind _crabe (`self.Crabe`))
  (bind _mesh (`Character.Mesh` (`self.Crabe`)))
  (`/Engine/EditorBlueprintResources/StandardMacros.DoOnce` false :!label _label
    (:`Completed`
      (`KismetSystemLibrary.K2_ClearAndInvalidateTimerHandle` (`self.Handler`))
      (if (`self.TooMuchHit`)
        (`/Game/Characters/Enemy/Boss/Crabe/BP_Crabe.GlowingAttacking` (`self.Crabe`))
        (`|PlayMontage` _mesh "/Game/Characters/Enemy/Boss/Crabe/ModularMesh/Anim_Retarget_VF/AM_BlockBash.AM_BlockBash"
          (:`OnBlendOut`
            (`/Game/Characters/Enemy/Boss/Crabe/BP_Crabe.StopGlowingAttacking` _crabe)))
        (else
          (`|PlayMontage` _mesh "/Game/Characters/Enemy/Boss/Crabe/ModularMesh/Anim_Retarget_VF/AM_Unblock.AM_Unblock"
            (:`then`
              _))))
      (set `/Game/Characters/Enemy/Boss/Crabe/BP_Crabe.IsBlocking` false _crabe)
      (set `/Game/Characters/Enemy/Boss/Crabe/BP_Crabe.IsFocusing?` true (`self.Crabe`))
      (`self.FinishedSkill`))))

(event `AllowUnblock`
  (goto _label :!via `Reset`))