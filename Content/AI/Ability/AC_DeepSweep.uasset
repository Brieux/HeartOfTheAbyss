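; AC_DeepSweep is an AI ability component that makes the Crabe enemy perform its deep sweep attack.
; On activation it triggers the attack glow, disables gravity and plays the sweep montage, faster when staggered and otherwise at a slightly randomized rate.
; When the montage completes, it restores gravity, ends the skill and raises the selection weights of backward and strafe abilities to favor repositioning next.
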(event `self.ReceiveBeginPlay`
  (`parent.ReceiveBeginPlay`))

(event `self.ReceiveTick`
  (params (DeltaSeconds :type "Float (single-precision)"))
  (`parent.ReceiveTick` DeltaSeconds))

(event `self.Activation`
  (params (IsMovementAbility :type Boolean))
  (bind _crabe (`self.Crabe`))
  (`parent.Activation` false)
  (`/Game/Characters/Enemy/Boss/Crabe/BP_Crabe.GlowingAttacking` (`self.Crabe`))
  (set `CharacterMovementComponent.GravityScale` 0.0 (`Character.CharacterMovement` (`self.Crabe`)))
  (`|PlayMontage` (`Character.Mesh` _crabe) "/Game/Characters/Enemy/Boss/Crabe/Anim/Eugene_deep_Sweep_02_Montage.Eugene_deep_Sweep_02_Montage" (select `bool` (`/Game/Characters/Enemy/Boss/Crabe/BP_Crabe.IsStagger` _crabe) :`false` (`KismetMathLibrary.RandomFloatInRange` 0.9 1.1) :`true` 1.4 :!type "Float (single-precision)")
    (:`OnCompleted`
      (set `CharacterMovementComponent.GravityScale` 1.0 (`Character.CharacterMovement` (`self.Crabe`)))
      (`self.FinishedSkill`)
      (`self.MoreWeight` (`/Game/AI/AIC_Crabe.AC_Backward` (`self.AIC Crabe`)) 0.1 0.2)
      (`self.MoreWeight` (`/Game/AI/AIC_Crabe.AC_Straf` (`self.AIC Crabe`)) 0.1 0.2)
      (`self.MoreWeight` (`/Game/AI/AIC_Crabe.OKAC_StrafeWithoutFocus` (`self.AIC Crabe`)) 0.1 0.2))))