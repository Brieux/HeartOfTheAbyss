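; AC_Bombardement is an AI ability for the Crabe character that rains waves of sky bombs over a fixed world area.
; Activation, skipped during stagger security, turns on the attack glow and plays the bombardment montage.
; Each montage notify advances a counter that selects the wave's bomb count, height and following flag, then spawns indexed BP_BombeInTheSky actors at random XY positions.
; Montage blend-out stops the glow and finishes the skill.
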(event `self.ReceiveBeginPlay`
  (`parent.ReceiveBeginPlay`))

(event `self.ReceiveTick`
  (params (DeltaSeconds :type "Float (single-precision)"))
  (`parent.ReceiveTick` DeltaSeconds))

(event `self.Activation`
  (params (IsMovementAbility :type Boolean))
  (bind _counter (`self.Counter`))
  (bind _crabe (`self.Crabe`))
  (if (not (`/Game/Characters/Enemy/Boss/Crabe/BP_Crabe.isDoingStagger_Security` (`self.Crabe`)))
    (`parent.Activation` false)
    (set `self.Counter` 0)
    (`/Game/Characters/Enemy/Boss/Crabe/BP_Crabe.GlowingAttacking` _crabe)
    (`|PlayMontage` (`Character.Mesh` _crabe) "/Game/Characters/Enemy/Boss/Crabe/ModularMesh/Anim_Retarget_VF/AM_Bombardement.AM_Bombardement"
      (:`OnBlendOut`
        (`/Game/Characters/Enemy/Boss/Crabe/BP_Crabe.StopGlowingAttacking` _crabe)
        (`self.FinishedSkill`))
      (:`OnNotifyBegin`
        (`/Engine/EditorBlueprintResources/StandardMacros.IncrementInt` (`self.Counter`)
          (:`  `
            (for _index (range (+ (select `int` (`self.Counter`) :`0` 0 :`1` 35 :`2` 8 :`3` 35) 1))
              (`|SpawnActorFromClass` "/Game/Characters/Enemy/Boss/Crabe/BP_BombeInTheSky.BP_BombeInTheSky_C" (`Actor.GetTransform` _crabe) "Undefined" "OverrideRootScale" null (`KismetMathLibrary.MakeVector` (`KismetMathLibrary.RandomFloatInRange` 12370.0 25260.0) (`KismetMathLibrary.RandomFloatInRange` -31160.0 -23400.0) (select `int` _counter :`0` 0.0 :`1` 3300.0 :`2` 2900.0 :`3` 2700.0)) (select `int` _counter :`0` false :`1` false :`2` true :`3` false) (`KismetMathLibrary.Conv_IntToDouble` _index) null))))))))