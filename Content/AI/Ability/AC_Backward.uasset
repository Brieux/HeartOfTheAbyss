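; AC_Backward is an AI skill component that makes the crab retreat from the player.
; Activation extrapolates past the crab, away from the player, and writes a random reachable point near there to the blackboard with the InMove flag.
; It also raises the selection weight of the Pistolet, PinceZlag, CoupDeMarteau and CoupDePince skills.
; Tick watches InMove and calls FinishedSkill once the blackboard clears it.
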(event `self.ReceiveTick`
  (params (DeltaSeconds :type "Float (single-precision)"))
  (if (`self.inMove`)
    (if (not (`BlackboardComponent.GetValueAsBool` (`AIBlueprintHelperLibrary.GetBlackboard` (`self.AIC Crabe`)) "InMove"))
      (set `self.inMove` false)
      (`self.FinishedSkill`))))

(event `self.Activation`
  (bind _returnvalue (`AIBlueprintHelperLibrary.GetBlackboard` (`self.AIC Crabe`)))
  (bind (_randomlocation _returnvalue_2) (`NavigationSystemV1.K2_GetRandomReachablePointInRadius` (`KismetMathLibrary.VLerp` (`Actor.K2_GetActorLocation` (`self.Player`)) (`Actor.K2_GetActorLocation` (`self.Crabe`)) 5.0) (`self.CloseRadius`) null null))
  (if _returnvalue_2
    (`BlackboardComponent.SetValueAsVector` _returnvalue "Location" _randomlocation)
    (`BlackboardComponent.SetValueAsBool` _returnvalue "InMove" true)
    (set `self.inMove` true)
    (for _array_element (`/Game/AI/AIC_Crabe.acSkills` (`self.AIC Crabe`))
      (bind _returnvalue_3 (`GameplayStatics.GetObjectClass` _array_element))
      (if (or (== _returnvalue_3 "/Game/AI/Ability/AC_Pistolet.AC_Pistolet_C") (== _returnvalue_3 "/Game/AI/Ability/AC_PinceZlag.AC_PinceZlag_C") (== _returnvalue_3 "/Game/AI/Ability/AC_CoupDeMarteau.AC_CoupDeMarteau_C") (== _returnvalue_3 "/Game/AI/Ability/AC_CoupDePince.AC_CoupDePince_C"))
        (`self.MoreWeight` _array_element 0.1 0.2)))))

(event `self.ReceiveBeginPlay`
  (`parent.ReceiveBeginPlay`))