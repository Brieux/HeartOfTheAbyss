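; AC_Skill is a component for the crab enemy's AI skills, caching the SeaWatcher player, the crab and its AI controller at begin play.
; Each tick it counts down a cooldown and raises a selection weight by a random rate.
; Activation restarts the cooldown, rerolls a low weight (range depends on movement abilities) and blocks new skills on the controller.
; FinishedSkill unblocks the controller and requests its next action, while MoreWeight adds a clamped random boost.
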(event `self.ReceiveBeginPlay`
  (bind _returnvalue (`GameplayStatics.GetActorOfClass` "/Game/Characters/SeaWatcher/BP_SeaWatcher.BP_SeaWatcher_C"))
  (set `self.Player` _returnvalue)
  (bind _returnvalue_2 (`GameplayStatics.GetActorOfClass` "/Game/Characters/Enemy/Boss/Crabe/BP_Crabe.BP_Crabe_C"))
  (bind _output_get (set `self.Crabe` _returnvalue_2))
  (bind _asaic_crabe (cast `/Game/AI/AIC_Crabe` (`Pawn.GetController` _output_get)))
  (set `self.AIC Crabe` _asaic_crabe))

(event `self.ReceiveTick`
  (params (DeltaSeconds :type "Float (single-precision)"))
  (set `self.CD` (`KismetMathLibrary.FClamp` (- (`self.CD`) DeltaSeconds) 0.0 (`self.CDBase`)))
  (set `self.Weight` (+ (`self.Weight`) (* DeltaSeconds (`KismetMathLibrary.RandomFloatInRange` 0.05 0.08)))))

(event `Activation`
  (params (IsMovementAbility :type Boolean))
  (set `self.CD` (`self.CDBase`))
  (set `self.Weight` (`KismetMathLibrary.RandomFloatInRange` (`KismetMathLibrary.SelectFloat` 0.05 0.15 IsMovementAbility) (`KismetMathLibrary.SelectFloat` 0.1 0.25 IsMovementAbility)))
  (set `/Game/AI/AIC_Crabe.CanDoNewSkill` false (`self.AIC Crabe`)))

(event `FinishedSkill`
  (bind _aic_crabe (`self.AIC Crabe`))
  (set `/Game/AI/AIC_Crabe.CanDoNewSkill` true _aic_crabe)
  (`/Game/AI/AIC_Crabe.NewAction` _aic_crabe))

(event `MoreWeight`
  (params (Min :type "Float (double-precision)" :default 0.4) (Max :type "Float (double-precision)" :default 0.6))
  (set `self.Weight` (`KismetMathLibrary.FClamp` (+ (`self.Weight`) (`KismetMathLibrary.RandomFloatInRange` Min Max)))))