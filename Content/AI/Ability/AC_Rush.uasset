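; AI ability component for the crab enemy's rush attack, a high-speed charge.
; Activation boosts movement, starts the glow and plays a preparation montage, whose blend-out sets blackboard movement keys, ignores selected collision channels and starts a timeout.
; StopRush restores movement and focus, adjusts other abilities' selection weights via MoreWeight and finishes the skill.
; It shares BreakRush's collision logic, returning weak-point boxes to overlap.
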(event `self.ReceiveBeginPlay`
  (`parent.ReceiveBeginPlay`))

(event `self.ReceiveTick`
  (params (DeltaSeconds :type "Float (single-precision)"))
  (`parent.ReceiveTick` DeltaSeconds))

(event `BreakRush`
  (bind _crabe (`self.Crabe`))
  (bind _boxweakpoint (`/Game/Characters/Enemy/Boss/Crabe/BP_Crabe.BoxWeakPoint` _crabe))
  (bind _capsulecomponent (`Character.CapsuleComponent` _crabe))
  (`PrimitiveComponent.SetCollisionResponseToChannel` _capsulecomponent "ECC_GameTraceChannel2" "ECR_Ignore" :!label _label)
  (`PrimitiveComponent.SetCollisionResponseToChannel` (`/Game/Characters/Enemy/Boss/Crabe/BP_Crabe.RealHitCollider` _crabe) "ECC_GameTraceChannel2" "ECR_Ignore")
  (`PrimitiveComponent.SetCollisionResponseToChannel` _capsulecomponent "ECC_WorldDynamic" "ECR_Ignore")
  (`PrimitiveComponent.SetCollisionResponseToChannel` (`/Game/Characters/Enemy/Boss/Crabe/BP_Crabe.RealHitCollider` _crabe) "ECC_WorldDynamic" "ECR_Ignore")
  (`PrimitiveComponent.SetCollisionResponseToChannel` _boxweakpoint "ECC_GameTraceChannel2" "ECR_Overlap")
  (`PrimitiveComponent.SetCollisionResponseToChannel` (`/Game/Characters/Enemy/Boss/Crabe/BP_Crabe.Box2` _crabe) "ECC_GameTraceChannel2" "ECR_Overlap")
  (`PrimitiveComponent.SetCollisionResponseToChannel` _boxweakpoint "ECC_WorldDynamic" "ECR_Overlap")
  (`PrimitiveComponent.SetCollisionResponseToChannel` (`/Game/Characters/Enemy/Boss/Crabe/BP_Crabe.Box2` _crabe) "ECC_WorldDynamic" "ECR_Overlap"))

(event `self.Activation`
  (params (IsMovementAbility :type Boolean))
  (bind _returnvalue (`AIBlueprintHelperLibrary.GetBlackboard` (`self.AIC Crabe`)))
  (bind _capsulecomponent (`Character.CapsuleComponent` (`self.Crabe`)))
  (`parent.Activation` true)
  (bind _returnvalue_2 (`GameplayStatics.GetActorOfClass` "/Game/Characters/Enemy/Boss/Crabe/BP_Crabe.BP_Crabe_C"))
  (set `/Game/Characters/Enemy/Boss/Crabe/BP_Crabe.ActivAttackRush?` true _returnvalue_2)
  (`/Game/Characters/Enemy/Boss/Crabe/BP_Crabe.GlowingAttacking` _returnvalue_2)
  (bind _charactermovement (`Character.CharacterMovement` _returnvalue_2))
  (set `CharacterMovementComponent.BrakingDecelerationWalking` 10000.0 _charactermovement)
  (set `CharacterMovementComponent.MaxWalkSpeed` 10000.0 _charactermovement)
  (set `CharacterMovementComponent.MaxAcceleration` 10000.0 _charactermovement)
  (`|PlayMontage` (`Character.Mesh` (`self.Crabe`)) "/Game/Characters/Enemy/Boss/Crabe/ModularMesh/Anim_Retarget_VF/AM_PreparationRush_VF.AM_PreparationRush_VF" 1.1
    (:`OnBlendOut`
      (`BlackboardComponent.SetValueAsEnum` _returnvalue "Direction" (enumliteral `/Game/AI/Enum_Direction` "NewEnumerator6"))
      (`BlackboardComponent.SetValueAsBool` _returnvalue "InMove" true)
      (set `self.inMove` true)
      (bind _returnvalue_3 (`KismetSystemLibrary.K2_SetTimerDelegate` (delegate `StopRush`) 10.0))
      (set `self.TimerResetRush` _returnvalue_3)
      (`PrimitiveComponent.SetCollisionResponseToChannel` _capsulecomponent "ECC_GameTraceChannel2" "ECR_Ignore")
      (`PrimitiveComponent.SetCollisionResponseToChannel` (`/Game/Characters/Enemy/Boss/Crabe/BP_Crabe.BoxWeakPoint` (`self.Crabe`)) "ECC_GameTraceChannel2" "ECR_Ignore")
      (`PrimitiveComponent.SetCollisionResponseToChannel` (`/Game/Characters/Enemy/Boss/Crabe/BP_Crabe.Box2` (`self.Crabe`)) "ECC_GameTraceChannel2" "ECR_Ignore")
      (`PrimitiveComponent.SetCollisionResponseToChannel` (`/Game/Characters/Enemy/Boss/Crabe/BP_Crabe.RealHitCollider` (`self.Crabe`)) "ECC_GameTraceChannel2" "ECR_Ignore")
      (`PrimitiveComponent.SetCollisionResponseToChannel` _capsulecomponent "ECC_WorldDynamic" "ECR_Ignore")
      (`PrimitiveComponent.SetCollisionResponseToChannel` (`/Game/Characters/Enemy/Boss/Crabe/BP_Crabe.BoxWeakPoint` (`self.Crabe`)) "ECC_WorldDynamic" "ECR_Ignore")
      (`PrimitiveComponent.SetCollisionResponseToChannel` (`/Game/Characters/Enemy/Boss/Crabe/BP_Crabe.Box2` (`self.Crabe`)) "ECC_WorldDynamic" "ECR_Ignore")
      (`PrimitiveComponent.SetCollisionResponseToChannel` (`/Game/Characters/Enemy/Boss/Crabe/BP_Crabe.RealHitCollider` (`self.Crabe`)) "ECC_WorldDynamic" "ECR_Ignore"))))

(event `StopRush`
  (bind _crabe (`self.Crabe`))
  (bind _crabe_2 (`self.Crabe`))
  (bind _charactermovement (`Character.CharacterMovement` _crabe))
  (bind _charactermovement_2 (`Character.CharacterMovement` _crabe_2))
  (`|ExecutionSequence`
    (:`then_0`
      (if (`KismetSystemLibrary.K2_IsValidTimerHandle` (`self.TimerResetRush`))
        (`KismetSystemLibrary.K2_ClearAndInvalidateTimerHandle` (`self.TimerResetRush`))))
    (:`then_1`
      (set `CharacterMovementComponent.MaxWalkSpeed` 800.0 _charactermovement_2)
      (set `CharacterMovementComponent.MaxAcceleration` 700.0 _charactermovement_2)
      (`/Game/Characters/Enemy/Boss/Crabe/BP_Crabe.StopGlowingAttacking` _crabe_2)
      (set `/Game/Characters/Enemy/Boss/Crabe/BP_Crabe.ActivAttackRush?` false _crabe_2)
      (`BlackboardComponent.SetValueAsBool` (`AIBlueprintHelperLibrary.GetBlackboard` (`self.AIC Crabe`)) "InMove" false)
      (set `self.inMove` false)
      (`self.MoreWeight` (`/Game/AI/AIC_Crabe.AC_Backward` (`self.AIC Crabe`)) 0.1 0.2)
      (`self.MoreWeight` (`/Game/AI/AIC_Crabe.AC_Straf` (`self.AIC Crabe`)) 0.1 0.2)
      (`self.MoreWeight` (`/Game/AI/AIC_Crabe.OKAC_StrafeWithoutFocus` (`self.AIC Crabe`)) 0.1 0.2)
      (`self.MoreWeight` (`/Game/AI/AIC_Crabe.AC_CoupDePince` (`self.AIC Crabe`)) 0.1 0.2)
      (`self.MoreWeight` (`/Game/AI/AIC_Crabe.OKAC_CoupDePinceAR` (`self.AIC Crabe`)) 0.1 0.2)
      (set `MovementComponent.Velocity` (0.0 0.0 0.0) _charactermovement)
      (set `CharacterMovementComponent.BrakingDecelerationWalking` 512.0 _charactermovement)
      (set `CharacterMovementComponent.RotationRate` (struct :`Yaw` 360.0) _charactermovement)
      (`KismetSystemLibrary.DelayUntilNextTick`)
      (set `/Game/Characters/Enemy/Boss/Crabe/BP_Crabe.IsFocusing?` true _crabe)
      (`self.FinishedSkill`))
    (:`then_2`
      (goto _label))))