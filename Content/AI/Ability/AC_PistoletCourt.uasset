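; Crab AI ability component for the short "PistoletCourt" attack, skipped while the crab is in its stagger-security state.
; On activation it starts the crab's attack glow, then two random rolls pick a single montage (75%) or three chained plays (25%).
; Montage notifies trigger controller vibration, plus camera shake on all but the chain's last play.
; The final blend-out stops the glow and finishes the skill.
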(event `self.ReceiveBeginPlay`
  (`parent.ReceiveBeginPlay`))

(event `self.ReceiveTick`
  (params (DeltaSeconds :type "Float (single-precision)"))
  (`parent.ReceiveTick` DeltaSeconds))

(event `self.Activation`
  (params (IsMovementAbility :type Boolean))
  (bind _crabe (`self.Crabe`))
  (if (not (`/Game/Characters/Enemy/Boss/Crabe/BP_Crabe.isDoingStagger_Security` (`self.Crabe`)))
    (`parent.Activation` false)
    (bind _returnvalue (`GameplayStatics.GetActorOfClass` "/Game/Characters/Enemy/Boss/Crabe/BP_Crabe.BP_Crabe_C"))
    (`/Game/Characters/Enemy/Boss/Crabe/BP_Crabe.GlowingAttacking` _returnvalue)
    (if (`KismetMathLibrary.RandomBool`)
      (if (`KismetMathLibrary.RandomBool`)
        (`|PlayMontage` (`Character.Mesh` (`self.Crabe`)) "/Game/Characters/Enemy/Boss/Crabe/ModularMesh/Anim_Retarget_VF/Anim_PistoletCourt1_Montage.Anim_PistoletCourt1_Montage"
          (:`OnBlendOut`
            (`|PlayMontage` (`Character.Mesh` (`self.Crabe`)) "/Game/Characters/Enemy/Boss/Crabe/ModularMesh/Anim_Retarget_VF/Anim_PistoletCourt1_Montage.Anim_PistoletCourt1_Montage"
              (:`OnBlendOut`
                (`|PlayMontage` (`Character.Mesh` (`self.Crabe`)) "/Game/Characters/Enemy/Boss/Crabe/ModularMesh/Anim_Retarget_VF/Anim_PistoletCourt1_Montage.Anim_PistoletCourt1_Montage"
                  (:`OnBlendOut`
                    (`/Game/Characters/Enemy/Boss/Crabe/BP_Crabe.StopGlowingAttacking` _crabe :!label _label)
                    (`self.FinishedSkill`))
                  (:`OnNotifyBegin`
                    (`PlayerController.K2_ClientPlayForceFeedback` (`GameplayStatics.GetPlayerController` 0) "/Game/GeneralSettings/FFE_Vibration.FFE_Vibration" "None" false false false :!label _label_2))))
              (:`OnNotifyBegin`
                (`GameplayStatics.PlayWorldCameraShake` "/Game/GeneralSettings/BP_CamShakeXPlodeLittle.BP_CamShakeXPlodeLittle_C" (`SceneComponent.K2_GetComponentLocation` (`/Game/Characters/SeaWatcher/BP_SeaWatcher.Camera` (cast `/Game/Characters/SeaWatcher/BP_SeaWatcher` (`GameplayStatics.GetPlayerCharacter` 0) :!pure true))) :!label _label_3)
                (goto _label_2))))
          (:`OnNotifyBegin`
            (goto _label_3)))
        (else
          (`|PlayMontage` (`Character.Mesh` _crabe) "/Game/Characters/Enemy/Boss/Crabe/ModularMesh/Anim_Retarget_VF/Anim_PistoletCourt1_Montage.Anim_PistoletCourt1_Montage" :!label _label_4
            (:`OnBlendOut`
              (goto _label))
            (:`OnNotifyBegin`
              (goto _label_3)))))
      (else
        (goto _label_4)))))