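; AC_JumpBack is an AI ability that makes the Crabe perform a backward jump.
; On activation, it runs only if the Crabe is not in stagger security, then calls the parent activation.
; It finds the BP_Crabe actor in the level and plays the AM_BackJump montage on its mesh.
; When the montage completes, it signals that the skill is finished.
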(event `self.ReceiveBeginPlay`
  (`parent.ReceiveBeginPlay`))

(event `self.ReceiveTick`
  (params (DeltaSeconds :type "Float (single-precision)"))
  (`parent.ReceiveTick` DeltaSeconds))

(event `self.Activation`
  (params (IsMovementAbility :type Boolean))
  (if (not (`/Game/Characters/Enemy/Boss/Crabe/BP_Crabe.isDoingStagger_Security` (`self.Crabe`)))
    (`parent.Activation` false)
    (bind _returnvalue (`GameplayStatics.GetActorOfClass` "/Game/Characters/Enemy/Boss/Crabe/BP_Crabe.BP_Crabe_C"))
    (`|PlayMontage` (`Character.Mesh` _returnvalue) "/Game/Characters/Enemy/Boss/Crabe/ModularMesh/AnimRetarget/AM_BackJump.AM_BackJump"
      (:`OnCompleted`
        (`self.FinishedSkill`)))))