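; AC_Crachat is an AI ability for the Crabe that plays its spit (crachat) attack montage.
; On activation it calls the parent logic, starts the Crabe's attack glow and plays the montage.
; Playback is faster when the Crabe is staggered, otherwise its rate varies slightly at random.
; When the montage blends out, the glow stops and the skill reports itself finished.
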(event `self.ReceiveBeginPlay`
  (`parent.ReceiveBeginPlay`))

(event `self.ReceiveTick`
  (params (DeltaSeconds :type "Float (single-precision)"))
  (`parent.ReceiveTick` DeltaSeconds))

(event `self.Activation`
  (params (IsMovementAbility :type Boolean))
  (bind _crabe (`self.Crabe`))
  (`parent.Activation` false)
  (`/Game/Characters/Enemy/Boss/Crabe/BP_Crabe.GlowingAttacking` (`self.Crabe`))
  (`|PlayMontage` (`Character.Mesh` _crabe) "/Game/Characters/Enemy/Boss/Crabe/Anim/AM_Crachat_VF.AM_Crachat_VF" (select `bool` (`/Game/Characters/Enemy/Boss/Crabe/BP_Crabe.IsStagger` _crabe) :`false` (`KismetMathLibrary.RandomFloatInRange` 0.9 1.1) :`true` 1.4 :!type "Float (single-precision)")
    (:`OnBlendOut`
      (`/Game/Characters/Enemy/Boss/Crabe/BP_Crabe.StopGlowingAttacking` (`self.Crabe`))
      (`self.FinishedSkill`))))