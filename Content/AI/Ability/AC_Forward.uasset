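; AC_Forward is an AI ability for the crab AI that biases skill weighting toward a set of attack skills.
; On Activation, it loops over the AICCrabe skill list and picks out Pistolet, PinceZlag, CoupDeMarteau and CoupDePince by exact class match.
; Each match receives a MoreWeight call with a small min/max range; the ability itself contains no movement logic.
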(event `self.ReceiveBeginPlay`
  (`parent.ReceiveBeginPlay`))

(event `self.Activation`
  (for _array_element (`/Game/AI/AIC_Crabe.acSkills` (`self.AIC Crabe`))
    (bind _returnvalue (`GameplayStatics.GetObjectClass` _array_element))
    (if (or (== _returnvalue "/Game/AI/Ability/AC_Pistolet.AC_Pistolet_C") (== _returnvalue "/Game/AI/Ability/AC_PinceZlag.AC_PinceZlag_C") (== _returnvalue "/Game/AI/Ability/AC_CoupDeMarteau.AC_CoupDeMarteau_C") (== _returnvalue "/Game/AI/Ability/AC_CoupDePince.AC_CoupDePince_C"))
      (`self.MoreWeight` _array_element 0.1 0.2))))