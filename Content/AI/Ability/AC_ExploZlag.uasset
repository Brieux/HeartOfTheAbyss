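; AC_ExploZlag is an AI skill component for the Crabe that detonates the spikes in the level.
; Activation plays the invocation montage on the Crabe's mesh and, on a notify, calls XplodeZlag on every BP_Spike actor.
; It then finishes the skill, adds weight to the forward ability and removes itself from the AI controller's skill list.
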(event `self.ReceiveBeginPlay`
  (`parent.ReceiveBeginPlay`))

(event `self.ReceiveTick`
  (params (DeltaSeconds :type "Float (single-precision)"))
  (`parent.ReceiveTick` DeltaSeconds))

(event `self.Activation`
  (params (IsMovementAbility :type Boolean))
  (bind _aic_crabe (`self.AIC Crabe`))
  (`parent.Activation` false)
  (`|PlayMontage` (`/Game/Characters/Enemy/Boss/Crabe/BP_Crabe.SkeletalMesh` (`self.Crabe`)) "/Game/Characters/Enemy/Boss/Crabe/Anim/AM_Invocation.AM_Invocation"
    (:`OnNotifyBegin`
      (bind _outactors (`GameplayStatics.GetAllActorsOfClass` "/Game/Characters/Enemy/Boss/Crabe/BP_Spike.BP_Spike_C"))
      (for _array_element _outactors
        (`/Game/Characters/Enemy/Boss/Crabe/BP_Spike.xplodeZlag` _array_element))
      (`self.FinishedSkill`)
      (`self.MoreWeight` (`/Game/AI/AIC_Crabe.AC_Forward` _aic_crabe) 0.25 0.35)
      (`KismetArrayLibrary.Array_RemoveItem` (`/Game/AI/AIC_Crabe.acSkills` _aic_crabe) (`/Game/AI/AIC_Crabe.AC_ExploZlag` _aic_crabe)))))