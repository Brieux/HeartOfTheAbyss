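; Crab AI ability component that staggers the crab, interrupting its current skills and movement.
; Activation, gated by a security flag and a DoOnce re-armed via ResetStag, cancels other abilities' timers and plays the stagger montage.
; Its notify starts Niagara VFX and pulls Block and Tunnel from the Backpack.
; Completion starts a random UnStagger timer (VFX duration rolled separately), which restores Block, plus Tunnel in one behaviour phase.
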(event `self.Activation`
  (params (IsMovementAbility :type Boolean))
  (bind _returnvalue (`KismetMathLibrary.RandomFloatInRange` 20.0 30.0))
  (bind _aic_crabe (`self.AIC Crabe`))
  (bind _aic_crabe_2 (`self.AIC Crabe`))
  (bind _ns_stagger (`/Game/Characters/Enemy/Boss/Crabe/BP_Crabe.NS Stagger` (`self.Crabe`)))
  (bind _backpack (`/Game/AI/AIC_Crabe.Backpack` _aic_crabe))
  (`KismetSystemLibrary.PrintString` "Hello")
  (if (not (`/Game/Characters/Enemy/Boss/Crabe/BP_Crabe.isDoingStagger_Security` (`self.Crabe`)))
    (`parent.Activation` false)
    (`/Engine/EditorBlueprintResources/StandardMacros.DoOnce` false :!label _label
      (:`Completed`
        (set `/Game/Characters/Enemy/Boss/Crabe/BP_Crabe.isDoingStagger_Security` true (`self.Crabe`))
        (`self.FinishedSkill`)
        (set `/Game/AI/AIC_Crabe.CanDoNewSkill` false (`self.AIC Crabe`))
        (`self.RemoveAllActivities`)
        (set `/Game/Characters/Enemy/Boss/Crabe/BP_Crabe.IsFocusing?` false (`self.Crabe`))
        (set `/Game/Characters/Enemy/Boss/Crabe/BP_Crabe.IsStagger` true (`self.Crabe`))
        (`|PlayMontage` (`Character.Mesh` (`self.Crabe`)) "/Game/Characters/Enemy/Boss/Crabe/ModularMesh/Anim_Retarget_VF/AM_Stagger_VF.AM_Stagger_VF"
          (:`OnCompleted`
            (`KismetSystemLibrary.K2_SetTimerDelegate` (delegate `UnStagger`) _returnvalue)
            (`NiagaraComponent.SetVariableFloat` _ns_stagger "ValueTimeStagger" _returnvalue)
            (`/Game/AI/Ability/OKAC_CoupDeMarteau.OpenGateAfterStagger` (`/Game/AI/AIC_Crabe.AC_CoupDeMarteau` (`self.AIC Crabe`)))
            (set `/Game/Characters/Enemy/Boss/Crabe/BP_Crabe.isDoingStagger_Security` false (`self.Crabe`))
            (if (`|EnumEquality` (`/Game/AI/AIC_Crabe.Phase&Comportement` _aic_crabe_2) "NewEnumerator0")
              (`/Game/AI/AIC_Crabe.AddInBackBackAfterFirstStagger` _aic_crabe_2))
            (`self.FinishedSkill`))
          (:`OnNotifyBegin`
            (`self.Activate` _ns_stagger true)
            (`KismetArrayLibrary.Array_RemoveItem` _backpack (`/Game/AI/AIC_Crabe.AC_Block` _aic_crabe))
            (`KismetArrayLibrary.Array_RemoveItem` _backpack (`/Game/AI/AIC_Crabe.AC_Tunnel` _aic_crabe))))))))

(event `self.ReceiveBeginPlay`
  (`parent.ReceiveBeginPlay`))

(event `ResetStag`
  (goto _label :!via `Reset`))

(event `UnStagger`
  (bind _aic_crabe (`self.AIC Crabe`))
  (set `/Game/Characters/Enemy/Boss/Crabe/BP_Crabe.IsStagger` false (`self.Crabe`))
  (`self.Deactivate` (`/Game/Characters/Enemy/Boss/Crabe/BP_Crabe.NS Stagger` (`self.Crabe`)))
  (`KismetArrayLibrary.Array_Add` (`/Game/AI/AIC_Crabe.Backpack` _aic_crabe) (`/Game/AI/AIC_Crabe.AC_Block` _aic_crabe))
  (if (`|EnumEquality` (`/Game/AI/AIC_Crabe.Phase&Comportement` _aic_crabe) "NewEnumerator0")
    (`KismetArrayLibrary.Array_Add` (`/Game/AI/AIC_Crabe.Backpack` _aic_crabe) (`/Game/AI/AIC_Crabe.AC_Tunnel` _aic_crabe))))

(event `RemoveAllActivities`
  (bind _aic_crabe (`self.AIC Crabe`))
  (bind _aic_crabe_2 (`self.AIC Crabe`))
  (bind _ac_rush (`/Game/AI/AIC_Crabe.AC_Rush` _aic_crabe))
  (bind _timerresetrush (`/Game/AI/Ability/AC_Rush.TimerResetRush` _ac_rush))
  (bind _handler (`/Game/AI/Ability/AC_Block.Handler` (`/Game/AI/AIC_Crabe.AC_Block` _aic_crabe)))
  (bind _handler_2 (`/Game/AI/Ability/OKAC_StrafeWithoutFocus.Handler` (`/Game/AI/AIC_Crabe.OKAC_StrafeWithoutFocus` _aic_crabe_2)))
  (bind _handler_3 (`/Game/AI/Ability/OKAC_Forward.Handler` (`/Game/AI/AIC_Crabe.AC_Forward` _aic_crabe_2)))
  (bind _handler_4 (`/Game/AI/Ability/OKAC_Backward.Handler` (`/Game/AI/AIC_Crabe.AC_Backward` _aic_crabe_2)))
  (bind _handler_5 (`/Game/AI/Ability/AC_NewStrafe.Handler` (`/Game/AI/AIC_Crabe.AC_NewStrafe` _aic_crabe_2)))
  (`SkeletalMeshComponent.Stop` (`Character.Mesh` (`self.Crabe`)))
  (`|ExecutionSequence`
    (:`then_0`
      (if (`KismetSystemLibrary.K2_IsValidTimerHandle` _handler)
        (`KismetSystemLibrary.K2_ClearAndInvalidateTimerHandle` _handler)))
    (:`then_1`
      (if (`KismetSystemLibrary.K2_IsValidTimerHandle` _timerresetrush)
        (`KismetSystemLibrary.K2_ClearAndInvalidateTimerHandle` _timerresetrush)
        (`/Game/AI/Ability/AC_Rush.BreakRush` _ac_rush)))
    (:`then_2`
      (set `/Game/AI/Ability/AC_Tunnel.InMove` false (`/Game/AI/AIC_Crabe.AC_Tunnel` _aic_crabe)))
    (:`then_3`
      (`/Game/AI/Ability/OKAC_CoupDeMarteau.CloseGateStagger` (`/Game/AI/AIC_Crabe.AC_CoupDeMarteau` _aic_crabe)))
    (:`then_4`
      (`|ExecutionSequence`
        (:`then_0`
          (`BlackboardComponent.SetValueAsBool` (`AIBlueprintHelperLibrary.GetBlackboard` (`self.AIC Crabe`)) "InMove" false))
        (:`then_1`
          (set `CharacterMovementComponent.MaxWalkSpeed` 800.0 (`Character.CharacterMovement` (`self.Crabe`))))
        (:`then_2`
          (if (`KismetSystemLibrary.K2_IsValidTimerHandle` _handler_2)
            (`KismetSystemLibrary.K2_ClearAndInvalidateTimerHandle` _handler_2)))
        (:`then_3`
          (if (`KismetSystemLibrary.K2_IsValidTimerHandle` _handler_5)
            (`KismetSystemLibrary.K2_ClearAndInvalidateTimerHandle` _handler_5)))
        (:`then_4`
          (if (`KismetSystemLibrary.K2_IsValidTimerHandle` _handler_3)
            (`KismetSystemLibrary.K2_ClearAndInvalidateTimerHandle` _handler_3)))
        (:`then_5`
          (if (`KismetSystemLibrary.K2_IsValidTimerHandle` _handler_4)
            (`KismetSystemLibrary.K2_ClearAndInvalidateTimerHandle` _handler_4)))))))