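; BP_BreakWall is a breakable wall actor with a cinematic for the player's BP_SeaWatcher.
; CinematiqueLaunch runs once, disabling input, switching the view to the cine camera and playing the level sequence, then a duration-based timer restores input and blends back to the player.
; A separate Explode event triggers a Field to break the wall and makes the Box ignore all collision.
; The crab AI Tunnel call is disconnected.
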(event `self.ReceiveBeginPlay`)

(event `CinematiqueLaunch`
  (bind _returnvalue (`GameplayStatics.GetPlayerController` 0))
  (bind _asbp_sea_watcher (cast `/Game/Characters/SeaWatcher/BP_SeaWatcher` (`GameplayStatics.GetPlayerCharacter` 0)))
  (bind _output_get (set `self.As BP Sea Watcher` _asbp_sea_watcher))
  (bind _output_get_2 (set `self.PlayerController_REF` _returnvalue))
  (`/Engine/EditorBlueprintResources/StandardMacros.DoOnce` false
    (:`Completed`
      (`self.DisableInput` _asbp_sea_watcher _output_get_2)
      (`self.DisableInput` _output_get _output_get_2)
      (bind _outactor (`LevelSequencePlayer.CreateLevelSequencePlayer` "/Game/Cinematics/LevelSequenceBreakWall.LevelSequenceBreakWall"))
      (`PlayerController.SetViewTargetWithBlend` _returnvalue (`ActorComponent.GetOwner` (`self.CineCamera`)) 0.0 "VTBlend_Linear" 0.0 false)
      (bind _sequenceplayer (`LevelSequenceActor.SequencePlayer` _outactor))
      (`MovieSceneSequencePlayer.Play` _sequenceplayer)
      (`KismetSystemLibrary.K2_SetTimerDelegate` (delegate `Enable Input`) (`TimeManagementBlueprintLibrary.Conv_QualifiedFrameTimeToSeconds` (`MovieSceneSequencePlayer.GetDuration` _sequenceplayer))))))

(event `self.triggertestLevelSequence.OnComponentBeginOverlap`
  (params (OverlappedComponent :type "PrimitiveComponent Object Reference") (OtherActor :type "Actor Object Reference") (OtherComp :type "PrimitiveComponent Object Reference") (OtherBodyIndex :type Integer) (bFromSweep :type Boolean) (SweepResult :type "HitResult Structure (by ref)")))

(event `Enable Input`
  (`self.EnableInput` (`self.As BP Sea Watcher`) (`self.PlayerController_REF`))
  (`PlayerController.SetViewTargetWithBlend` (`self.PlayerController_REF`) (`GameplayStatics.GetPlayerCharacter` 0) 0.5 "VTBlend_Linear" 0.0 false))

(event `Explode`
  (`/Engine/EditorResources/FieldNodes/FS_MasterField.CE_Trigger` (`self.Field`))
  (`PrimitiveComponent.SetCollisionResponseToAllChannels` (`self.Box`) "ECR_Ignore"))

(fn `UserConstructionScript`)