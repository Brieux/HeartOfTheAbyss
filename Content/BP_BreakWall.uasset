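; BP_BreakWall is a boss-fight wall that runs a cinematic transition after phase one and can be shattered.
; CinematiqueLaunch crossfades boss music, ducks the sound mix, switches data layers, then plays a level sequence once with the player hidden and input disabled.
; A timer matched to the sequence length restores the player and camera, notifies the crab and activates a barrier.
; Explode triggers a field and disables box collision.
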(event `self.ReceiveBeginPlay`
  ;[1 0.53 0.6303] fin music boss 01 début musique amb 02
  (bind _outactors (`GameplayStatics.GetAllActorsOfClass` "/Game/Sound/Music/BP_Switch_Music_CalmToVnr.BP_Switch_Music_CalmToVnr_C"))
  (set `self.StopMusic_BossFight_Phase01` (`|GetArrayItem` _outactors)))

(event `CinematiqueLaunch`
  (bind _returnvalue (`GameplayStatics.GetPlayerController` 0))
  ;[1 0.53 0.6303] fin music boss 01 début musique amb 02
  (`AudioComponent.FadeOut` (`/Game/Sound/Music/BP_Switch_Music_CalmToVnr.Music_Boss_Test` (`self.StopMusic_BossFight_Phase01`)) 4.0 0.0 "Linear")
  (`AudioComponent.FadeIn` (`/Game/Sound/Music/BP_Switch_Music_CalmToVnr.Music_Post_Phase01` (`self.StopMusic_BossFight_Phase01`)) 5.0 1.0 0.0 "Linear")
  ;[0.955 0.2919 1] MixModifier
  (`GameplayStatics.PushSoundMixModifier` "/Game/Sound/Mix/DuckCinematic.DuckCinematic")
  (`DataLayerSubsystem.SetDataLayerRuntimeState` (subsystem `DataLayerSubsystem`) (`self.In Data Layer_1`) "Activated" false)
  (`DataLayerSubsystem.SetDataLayerRuntimeState` (subsystem `DataLayerSubsystem`) (`self.In Data Layer`) "Activated" false)
  (`DataLayerSubsystem.SetDataLayerRuntimeState` (subsystem `DataLayerSubsystem`) (`self.In Data Layer_0`) "Unloaded" false)
  (bind _asbp_sea_watcher (cast `/Game/Characters/SeaWatcher/BP_SeaWatcher` (`GameplayStatics.GetPlayerCharacter` 0)))
  (bind _output_get (set `self.As BP Sea Watcher` _asbp_sea_watcher))
  (bind _output_get_2 (set `self.PlayerController_REF` _returnvalue))
  (`/Engine/EditorBlueprintResources/StandardMacros.DoOnce` false
    (:`Completed`
      (`self.DisableInput` _asbp_sea_watcher _output_get_2)
      (`self.DisableInput` _output_get _output_get_2)
      (`self.SetActorHiddenInGame` (`self.As BP Sea Watcher`) true)
      (bind _outactor (`LevelSequencePlayer.CreateLevelSequencePlayer` "/Game/CUTSCENES/FinPhase1/LevelSequenceBreakWall.LevelSequenceBreakWall"))
      (`PlayerController.SetViewTargetWithBlend` _returnvalue (`ActorComponent.GetOwner` (`self.CineCamera`)) 0.0 "VTBlend_Linear" 0.0 false)
      (bind _sequenceplayer (`LevelSequenceActor.SequencePlayer` _outactor))
      (`MovieSceneSequencePlayer.Play` _sequenceplayer)
      (`KismetSystemLibrary.K2_SetTimerDelegate` (delegate `Enable Input`) (`TimeManagementBlueprintLibrary.Conv_QualifiedFrameTimeToSeconds` (`MovieSceneSequencePlayer.GetDuration` _sequenceplayer))))))

(event `Enable Input`
  (`self.EnableInput` (`self.As BP Sea Watcher`) (`self.PlayerController_REF`))
  (`self.SetActorHiddenInGame` (`self.As BP Sea Watcher`) false)
  (`PlayerController.SetViewTargetWithBlend` (`self.PlayerController_REF`) (`GameplayStatics.GetPlayerCharacter` 0) 1.0 "VTBlend_Linear" 0.0 false)
  (`/Game/Characters/Enemy/Boss/Crabe/BP_Crabe.CinmeticOver` (`self.Crabe`))
  (`/Game/GeneralSettings/BP_BarriereDeBebz.Activate` (`self.BarriereRef`))
  ;[0.955 0.2919 1] MixModifier
  (`GameplayStatics.PopSoundMixModifier` "/Game/Sound/Mix/DuckCinematic.DuckCinematic"))

(event `Explode`
  (`/Engine/EditorResources/FieldNodes/FS_MasterField.CE_Trigger` (`self.Field`))
  (`PrimitiveComponent.SetCollisionResponseToAllChannels` (`self.Box`) "ECR_Ignore"))

(fn `UserConstructionScript`)