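; Giant clam spawn prop that runs the game's intro, holding the hidden SeaWatcher until the player struggles out.
; Gates make claw and tail inputs alternate; each accepted press rocks the shells with sound, shake and FOV effects.
; The press counter advances a spline target that Tick interpolates the intro camera toward.
; From four presses the clam can open, with bubbles, blending the view to the character and restoring controls through an exit montage.
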(event `self.ReceiveBeginPlay`
  (bind _returnvalue (pcsubsystem `EnhancedInputLocalPlayerSubsystem` (`GameplayStatics.GetPlayerController` 0)))
  (bind _returnvalue_2 (`|CreateWidget` "/Game/UI/UI_FadeBlackScreen.UI_FadeBlackScreen_C"))
  (bind _output_get (set `self.REF_BlackScreen_UI` _returnvalue_2))
  (`UserWidget.AddToViewport` _returnvalue_2 -1)
  (`UserWidget.AddToViewport` _output_get -1)
  (`/Game/UI/UI_FadeBlackScreen.Fade_Out` _output_get)
  (bind _returnvalue_3 (`GameplayStatics.GetActorOfClass` "/Game/Intro_Camera.Intro_Camera_C"))
  (set `self.CameraREF` _returnvalue_3)
  (set `self.Target` (`SplineComponent.GetLocationAtDistanceAlongSpline` (`/Game/Intro_Camera.Spline` (`self.CameraREF`)) 0.0 "World"))
  (bind _asbp_sea_watcher (cast `/Game/Characters/SeaWatcher/BP_SeaWatcher` (`GameplayStatics.GetPlayerCharacter` 0)))
  (bind _output_get_2 (set `self.As BP Sea Watcher` _asbp_sea_watcher))
  (`SceneComponent.SetVisibility` (`Character.CapsuleComponent` _output_get_2) false true)
  (`/Engine/EditorBlueprintResources/StandardMacros.IsValid` _returnvalue
    (:`Is Valid`
      (`EnhancedInputSubsystemInterface.AddMappingContext` _returnvalue "/Game/GeneralSettings/Input/IMC_SeaWatcherDansBenitier.IMC_SeaWatcherDansBenitier" 0 (struct))
      ;[1 1 1] Intro camera
      (`PlayerController.SetViewTargetWithBlend` (`GameplayStatics.GetPlayerController` 0) (`self.CameraREF`) 0.0 "VTBlend_Linear" 0.0 false)
      (bind (_direction _newtrack_0) (`Timeline|Timeline_2` :!label _label)
        (:`Update`
          (`SceneComponent.K2_SetRelativeLocation` (`CameraActor.CameraComponent` (`self.CameraREF`)) (`KismetMathLibrary.MakeVector` (`KismetMathLibrary.Lerp` 50.0 0.0 _newtrack_0) (`KismetMathLibrary.Lerp` 50.0 0.0 _newtrack_0)) false false))))))

(event `EnhancedInput|/Game/GeneralSettings/Input/IA_ClawToQuit`
  (params (ActionValue :type Boolean) (ElapsedSeconds :type "Float (double-precision)") (TriggeredSeconds :type "Float (double-precision)") (InputAction :type "InputAction Object Reference" :default "/Game/GeneralSettings/Input/IA_ClawToQuit.IA_ClawToQuit"))
  (bind _cameraref (`self.CameraREF`))
  (bind _benitierhaut (`self.BenitierHaut`))
  (bind _benitierbas (`self.BenitierBas`))
  (bind (_relativerotation_roll _relativerotation_pitch _relativerotation_yaw) (`KismetMathLibrary.BreakRotator` (`SceneComponent.RelativeRotation` (`self.BenitierHaut`))))
  (bind _spline (`/Game/Intro_Camera.Spline` (`self.CameraREF`)))
  (bind (_relativerotation_roll_2 _relativerotation_pitch_2 _relativerotation_yaw_2) (`KismetMathLibrary.BreakRotator` (`SceneComponent.RelativeRotation` _benitierhaut)))
  (bind (_relativerotation_roll_3 _relativerotation_pitch_3 _relativerotation_yaw_3) (`KismetMathLibrary.BreakRotator` (`SceneComponent.RelativeRotation` _benitierbas)))
  (:`Started`
    (`|ExecutionSequence`
      (:`then_0`
        (`/Engine/EditorBlueprintResources/StandardMacros.Gate` true :!label _label_2
          (:`Exit`
            (bind _result (`/Engine/EditorBlueprintResources/StandardMacros.IncrementInt` (`self.Counter`))
              (:`  `
                (set `self.Counter` _result)
                (set `self.Target` (`SplineComponent.GetLocationAtDistanceAlongSpline` _spline (* (/ (`self.Counter`) 4.0) (`SplineComponent.GetSplineLength` _spline)) "World") :!label _label_3)
                (`self.StopFirstTimeline`)
                (`GameplayStatics.PlaySoundAtLocation` "/Game/Sound/Benitier/Cue_Benitier_TryOpen.Cue_Benitier_TryOpen" (`SceneComponent.K2_GetComponentLocation` (`Character.Mesh` (`GameplayStatics.GetPlayerCharacter` 0))) (struct) 1.0 1.0 0.0 null null null null)
                (`|ExecutionSequence`
                  (:`then_0`
                    (`|MultiGate` true true 0
                      (:`Out 0`
                        (bind (_direction _newtrack_0) (`Timeline|Timeline_1` :!label _label_4)
                          (:`Update`
                            (`SceneComponent.K2_SetRelativeRotation` (`self.BenitierHaut`) (`KismetMathLibrary.MakeRotator` (`KismetMathLibrary.Lerp` 0.0 15.0 _newtrack_0) _relativerotation_pitch _relativerotation_yaw) false false)
                            ;[1 1 1] intro camera
                            (`PlayerController.K2_ClientPlayForceFeedback` (`GameplayStatics.GetPlayerController` 0) "/Game/GeneralSettings/FFE_VibrationMini.FFE_VibrationMini" "None" false false false)
                            (`KismetSystemLibrary.K2_SetTimerDelegate` (delegate `CustomEvent_0`) 0.25))
                          (:`Finished`
                            (if (>= (`self.Counter`) 4)
                              (`EnhancedInputSubsystemInterface.RemoveMappingContext` (pcsubsystem `EnhancedInputLocalPlayerSubsystem` (`GameplayStatics.GetPlayerController` 0)) "/Game/GeneralSettings/Input/IMC_SeaWatcherDansBenitier.IMC_SeaWatcherDansBenitier" (struct))
                              (`self.Open/Close`)
                              (`GameplayStatics.PlaySoundAtLocation` "/Game/Sound/Benitier/Cue_Benitier_Open.Cue_Benitier_Open" (`SceneComponent.K2_GetComponentLocation` (`Character.Mesh` (`GameplayStatics.GetPlayerCharacter` 0))) (struct) 1.0 1.0 0.0 null null null null)))))
                      (:`Out 1`
                        (goto _label_4 :!via `Reverse`))))
                  (:`then_1`
                    (bind (_direction_2 __) (`Timeline|Oscillate benitier` :!via `PlayFromStart`)
                      (:`Update`
                        (bind _returnvalue (`KismetMathLibrary.Lerp` 3.0 -3.0 __))
                        (`SceneComponent.K2_SetRelativeRotation` _benitierhaut (`KismetMathLibrary.MakeRotator` _relativerotation_roll_2 _returnvalue _relativerotation_yaw_2) false false)
                        (`SceneComponent.K2_SetRelativeRotation` _benitierbas (`KismetMathLibrary.MakeRotator` _relativerotation_roll_3 _returnvalue _relativerotation_yaw_3) false false))))
                  (:`then_2`
                    (bind (_direction_3 _newtrack_0_2) (`Timeline|Fov FX` :!via `PlayFromStart`)
                      (:`Update`
                        (`CameraComponent.SetFieldOfView` (`CameraActor.CameraComponent` _cameraref) (`KismetMathLibrary.Lerp` 40.0 45.0 _newtrack_0_2))
                        (`GameplayStatics.PlayWorldCameraShake` "/Game/GeneralSettings/BP_CamShake.BP_CamShake_C" (`SceneComponent.K2_GetComponentLocation` (`Actor.RootComponent` _cameraref)) 0.0 1.0))))))))))
      (:`then_1`
        (goto _label_5 :!via `Open`))
      (:`then_2`
        (goto _label_2 :!via `Close`)))))

(event `StopFirstTimeline`
  ;[1 1 1] Intro camera
  ;;[1 1 1] pour le déplacement de la spline
  (goto _label :!via `Stop`))

(event `EnhancedInput|/Game/GeneralSettings/Input/IA_TailToQuit`
  (params (ActionValue :type Boolean) (ElapsedSeconds :type "Float (double-precision)") (TriggeredSeconds :type "Float (double-precision)") (InputAction :type "InputAction Object Reference" :default "/Game/GeneralSettings/Input/IA_TailToQuit.IA_TailToQuit"))
  (:`Started`
    (`|ExecutionSequence`
      (:`then_0`
        (`/Engine/EditorBlueprintResources/StandardMacros.Gate` false :!label _label_5
          (:`Exit`
            (bind _result (`/Engine/EditorBlueprintResources/StandardMacros.IncrementInt` (`self.Counter`))
              (:`  `
                (set `self.Counter` _result)
                (goto _label_3))))))
      (:`then_1`
        (goto _label_2 :!via `Open`))
      (:`then_2`
        (goto _label_5 :!via `Close`)))))

(event `CustomEvent_0`
  ;[1 1 1] intro camera
  (`PlayerController.ClientStopForceFeedback` (`GameplayStatics.GetPlayerController` 0) "/Game/GeneralSettings/FFE_VibrationMini.FFE_VibrationMini" "None"))

(event `Open/Close`
  (bind _returnvalue (pcsubsystem `EnhancedInputLocalPlayerSubsystem` (`GameplayStatics.GetPlayerController` 0)))
  (bind (_relativerotation_roll _relativerotation_pitch _relativerotation_yaw) (`KismetMathLibrary.BreakRotator` (`SceneComponent.RelativeRotation` (`self.BenitierHaut`))))
  (`/Engine/EditorBlueprintResources/StandardMacros.FlipFlop` :!label _label_6
    (:`A`
      (bind (_direction _newtrack_0) (`Timeline|Timeline_0` :!label _label_7)
        (:`Update`
          (`SceneComponent.K2_SetRelativeRotation` (`self.BenitierHaut`) (`KismetMathLibrary.MakeRotator` (`KismetMathLibrary.Lerp` 0.0 -50.0 _newtrack_0) _relativerotation_pitch _relativerotation_yaw) false false)
          (`/Engine/EditorBlueprintResources/StandardMacros.DoOnce` false
            (:`Completed`
              (`ActorComponent.Activate` (`self.NS OpeningBubbles`) true)
              (`KismetSystemLibrary.Delay` 0.2)
              (`/Game/UI/BP_UI_InWorld.Deactivate` (`self.UIToDisable`))
              (`EnhancedInputSubsystemInterface.RemoveMappingContext` _returnvalue "/Game/GeneralSettings/Input/IMC_SeaWatcherDansBenitier.IMC_SeaWatcherDansBenitier" (struct))
              (`EnhancedInputSubsystemInterface.RemoveMappingContext` _returnvalue "/Game/GeneralSettings/Input/IMC_SeaWatcher.IMC_SeaWatcher" (struct))
              ;[1 1 1] intro camera
              (`PlayerController.SetViewTargetWithBlend` (`GameplayStatics.GetPlayerController` 0) (`self.As BP Sea Watcher`) 1.0 "VTBlend_Linear" 0.0 false)
              (`|PlayMontage` (`Character.Mesh` (`self.As BP Sea Watcher`)) "/Game/Characters/SeaWatcher/Animation/NEWRIG/AM_SortieBenitier_NR.AM_SortieBenitier_NR"
                (:`then`
                  (`/Game/Characters/SeaWatcher/BP_SeaWatcher.SpawnBenit` (`self.As BP Sea Watcher`))
                  (`SceneComponent.SetVisibility` (`Character.CapsuleComponent` (`self.As BP Sea Watcher`)) true true))
                (:`OnBlendOut`
                  (`EnhancedInputSubsystemInterface.AddMappingContext` _returnvalue "/Game/GeneralSettings/Input/IMC_SeaWatcher.IMC_SeaWatcher" 0 (struct))
                  (`PlayerController.K2_ClientPlayForceFeedback` (`GameplayStatics.GetPlayerController` 0) "/Game/GeneralSettings/FFE_Vibration.FFE_Vibration" "None" false false false)
                  (`KismetSystemLibrary.K2_SetTimerDelegate` (delegate `CustomEvent`) 0.5)
                  (set `/Game/Characters/SeaWatcher/BP_SeaWatcher.InClam?` false (`self.As BP Sea Watcher`)))))))))
    (:`B`
      (goto _label_7 :!via `Reverse`))))

(event `/Game/GeneralSettings/Int_Hittable.GetHit`
  (params (Dammage :type "Float (double-precision)") (PositionHited :type "Vector Structure") (ComboEnd :type Boolean) (`Missile?` :type Boolean) (ClawAttack :type Boolean) (ComboAttackValue :type "/Game/GeneralSettings/Enum_ComboType Enum" :default "NewEnumerator0"))
  (goto _label_6))

(event `self.ReceiveTick`
  (params (DeltaSeconds :type "Float (single-precision)"))
  (bind _cameracomponent (`CameraActor.CameraComponent` (`self.CameraREF`)))
  ;[0.5865 1 0.4136] pour la spline camera
  (`SceneComponent.K2_SetWorldLocation` _cameracomponent (`KismetMathLibrary.VInterpTo` (`SceneComponent.K2_GetComponentLocation` _cameracomponent) (`self.Target`) (`GameplayStatics.GetWorldDeltaSeconds`) 2.0) false false))

(event `CustomEvent`
  ;[1 1 1] intro camera
  (`PlayerController.ClientStopForceFeedback` (`GameplayStatics.GetPlayerController` 0) "/Game/GeneralSettings/FFE_Vibration.FFE_Vibration" "None"))

(fn `UserConstructionScript`)