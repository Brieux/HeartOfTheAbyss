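; Destructible pillar prop that, on a one-time Break event, topples away from the actor that broke it and shatters.
; It offsets the actor and counter-offsets its Scene component to shift the pivot, then a Timeline drives the tilt.
; While breaking, its Box damages BP_SeaWatcher or BP_Crabe, or sends hit messages to other Int_Hittable actors.
; After the fall, ten shards get physics and random cone impulses, then are destroyed after a delay.
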(event `Break`
  (bind _returnvalue_x (`KismetMathLibrary.BreakVector` (`self.GetActorScale3D`)))
  (bind (_returnvalue_x_2 _returnvalue_y _returnvalue_z) (`KismetMathLibrary.BreakVector` (`self.K2_GetActorLocation`)))
  (bind (_returnvalue_roll _returnvalue_pitch _returnvalue_yaw) (`KismetMathLibrary.BreakRotator` (`self.K2_GetActorRotation`)))
  (bind _box (`self.Box`))
  (bind (_initlocation_x _initlocation_y) (`KismetMathLibrary.BreakVector` (`self.InitLocation`)))
  (bind _returnvalue (/ 1.0 _returnvalue_x))
  (bind (_returnvalue_x_3 _returnvalue_y_2) (`KismetMathLibrary.BreakVector` (`KismetMathLibrary.GetDirectionUnitVector` (`self.K2_GetActorLocation` (`self.ActorThatBreakComeFrom`)) (`self.K2_GetActorLocation`))))
  (bind (_returnvalue_x_4 _returnvalue_y_3) (`KismetMathLibrary.BreakVector` (`KismetMathLibrary.GetDirectionUnitVector` (`self.K2_GetActorLocation` (`self.ActorThatBreakComeFrom`)) (`self.K2_GetActorLocation`))))
  (bind _returnvalue_2 (* _returnvalue_x_4 292.61))
  (bind _returnvalue_3 (* _returnvalue_y_3 292.61))
  (`/Engine/EditorBlueprintResources/StandardMacros.DoOnce` false
    (:`Completed`
      (`/Engine/EditorBlueprintResources/StandardMacros.IsValid` (`self.ActorThatBreakComeFrom`)
        (:`Is Valid`
          _)
        (:`Is Not Valid`
          (set `self.ActorThatBreakComeFrom` null)))
      (set `self.break?` true)
      (`ActorComponent.Activate` (`self.Box`) true)
      (`self.K2_SetActorLocation` (`KismetMathLibrary.MakeVector` (+ _initlocation_x (/ _returnvalue_2 _returnvalue)) (+ _initlocation_y (/ _returnvalue_3 _returnvalue)) _returnvalue_z))
      (`SceneComponent.K2_SetRelativeLocation` (`self.Scene`) (`KismetMathLibrary.MakeVector` (* _returnvalue_2 -1.0) (* _returnvalue_3 -1.0)) false false)
      (bind (_direction _newtrack_0) (`Timeline|Timeline_0`)
        (:`Update`
          (bind _returnvalue_4 (`KismetMathLibrary.Lerp` 0.0 92.0 _newtrack_0))
          (`self.K2_SetActorRotation` (`KismetMathLibrary.MakeRotator` (* _returnvalue_y_2 _returnvalue_4) (* _returnvalue_x_3 _returnvalue_4 -1.0) _returnvalue_yaw)))
        (:`Finished`
          (for _array_element (`self.AllShard`)
            (`PrimitiveComponent.SetSimulatePhysics` _array_element true)
            (`PrimitiveComponent.AddImpulse` _array_element (* (`KismetMathLibrary.RandomUnitVectorInConeInDegrees` (-1.0 0.0 0.0) 45.0) (`self.Strengh`)) "None" true))
          (`/Engine/EditorBlueprintResources/StandardMacros.IsValid` _box
            (:`Is Valid`
              (`ActorComponent.Deactivate` _box)
              (`ActorComponent.K2_DestroyComponent` _box))
            (:`Is Not Valid`
              _))
          (`KismetSystemLibrary.Delay` 3.0)
          (for _array_element_2 (`|MakeArray` (`self.PillardShard1`) (`self.PillardShard2`) (`self.PillardShard3`) (`self.PillardShard4`) (`self.PillardShard5`) (`self.PillardShard6`) (`self.PillardShard7`) (`self.PillardShard8`) (`self.PillardShard9`) (`self.PillardShard10`))
            (`ActorComponent.K2_DestroyComponent` _array_element_2)))))))

(event `self.ReceiveBeginPlay`
  (set `self.AllShard` (`|MakeArray` (`self.PillardShard1`) (`self.PillardShard2`) (`self.PillardShard3`) (`self.PillardShard4`) (`self.PillardShard5`) (`self.PillardShard6`) (`self.PillardShard7`) (`self.PillardShard8`) (`self.PillardShard9`) (`self.PillardShard10`)))
  (set `self.InitLocation` (`self.K2_GetActorLocation`))
  (`ActorComponent.Deactivate` (`self.Box`)))

(event `self.Box.OnComponentBeginOverlap`
  (params (OverlappedComponent :type "PrimitiveComponent Object Reference") (OtherActor :type "Actor Object Reference") (OtherComp :type "PrimitiveComponent Object Reference") (OtherBodyIndex :type Integer) (bFromSweep :type Boolean) (SweepResult :type "HitResult Structure (by ref)"))
  (if (`self.break?`)
    (bind _asbp_sea_watcher (cast `/Game/Characters/SeaWatcher/BP_SeaWatcher` OtherActor)
      (:`then`
        (`GameplayStatics.ApplyDamage` _asbp_sea_watcher 40.0)
        (`ActorComponent.K2_DestroyComponent` (`self.Box`) :!label _label))
      (:`CastFailed`
        (bind _asbp_crabe (cast `/Game/Characters/Enemy/Boss/Crabe/BP_Crabe` OtherActor)
          (:`then`
            (`GameplayStatics.ApplyDamage` _asbp_crabe 10.0)
            (goto _label))
          (:`CastFailed`
            (if (`KismetSystemLibrary.DoesImplementInterface` OtherActor "/Game/GeneralSettings/Int_Hittable.Int_Hittable_C")
              (message `/Game/GeneralSettings/Int_Hittable.GetHit` OtherActor 0.0 (0.0 0.0 0.0) false true false))))))))

(fn `UserConstructionScript`)