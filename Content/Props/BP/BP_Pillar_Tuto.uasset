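; Tutorial pillar that breaks once, damaging the first BP_SeaWatcher to overlap its hit box during the break.
; Break shifts the actor away from the breaker and counter-offsets the Scene component to move the pivot, then plays a timeline.
; When it finishes, ten shards get physics and random cone impulses, the box is removed, and shards are destroyed after a delay.
; The timeline-driven toppling rotation is unwired and never runs.
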(event `Break`
  (bind _returnvalue_x (`KismetMathLibrary.BreakVector` (`self.GetActorScale3D`)))
  (bind (_returnvalue_x_2 _returnvalue_y _returnvalue_z) (`KismetMathLibrary.BreakVector` (`self.K2_GetActorLocation`)))
  (bind _box (`self.Box`))
  (bind (_init_location_x _init_location_y) (`KismetMathLibrary.BreakVector` (`self.Init Location`)))
  (bind _returnvalue (/ 1.0 _returnvalue_x))
  (bind (_returnvalue_x_3 _returnvalue_y_2) (`KismetMathLibrary.BreakVector` (`KismetMathLibrary.GetDirectionUnitVector` (`self.K2_GetActorLocation` (`self.ActorThatBreakComeFrom`)) (`self.K2_GetActorLocation`))))
  (bind _returnvalue_2 (* _returnvalue_x_3 292.61))
  (bind _returnvalue_3 (* _returnvalue_y_2 292.61))
  (`/Engine/EditorBlueprintResources/StandardMacros.DoOnce` false
    (:`Completed`
      (`/Engine/EditorBlueprintResources/StandardMacros.IsValid` (`self.ActorThatBreakComeFrom`)
        (:`Is Valid`
          _)
        (:`Is Not Valid`
          (set `self.ActorThatBreakComeFrom` null)))
      (set `self.break?` true)
      (`ActorComponent.Activate` (`self.Box`) true)
      (`self.K2_SetActorLocation` (`KismetMathLibrary.MakeVector` (+ _init_location_x (/ _returnvalue_2 _returnvalue)) (+ _init_location_y (/ _returnvalue_3 _returnvalue)) _returnvalue_z))
      (`SceneComponent.K2_SetRelativeLocation` (`self.Scene`) (`KismetMathLibrary.MakeVector` (* _returnvalue_2 -1.0) (* _returnvalue_3 -1.0)) false false)
      (bind (_direction _newtrack_0) (`Timeline|Timeline_0`)
        (:`Finished`
          (for _array_element (`self.All Shard`)
            (`PrimitiveComponent.SetSimulatePhysics` _array_element true)
            (`PrimitiveComponent.AddImpulse` _array_element (* (`KismetMathLibrary.RandomUnitVectorInConeInDegrees` (-1.0 0.0 0.0) 45.0) (`self.Strengh`)) "None" true))
          (`/Engine/EditorBlueprintResources/StandardMacros.IsValid` _box
            (:`Is Valid`
              (`ActorComponent.Deactivate` _box)
              (`ActorComponent.K2_DestroyComponent` _box))
            (:`Is Not Valid`
              _))
          (`KismetSystemLibrary.Delay` 3.0)
          (for _array_element_2 (`self.All Shard`)
            (`ActorComponent.K2_DestroyComponent` _array_element_2)))))))

(event `self.ReceiveBeginPlay`
  (set `self.All Shard` (`|MakeArray` (`self.PillarShard1`) (`self.PillarShard2`) (`self.PillarShard3`) (`self.PillarShard4`) (`self.PillarShard5`) (`self.PillarShard6`) (`self.PillarShard7`) (`self.PillarShard8`) (`self.PillarShard9`) (`self.PillarShard10`)))
  (set `self.Init Location` (`self.K2_GetActorLocation`))
  (`ActorComponent.Deactivate` (`self.Box`)))

(event `self.Box.OnComponentBeginOverlap`
  (params (OverlappedComponent :type "PrimitiveComponent Object Reference") (OtherActor :type "Actor Object Reference") (OtherComp :type "PrimitiveComponent Object Reference") (OtherBodyIndex :type Integer) (bFromSweep :type Boolean) (SweepResult :type "HitResult Structure (by ref)"))
  (if (`self.break?`)
    (bind _asbp_sea_watcher (cast `/Game/Characters/SeaWatcher/BP_SeaWatcher` OtherActor))
    (`GameplayStatics.ApplyDamage` _asbp_sea_watcher 40.0)
    (`ActorComponent.K2_DestroyComponent` (`self.Box`))))

(fn `UserConstructionScript`)