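; Pillar platform prop made of static mesh pillars, configured entirely in the Construction Script with no active event logic.
; The BlackOrWhite flag picks one of two materials for slot 0 on each static mesh directly under the root.
; When Randomized is set, each of those meshes gets an unseeded random world Z scale between its current value and that plus MaxHeight, leaving X and Y unchanged.
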(fn `UserConstructionScript`
  (`|ExecutionSequence`
    (:`then_0`
      (for _array_element (`SceneComponent.GetChildrenComponents` (`self.DefaultSceneRoot`) false)
        (bind _asstatic_mesh_component (cast `StaticMeshComponent` _array_element))
        (if (`self.BlackOrWhite?`)
          (`PrimitiveComponent.SetMaterial` _asstatic_mesh_component 0 "/Game/Props/Material/Pillars/M_PillarSolo.M_PillarSolo")
          (else
            (`PrimitiveComponent.SetMaterial` _asstatic_mesh_component 0 "/Game/Props/Material/Pillars/M_PillarSoloV2.M_PillarSoloV2")))))
    (:`then_1`
      (if (`self.Randomized?`)
        (for _array_element_2 (`SceneComponent.GetChildrenComponents` (`self.DefaultSceneRoot`) false)
          (bind _asstatic_mesh_component_2 (cast `StaticMeshComponent` _array_element_2))
          (bind (_returnvalue_x _returnvalue_y _returnvalue_z) (`KismetMathLibrary.BreakVector` (`SceneComponent.K2_GetComponentScale` _asstatic_mesh_component_2)))
          (`SceneComponent.SetWorldScale3D` _asstatic_mesh_component_2 (`KismetMathLibrary.MakeVector` _returnvalue_x _returnvalue_y (`KismetMathLibrary.RandomFloatInRange` _returnvalue_z (+ _returnvalue_z (`self.MaxHeight`))))))))))