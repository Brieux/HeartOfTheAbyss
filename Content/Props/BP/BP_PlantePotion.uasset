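; Healing plant prop that, when hit, opens once and gives the player potions and health.
; GetHit drives the plant's anim blueprint, a petal dynamic-material fade and Niagara effects, then after delays adds clamped potions to BP_SeaWatcher.
; A timeline lerps health up to the capped value before removing the fruit.
; When flagged as a tutorial, it also shows a UI_Heal widget that follows above the player until UI_Disapear.
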(event `UI_Disapear`
  (if (`self.tutoIsEnable`)
    (bind _asui_heal (cast `/Game/UI/UI_Heal` (`WidgetComponent.GetWidget` (`self.Widget`))))
    (`/Game/UI/UI_Heal.Appear` _asui_heal false)
    (set `self.tutoIsEnable` false)))

(event `self.ReceiveTick`
  (params (DeltaSeconds :type "Float (single-precision)"))
  (bind (_returnvalue_x _returnvalue_y _returnvalue_z) (`KismetMathLibrary.BreakVector` (`self.K2_GetActorLocation` (`GameplayStatics.GetPlayerCharacter` 0))))
  (if (`self.tutoIsEnable`)
    (`SceneComponent.K2_SetWorldLocation` (`self.Widget`) (`KismetMathLibrary.MakeVector` _returnvalue_x _returnvalue_y (+ _returnvalue_z 450.0)) false false)))

(event `/Game/GeneralSettings/Int_Hittable.GetHit`
  (params (Dammage :type "Float (double-precision)") (PositionHited :type "Vector Structure") (ComboEnd :type Boolean) (`Missile?` :type Boolean) (ClawAttack :type Boolean))
  (`/Engine/EditorBlueprintResources/StandardMacros.DoOnce` false
    (:`Completed`
      (if (`self.Tuto`)
        (bind _asui_heal (cast `/Game/UI/UI_Heal` (`WidgetComponent.GetWidget` (`self.Widget`))))
        (`/Game/UI/UI_Heal.Appear` _asui_heal true)
        (set `self.tutoIsEnable` true))
      (bind _asabp_plante (cast `/Game/Props/PlantePotion/ABP_Plante` (`SkeletalMeshComponent.GetAnimInstance` (`self.Plante`))))
      (set `/Game/Props/PlantePotion/ABP_Plante.isOpen` true _asabp_plante)
      (`ActorComponent.Deactivate` (`self.NiagaraStandby`))
      (`self.SwitchColor`)
      (`KismetSystemLibrary.Delay` 0.4)
      (`ActorComponent.Activate` (`self.NS Plante Spore`) false)
      (`NiagaraFunctionLibrary.SpawnSystemAtLocation` "/Game/VFX/NiagaraSystem/NS_BubbleJet.NS_BubbleJet" (`self.K2_GetActorLocation`))
      (`SkeletalMeshComponent.PlayAnimation` (`self.fruit`) "/Game/Props/PlantePotion/Fruit/IdleFruit_Anim.IdleFruit_Anim" true)
      (`ActorComponent.Activate` (`self.NS_PLanteHeal`) true)
      (`KismetSystemLibrary.Delay` 2.4)
      (bind _asbp_sea_watcher (cast `/Game/Characters/SeaWatcher/BP_SeaWatcher` (`GameplayStatics.GetPlayerCharacter` 0)))
      (set `/Game/Characters/SeaWatcher/BP_SeaWatcher.NbPotions` (`KismetMathLibrary.Clamp` (+ (`/Game/Characters/SeaWatcher/BP_SeaWatcher.NbPotions` _asbp_sea_watcher) (`self.NbPotionGive`)) 0 (`/Game/Characters/SeaWatcher/BP_SeaWatcher.NbPotionMax` _asbp_sea_watcher)) _asbp_sea_watcher)
      (bind _health (`/Game/Characters/SeaWatcher/BP_SeaWatcher.Health` _asbp_sea_watcher))
      (set `self.Debuthealth` _health)
      (set `self.endHealth` (`KismetMathLibrary.Conv_IntToDouble` (`KismetMathLibrary.Clamp` (`KismetMathLibrary.FTrunc` (+ (`self.NbPvHeal`) _health)) 0 (`KismetMathLibrary.FTrunc` (`/Game/Characters/SeaWatcher/BP_SeaWatcher.MaxHealth` _asbp_sea_watcher)))))
      (bind (_direction _newtrack_0) (`Timeline|Timeline_1` :!via `PlayFromStart`)
        (:`Update`
          (set `/Game/Characters/SeaWatcher/BP_SeaWatcher.Health` (`KismetMathLibrary.Lerp` (`self.Debuthealth`) (`self.endHealth`) _newtrack_0) _asbp_sea_watcher))
        (:`Finished`
          (`ActorComponent.K2_DestroyComponent` (`self.fruit`))
          (`ActorComponent.Activate` (`self.NS TakingFruit`) false))))))

(event `SwitchColor`
  (`/Engine/EditorBlueprintResources/StandardMacros.FlipFlop`
    (:`A`
      (bind (_direction _newtrack_0) (`Timeline|Timeline_0` :!label _label)
        (:`Update`
          (`MaterialInstanceDynamic.SetScalarParameterValue` (`self.Mat`) "Param" _newtrack_0))))
    (:`B`
      (goto _label :!via `Reverse`))))

(fn `UserConstructionScript`
  (bind _returnvalue (`KismetMaterialLibrary.CreateDynamicMaterialInstance` "/Game/Props/PlantePotion/M_PetalesPlantePotion_Inst.M_PetalesPlantePotion_Inst"))
  (bind _output_get (set `self.Mat` _returnvalue))
  (`PrimitiveComponent.SetMaterial` (`self.Plante`) 1 _output_get))