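; BP_Hiding is a prop whose static mesh can fade out and back in through its material opacity.
; On BeginPlay it creates a dynamic material instance and applies it to the mesh's first slot.
; FadeOut plays and FadeIn reverses a shared timeline that drives the Opacity parameter.
; Two cross-resetting DoOnce gates let each direction fire only once until the opposite event is called.
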(event `self.ReceiveBeginPlay`
  (bind _returnvalue (`KismetMaterialLibrary.CreateDynamicMaterialInstance` (`self.MaterialInstance`)))
  (bind _output_get (set `self.MI` _returnvalue))
  (`PrimitiveComponent.SetMaterial` (`self.StaticMesh`) 0 _output_get))

(event `FadeOut`
  (`|ExecutionSequence`
    (:`then_0`
      (goto _label_3 :!via `Reset`))
    (:`then_1`
      (`/Engine/EditorBlueprintResources/StandardMacros.DoOnce` false :!label _label
        (:`Completed`
          (bind (_direction _newtrack_0) (`Timeline|Timeline_0` :!label _label_2)
            (:`Update`
              (`MaterialInstanceDynamic.SetScalarParameterValue` (`self.MI`) "Opacity" _newtrack_0))))))))

(event `FadeIn`
  (`|ExecutionSequence`
    (:`then_0`
      (goto _label :!via `Reset`))
    (:`then_1`
      (`/Engine/EditorBlueprintResources/StandardMacros.DoOnce` false :!label _label_3
        (:`Completed`
          (goto _label_2 :!via `Reverse`))))))

(fn `UserConstructionScript`)