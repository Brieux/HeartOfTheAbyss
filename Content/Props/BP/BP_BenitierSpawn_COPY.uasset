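; Giant clam (bénitier) spawn prop for the intro: hides the SeaWatcher at BeginPlay, switches to a traveling intro camera and adds an escape input context.
; Gated claw and tail inputs alternate to raise a counter, randomly rocking the upper shell with camera shake and FOV changes.
; At four or more, a FlipFlop, also triggered by GetHit, opens the shell with bubbles, reveals the player, blends the view back and plays an exit montage.
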(event `self.ReceiveBeginPlay`
  (bind _returnvalue (pcsubsystem `EnhancedInputLocalPlayerSubsystem` (`GameplayStatics.GetPlayerController` 0)))
  (bind _returnvalue_2 (`GameplayStatics.GetActorOfClass` "/Game/Intro_Camera.Intro_Camera_C"))
  (set `self.CameraREF` _returnvalue_2)
  (bind _asbp_sea_watcher (cast `/Game/Characters/SeaWatcher/BP_SeaWatcher` (`GameplayStatics.GetPlayerCharacter` 0)))
  (bind _output_get (set `self.As BP Sea Watcher` _asbp_sea_watcher))
  (`SceneComponent.SetVisibility` (`Character.CapsuleComponent` _output_get) false true)
  (`/Engine/EditorBlueprintResources/StandardMacros.IsValid` _returnvalue
    (:`Is Valid`
      (`EnhancedInputSubsystemInterface.AddMappingContext` _returnvalue "/Game/GeneralSettings/Input/IMC_SeaWatcherDansBenitier.IMC_SeaWatcherDansBenitier" 0 (struct))
      ;[1 1 1] Intro camera
      (`PlayerController.SetViewTargetWithBlend` (`GameplayStatics.GetPlayerController` 0) (`self.CameraREF`) 0.0 "VTBlend_Linear" 0.0 false)
      (bind (_direction _newtrack_0) (`Timeline|CameraTraveling`)
        (:`Update`
          (`SceneComponent.K2_SetRelativeLocation` (`CameraActor.CameraComponent` (`self.CameraREF`)) (`KismetMathLibrary.MakeVector` (`KismetMathLibrary.Lerp` 50.0 0.0 _newtrack_0) (`KismetMathLibrary.Lerp` 50.0 0.0 _newtrack_0)) false false))))))

(event `EnhancedInput|/Game/GeneralSettings/Input/IA_ClawToQuit`
  (params (ActionValue :type Boolean) (ElapsedSeconds :type "Float (double-precision)") (TriggeredSeconds :type "Float (double-precision)") (InputAction :type "InputAction Object Reference" :default "/Game/GeneralSettings/Input/IA_ClawToQuit.IA_ClawToQuit"))
  (bind _cameraref (`self.CameraREF`))
  (bind (_relativerotation_roll _relativerotation_pitch _relativerotation_yaw) (`KismetMathLibrary.BreakRotator` (`SceneComponent.RelativeRotation` (`self.BenitierHaut`))))
  (:`Started`
    (`|ExecutionSequence`
      (:`then_0`
        (`/Engine/EditorBlueprintResources/StandardMacros.Gate` true :!label _label
          (:`Exit`
            (bind _result (`/Engine/EditorBlueprintResources/StandardMacros.IncrementInt` (`self.Counter`))
              (:`  `
                (set `self.Counter` _result)
                (`|MultiGate` true true 0 :!label _label_2
                  (:`Out 0`
                    (bind (_direction _newtrack_0) (`Timeline|Timeline_1` :!label _label_3)
                      (:`Update`
                        (`SceneComponent.K2_SetRelativeRotation` (`self.BenitierHaut`) (`KismetMathLibrary.MakeRotator` (`KismetMathLibrary.Lerp` 0.0 15.0 _newtrack_0) _relativerotation_pitch _relativerotation_yaw) false false)
                        ;[1 1 1] intro camera
                        (`GameplayStatics.PlayWorldCameraShake` "/Game/GeneralSettings/BP_CamShake.BP_CamShake_C" (`SceneComponent.K2_GetComponentLocation` (`Actor.RootComponent` _cameraref)) 0.0 1.0)
                        (`CameraComponent.SetFieldOfView` (`CameraActor.CameraComponent` _cameraref) (`KismetMathLibrary.Lerp` 30.0 35.0 _newtrack_0)))
                      (:`Finished`
                        (if (>= (`self.Counter`) 4)
                          (`EnhancedInputSubsystemInterface.RemoveMappingContext` (pcsubsystem `EnhancedInputLocalPlayerSubsystem` (`GameplayStatics.GetPlayerController` 0)) "/Game/GeneralSettings/Input/IMC_SeaWatcherDansBenitier.IMC_SeaWatcherDansBenitier" (struct))
                          (`self.Open/Close`)))))
                  (:`Out 1`
                    (goto _label_3 :!via `Reverse`))))))))
      (:`then_1`
        (goto _label_4 :!via `Open`))
      (:`then_2`
        (goto _label :!via `Close`)))))

(event `EnhancedInput|/Game/GeneralSettings/Input/IA_TailToQuit`
  (params (ActionValue :type Boolean) (ElapsedSeconds :type "Float (double-precision)") (TriggeredSeconds :type "Float (double-precision)") (InputAction :type "InputAction Object Reference" :default "/Game/GeneralSettings/Input/IA_TailToQuit.IA_TailToQuit"))
  (:`Started`
    (`|ExecutionSequence`
      (:`then_0`
        (`/Engine/EditorBlueprintResources/StandardMacros.Gate` false :!label _label_4
          (:`Exit`
            (bind _result (`/Engine/EditorBlueprintResources/StandardMacros.IncrementInt` (`self.Counter`))
              (:`  `
                (set `self.Counter` _result)
                (goto _label_2))))))
      (:`then_1`
        (goto _label :!via `Open`))
      (:`then_2`
        (goto _label_4 :!via `Close`)))))

(event `Open/Close`
  (bind _as_bp_sea_watcher (`self.As BP Sea Watcher`))
  (bind (_relativerotation_roll _relativerotation_pitch _relativerotation_yaw) (`KismetMathLibrary.BreakRotator` (`SceneComponent.RelativeRotation` (`self.BenitierHaut`))))
  (`/Engine/EditorBlueprintResources/StandardMacros.FlipFlop` :!label _label_5
    (:`A`
      (bind (_direction _newtrack_0) (`Timeline|Timeline_0` :!label _label_6)
        (:`Update`
          (`SceneComponent.K2_SetRelativeRotation` (`self.BenitierHaut`) (`KismetMathLibrary.MakeRotator` (`KismetMathLibrary.Lerp` 0.0 -50.0 _newtrack_0) _relativerotation_pitch _relativerotation_yaw) false false)
          (`/Engine/EditorBlueprintResources/StandardMacros.DoOnce` false
            (:`Completed`
              (`ActorComponent.Activate` (`self.Niagara`) true))))
        (:`Finished`
          (`NiagaraFunctionLibrary.SpawnSystemAtLocation` "/Game/VFX/NiagaraSystem/NS_BubbleJet.NS_BubbleJet" (`self.K2_GetActorLocation`))
          (`/Game/Characters/SeaWatcher/BP_SeaWatcher.SpawnBenit` _as_bp_sea_watcher)
          (`SceneComponent.SetVisibility` (`Character.CapsuleComponent` _as_bp_sea_watcher) true true)
          (`EnhancedInputSubsystemInterface.RemoveMappingContext` (pcsubsystem `EnhancedInputLocalPlayerSubsystem` (`GameplayStatics.GetPlayerController` 0)) "/Game/GeneralSettings/Input/IMC_SeaWatcherDansBenitier.IMC_SeaWatcherDansBenitier" (struct))
          ;[1 1 1] intro camera
          (`PlayerController.SetViewTargetWithBlend` (`GameplayStatics.GetPlayerController` 0) (`self.As BP Sea Watcher`) 1.0 "VTBlend_Linear" 0.0 false)
          (`|PlayMontage` (`Character.Mesh` (`self.As BP Sea Watcher`)) "/Game/Characters/SeaWatcher/SortieBenitier/AM_SortieBenitier.AM_SortieBenitier"))))
    (:`B`
      (goto _label_6 :!via `Reverse`))))

(event `/Game/GeneralSettings/Int_Hittable.GetHit`
  (params (Dammage :type "Float (double-precision)") (PositionHited :type "Vector Structure") (ComboEnd :type Boolean) (`Missile?` :type Boolean) (ClawAttack :type Boolean))
  (goto _label_5))

(fn `UserConstructionScript`)