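; BP_ZlagZoneGround is a ground hazard that slows and damages BP_SeaWatcher while it is inside the Box.
; Overlap begin forces a crouch, activates a Niagara effect and starts a looping damage timer; overlap end reverses all three.
; While the player is caught, Tick writes both leg socket locations to the same Niagara Aim_Position parameter, so the left leg's value wins.
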(event `self.ReceiveTick`
  (params (DeltaSeconds :type "Float (single-precision)"))
  (if (`self.PlayerSlow`)
    (bind _returnvalue (`GameplayStatics.GetActorOfClass` "/Game/Characters/SeaWatcher/BP_SeaWatcher.BP_SeaWatcher_C"))
    (`|ExecutionSequence`
      (:`then_0`
        (set `self.SocketName` "Bind_Leg_R"))
      (:`then_1`
        (set `self.SocketName` "Bind_Leg_L")))
    (`NiagaraComponent.SetVariableVec3` (`self.Niagara1`) "Aim_Position" (`SceneComponent.GetSocketLocation` (`Character.Mesh` _returnvalue) (`self.SocketName`)))))

(event `ZlagCatchPlayer`
  (if (`self.PlayerSlow`)
    (`ActorComponent.Activate` (`self.Niagara1`) false)
    (else
      (`ActorComponent.Deactivate` (`self.Niagara1`)))))

(event `self.Box.OnComponentBeginOverlap`
  (params (OverlappedComponent :type "PrimitiveComponent Object Reference") (OtherActor :type "Actor Object Reference") (OtherComp :type "PrimitiveComponent Object Reference") (OtherBodyIndex :type Integer) (bFromSweep :type Boolean) (SweepResult :type "HitResult Structure (by ref)"))
  (bind _asbp_sea_watcher (cast `/Game/Characters/SeaWatcher/BP_SeaWatcher` OtherActor))
  (set `self.PlayerSlow` true)
  (`self.ZlagCatchPlayer`)
  (`Character.Crouch` _asbp_sea_watcher)
  (bind _returnvalue (`KismetSystemLibrary.K2_SetTimerDelegate` (delegate `DealDammage`) 1.0 true))
  (set `self.DOTHandler` _returnvalue))

(event `DealDammage`
  (bind _asbp_sea_watcher (cast `/Game/Characters/SeaWatcher/BP_SeaWatcher` (`GameplayStatics.GetPlayerCharacter` 0)))
  (`GameplayStatics.ApplyDamage` _asbp_sea_watcher 5.0))

(event `self.Box.OnComponentEndOverlap`
  (params (OverlappedComponent :type "PrimitiveComponent Object Reference") (OtherActor :type "Actor Object Reference") (OtherComp :type "PrimitiveComponent Object Reference") (OtherBodyIndex :type Integer))
  (bind _asbp_sea_watcher (cast `/Game/Characters/SeaWatcher/BP_SeaWatcher` OtherActor))
  (set `self.PlayerSlow` false)
  (`self.ZlagCatchPlayer`)
  (`Character.UnCrouch` _asbp_sea_watcher)
  (if (`KismetSystemLibrary.K2_IsValidTimerHandle` (`self.DOTHandler`))
    (`KismetSystemLibrary.K2_ClearAndInvalidateTimerHandle` (`self.DOTHandler`))))

(fn `UserConstructionScript`
  (`ActorComponent.SetAutoActivate` (`self.Niagara1`) false))