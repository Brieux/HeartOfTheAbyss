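; BP_Benitier is an underwater giant clam prop that toggles open and closed through its Open/Close event or when hit.
; A FlipFlop alternately plays and reverses a timeline that lerps the upper shell's pitch.
; When the timeline finishes in either direction, it spawns a Niagara bubble jet at the actor's location and reapplies the rotation.
; The player cast to BP_SeaWatcher after each rotation update drives nothing.
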(event `Open/Close`
  (bind (_relativerotation_roll _relativerotation_pitch _relativerotation_yaw) (`KismetMathLibrary.BreakRotator` (`SceneComponent.RelativeRotation` (`self.BenitierHaut`))))
  (`/Engine/EditorBlueprintResources/StandardMacros.FlipFlop` :!label _label
    (:`A`
      (bind (_direction _newtrack_0) (`Timeline|Timeline_0` :!label _label_2)
        (:`Update`
          _)
        (:`Finished`
          (`NiagaraFunctionLibrary.SpawnSystemAtLocation` "/Game/VFX/NiagaraSystem/NS_BubbleJet.NS_BubbleJet" (`self.K2_GetActorLocation`))))
      (`SceneComponent.K2_SetRelativeRotation` (`self.BenitierHaut`) (`KismetMathLibrary.MakeRotator` _relativerotation_roll (`KismetMathLibrary.Lerp` 0.0 50.0 _newtrack_0) _relativerotation_yaw) false false)
      (cast `/Game/Characters/SeaWatcher/BP_SeaWatcher` (`GameplayStatics.GetPlayerCharacter` 0)))
    (:`B`
      (goto _label_2 :!via `Reverse`))))

(event `/Game/GeneralSettings/Int_Hittable.GetHit`
  (params (Dammage :type "Float (double-precision)") (PositionHited :type "Vector Structure") (ComboEnd :type Boolean) (`Missile?` :type Boolean) (ClawAttack :type Boolean))
  (goto _label))

(fn `UserConstructionScript`)