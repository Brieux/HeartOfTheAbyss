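; BP_SoclePillar is a pillar base prop whose hit points (PV) drop when hit, breaking its referenced pillar at zero.
; GetHit subtracts clamped damage behind a DoOnce that ResetHit re-arms, while HitByCrabe subtracts a fixed amount.
; Two gates cross-close so whichever source depletes PV first is credited, player or BP_Crabe, via ActorThatBreakComeFrom before calling Break.
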(event `/Game/GeneralSettings/Int_Hittable.GetHit`
  (params (Dammage :type "Float (double-precision)") (PositionHited :type "Vector Structure"))
  (bind _pillarref (`self.PillarRef`))
  (bind _pillarref_2 (`self.PillarRef`))
  (`/Engine/EditorBlueprintResources/StandardMacros.DoOnce` false :!label _label
    (:`Completed`
      (bind _output_get (set `self.PV` (- (`self.PV`) (`KismetMathLibrary.FClamp` Dammage 0.0 2.0))))
      (if (<= _output_get 0.0)
        (`|ExecutionSequence`
          (:`then_0`
            (`/Engine/EditorBlueprintResources/StandardMacros.Gate` false :!label _label_2
              (:`Exit`
                (set `/Game/Props/BP/BP_DestroyPillar.ActorThatBreakComeFrom` (`GameplayStatics.GetPlayerCharacter` 0) _pillarref_2)
                (`/Game/Props/BP/BP_DestroyPillar.Break` _pillarref_2))))
          (:`then_1`
            (goto _label_3 :!via `Close`)))))))

(event `ResetHit`
  (goto _label :!via `Reset`))

(event `HitByCrabe`
  (bind _pillarref (`self.PillarRef`))
  (bind _output_get (set `self.PV` (- (`self.PV`) 2.0)))
  (if (<= _output_get 0.0)
    (`|ExecutionSequence`
      (:`then_0`
        (`/Engine/EditorBlueprintResources/StandardMacros.Gate` false :!label _label_3
          (:`Exit`
            (bind _returnvalue (`GameplayStatics.GetActorOfClass` "/Game/Characters/Enemy/Boss/Crabe/BP_Crabe.BP_Crabe_C"))
            (set `/Game/Props/BP/BP_DestroyPillar.ActorThatBreakComeFrom` _returnvalue _pillarref)
            (`/Game/Props/BP/BP_DestroyPillar.Break` _pillarref))))
      (:`then_1`
        (goto _label_2 :!via `Close`)))))

(fn `UserConstructionScript`)