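; Kelp prop that varies its look per placed instance, with all logic in the construction script and none in the event graph.
; It randomizes uniform scale around Size, animation playback speed within SpeedMin and SpeedMax, and yaw, with a fixed roll.
; The material comes from the MatIndex map: a random key when RandomMat is set, otherwise the last key flagged true.
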(fn `UserConstructionScript`
  (bind _matindex (`self.MatIndex`))
  (`SceneComponent.SetRelativeScale3D` (`self.algue`) (`KismetMathLibrary.Conv_DoubleToVector` (+ (`self.Size`) (* (`KismetMathLibrary.RandomFloatInRange` -1.0 1.0) 12.0))))
  (set `GeometryCacheComponent.PlaybackSpeed` (`KismetMathLibrary.RandomFloatInRange` (`self.SpeedMin`) (`self.SpeedMax`)) (`self.algue`))
  (`SceneComponent.K2_SetRelativeRotation` (`self.algue`) (`KismetMathLibrary.MakeRotator` 90.0 0.0 (`KismetMathLibrary.RandomFloatInRange` 0.0 360.0)) false false)
  (if (`self.RandomMat`)
    (bind _keys (`BlueprintMapLibrary.Map_Keys` _matindex))
    (`PrimitiveComponent.SetMaterial` (`self.algue`) 0 (`KismetArrayLibrary.Array_Random` _keys))
    (else
      (bind _keys_2 (`BlueprintMapLibrary.Map_Keys` _matindex))
      (for _array_element _keys_2
        (if (`BlueprintMapLibrary.Map_Find` _matindex _array_element)
          (`PrimitiveComponent.SetMaterial` (`self.algue`) 0 _array_element))))))