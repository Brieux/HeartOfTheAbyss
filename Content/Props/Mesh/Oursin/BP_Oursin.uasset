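; Sea urchin hazard that glows and extends its spikes when BP_SeaWatcher enters its Colision volume, reversing both on exit.
; Timelines drive spike brightness and scale, with flags deferring retraction until deployment finishes and Armed toggling at each finish.
; HitSphere damages the player on entry while armed.
; When the spike timeline finishes with the player inside, Hit repeats damage through a delayed self-call, calling ResetDammage after each delay.
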(event `Glowing`
  ;[1 1 1] GLOW EFFECT
  (bind (_direction _brightnessoftime) (`Timeline|Timeline_GlowTime` :!label _label)
    (:`Update`
      (`MeshComponent.SetScalarParameterValueOnMaterials` (`self.Spikes`) "Brightness" _brightnessoftime))))

(event `StopGlowing`
  ;[1 1 1] GLOW EFFECT
  (goto _label :!via `Reverse`))

(event `self.colision.OnComponentBeginOverlap`
  (params (OverlappedComponent :type "PrimitiveComponent Object Reference") (OtherActor :type "Actor Object Reference") (OtherComp :type "PrimitiveComponent Object Reference") (OtherBodyIndex :type Integer) (bFromSweep :type Boolean) (SweepResult :type "HitResult Structure (by ref)"))
  ;[1 1 1] Detect Player
  (cast `/Game/Characters/SeaWatcher/BP_SeaWatcher` OtherActor)
  (`self.Glowing`)
  (set `self.bouleboule` false)
  (bind (_direction _deploiment _retractation) (`Timeline|Déploiement` :!label _label_2)
    (:`Update`
      (`SceneComponent.SetRelativeScale3D` (`self.Spikes`) (`KismetMathLibrary.VLerp` (0.4 0.4 0.4) (1.0 1.0 1.0) (select `ETimelineDirection` _direction :`Forward` _deploiment :`Backward` _retractation))))
    (:`Finished`
      (set `self.Armed` (not (`self.Armed`)))
      (set `self.bouleboule` true)
      (if (not (`KismetArrayLibrary.Array_IsEmpty` (`PrimitiveComponent.GetOverlappingActors` (`self.HitSphere`) "/Game/Characters/SeaWatcher/BP_SeaWatcher.BP_SeaWatcher_C")))
        (`self.Hit`))
      (if (`self.bouleboule2`)
        (set `self.bouleboule2` false)
        (goto _label_2 :!via `Reverse`)))))

(event `self.colision.OnComponentEndOverlap`
  (params (OverlappedComponent :type "PrimitiveComponent Object Reference") (OtherActor :type "Actor Object Reference") (OtherComp :type "PrimitiveComponent Object Reference") (OtherBodyIndex :type Integer))
  ;[1 1 1] Detect Player
  (cast `/Game/Characters/SeaWatcher/BP_SeaWatcher` OtherActor)
  (`self.StopGlowing`)
  (set `self.bouleboule2` true)
  (if (`self.bouleboule`)
    (goto _label_2 :!via `Reverse`)))

(event `self.HitSphere.OnComponentBeginOverlap`
  (params (OverlappedComponent :type "PrimitiveComponent Object Reference") (OtherActor :type "Actor Object Reference") (OtherComp :type "PrimitiveComponent Object Reference") (OtherBodyIndex :type Integer) (bFromSweep :type Boolean) (SweepResult :type "HitResult Structure (by ref)"))
  ;[1 1 1] Hit Player
  (bind _asbp_sea_watcher (cast `/Game/Characters/SeaWatcher/BP_SeaWatcher` OtherActor))
  (if (`self.Armed`)
    (`GameplayStatics.ApplyDamage` _asbp_sea_watcher 5.0)
    (`KismetSystemLibrary.Delay` 1.0)
    (bind _asbp_sea_watcher_2 (cast `/Game/Characters/SeaWatcher/BP_SeaWatcher` (`GameplayStatics.GetPlayerCharacter` 0)))
    (`/Game/Characters/SeaWatcher/BP_SeaWatcher.ResetDammage` _asbp_sea_watcher)
    (`/Game/Characters/SeaWatcher/BP_SeaWatcher.ResetDammage` _asbp_sea_watcher_2)))

(event `Hit`
  (bind _output (`|GetArrayItem` (`PrimitiveComponent.GetOverlappingActors` (`self.HitSphere`) "/Game/Characters/SeaWatcher/BP_SeaWatcher.BP_SeaWatcher_C")))
  (`/Engine/EditorBlueprintResources/StandardMacros.IsValid` _output
    (:`Is Valid`
      (`GameplayStatics.ApplyDamage` _output 5.0)
      (`KismetSystemLibrary.Delay` 1.0)
      (bind _asbp_sea_watcher (cast `/Game/Characters/SeaWatcher/BP_SeaWatcher` (`GameplayStatics.GetPlayerCharacter` 0)))
      (`/Game/Characters/SeaWatcher/BP_SeaWatcher.ResetDammage` _asbp_sea_watcher)
      (`self.Hit`))))

(fn `UserConstructionScript`)