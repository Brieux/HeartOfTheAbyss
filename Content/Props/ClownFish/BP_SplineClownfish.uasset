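; BP_SplineClownfish is a clownfish prop that moves its skeletal mesh along a spline.
; On BeginPlay it sets a timeline play rate inversely proportional to the Time variable and plays the Movetrack timeline.
; Each update samples the spline at Movetrack to set the mesh's world location and rotation, adding a half-turn of yaw.
; The rotation is sampled in local space but applied as world rotation.
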(event `self.ReceiveBeginPlay`
  (bind _skeletalmesh (`self.SkeletalMesh`))
  (`TimelineComponent.SetPlayRate` (`self.Timeline_0`) (/ 0.4 (`self.time`)))
  (bind (_direction _movetrack) (`Timeline|Timeline_0`)
    (:`Update`
      (`SceneComponent.K2_SetWorldLocation` _skeletalmesh (`SplineComponent.GetLocationAtTime` (`self.Spline`) _movetrack "World" false) false false)
      (`SceneComponent.K2_SetWorldRotation` _skeletalmesh (`KismetMathLibrary.MakeRotator` (.roll (`SplineComponent.GetRotationAtTime` (`self.Spline`) _movetrack "Local" false)) (.pitch (`SplineComponent.GetRotationAtTime` (`self.Spline`) _movetrack "Local" false)) (+ (.yaw (`SplineComponent.GetRotationAtTime` (`self.Spline`) _movetrack "Local" false)) 180.0)) false false))))

(fn `UserConstructionScript`)