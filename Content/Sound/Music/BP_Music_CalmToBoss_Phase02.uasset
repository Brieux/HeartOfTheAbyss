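; Box trigger that switches the music from the post-phase-one track to the boss phase-two track.
; On BeginPlay it caches the first BP_Switch_Music_CalmToVnr actor, which owns both music components.
; The first BP_SeaWatcher overlap crossfades those tracks with a short delay, then fades in a Zlag ambience loop attached to its Loop component.
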(event `FadeMusic`
  (`AudioComponent.FadeOut` (`/Game/Sound/Music/BP_Switch_Music_CalmToVnr.Music_Post_Phase01` (`self.SwitchMusic`)) 5.0 0.0 "Linear")
  (`KismetSystemLibrary.Delay` 1.0)
  (`AudioComponent.FadeIn` (`/Game/Sound/Music/BP_Switch_Music_CalmToVnr.Music_Boss_Phase02` (`self.SwitchMusic`)) 1.0 1.0 0.0 "Linear"))

(event `self.ReceiveBeginPlay`
  (bind _outactors (`GameplayStatics.GetAllActorsOfClass` "/Game/Sound/Music/BP_Switch_Music_CalmToVnr.BP_Switch_Music_CalmToVnr_C"))
  (set `self.SwitchMusic` (`|GetArrayItem` _outactors)))

(event `self.Box.OnComponentBeginOverlap`
  (params (OverlappedComponent :type "PrimitiveComponent Object Reference") (OtherActor :type "Actor Object Reference") (OtherComp :type "PrimitiveComponent Object Reference") (OtherBodyIndex :type Integer) (bFromSweep :type Boolean) (SweepResult :type "HitResult Structure (by ref)"))
  (cast `/Game/Characters/SeaWatcher/BP_SeaWatcher` OtherActor)
  (`/Engine/EditorBlueprintResources/StandardMacros.DoOnce` false
    (:`Completed`
      (`self.FadeMusic`)
      (bind _returnvalue (`GameplayStatics.SpawnSoundAttached` "/Game/Sound/Ambs/AMB_Zlag_LP_Cue.AMB_Zlag_LP_Cue" (`self.Loop`) "None" (0.0 0.0 0.0) (struct) "KeepRelativeOffset" false 1.0 1.0 0.0 null null))
      (`AudioComponent.FadeIn` _returnvalue 8.0 1.0 0.0 "Linear"))))

(fn `UserConstructionScript`)