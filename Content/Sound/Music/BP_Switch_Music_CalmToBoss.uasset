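; BP_Switch_Music_CalmToBoss is a music trigger that switches the soundtrack from calm to boss music.
; On BeginPlay it finds the first BP_Switch_Music_CalmToVnr actor and stores it as the owner of the audio components.
; When a BP_SeaWatcher overlaps its Box, it crossfades that actor's components, fading out the calm track and fading in the boss track.
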(event `self.ReceiveBeginPlay`
  (bind _outactors (`GameplayStatics.GetAllActorsOfClass` "/Game/Sound/Music/BP_Switch_Music_CalmToVnr.BP_Switch_Music_CalmToVnr_C"))
  (set `self.Switch_Music02` (`|GetArrayItem` _outactors)))

(event `self.Box.OnComponentBeginOverlap`
  (params (OverlappedComponent :type "PrimitiveComponent Object Reference") (OtherActor :type "Actor Object Reference") (OtherComp :type "PrimitiveComponent Object Reference") (OtherBodyIndex :type Integer) (bFromSweep :type Boolean) (SweepResult :type "HitResult Structure (by ref)"))
  (bind _asbp_sea_watcher (cast `/Game/Characters/SeaWatcher/BP_SeaWatcher` OtherActor))
  (if (== _asbp_sea_watcher OtherActor)
    (`AudioComponent.FadeOut` (`/Game/Sound/Music/BP_Switch_Music_CalmToVnr.Music_Calm_Test` (`self.Switch_Music02`)) 5.0 0.0 "Linear")
    (`AudioComponent.FadeIn` (`/Game/Sound/Music/BP_Switch_Music_CalmToVnr.Music_Boss_Test` (`self.Switch_Music02`)) 5.0 1.0 0.0 "Linear")))

(fn `UserConstructionScript`)