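; Level music switch trigger that moves the soundtrack from calm to VNR music.
; On BeginPlay it fades in the calm track and stops the VNR and boss tracks.
; When BP_SeaWatcher overlaps its Box, it fades out the calm track and fades in the VNR track.
; The switch is one-way, and the boss track is never started here.
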(event `self.ReceiveBeginPlay`
  (`AudioComponent.FadeIn` (`self.Music_Calm_Test`) 8.0 1.0 0.0 "Linear")
  (`AudioComponent.Stop` (`self.Music_Vnr_Test`))
  (`AudioComponent.Stop` (`self.Music_Boss_Test`)))

(event `self.Box.OnComponentBeginOverlap`
  (params (OverlappedComponent :type "PrimitiveComponent Object Reference") (OtherActor :type "Actor Object Reference") (OtherComp :type "PrimitiveComponent Object Reference") (OtherBodyIndex :type Integer) (bFromSweep :type Boolean) (SweepResult :type "HitResult Structure (by ref)"))
  (bind _asbp_sea_watcher (cast `/Game/Characters/SeaWatcher/BP_SeaWatcher` OtherActor))
  (if (== OtherActor _asbp_sea_watcher)
    (`AudioComponent.FadeOut` (`self.Music_Calm_Test`) 2.0 0.0 "Linear")
    (`AudioComponent.FadeIn` (`self.Music_Vnr_Test`) 2.0 1.0 0.0 "Linear")))

(fn `UserConstructionScript`)