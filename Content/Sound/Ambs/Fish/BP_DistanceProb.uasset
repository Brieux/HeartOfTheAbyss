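; BP_DistanceProb is a debug probe for the distance between the BP_SeaWatcher character and a fish's audio source.
; At BeginPlay it caches the first BP_SeaWatcher and BP_SplineFish_2 found in the level.
; Each tick it normalizes the X-axis offset between the character mesh and the fish Audio component, then prints it.
; An unconnected node would mute the fish audio, so the volume is never changed.
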(event `self.ReceiveBeginPlay`
  (bind _outactors (`GameplayStatics.GetAllActorsOfClass` "/Game/Characters/SeaWatcher/BP_SeaWatcher.BP_SeaWatcher_C"))
  (set `self.Perso` (`|GetArrayItem` _outactors))
  (bind _outactors_2 (`GameplayStatics.GetAllActorsOfClass` "/Game/VFX/Blueprint/BP_SplineFish_2.BP_SplineFish_2_C"))
  (set `self.Poisson` (`|GetArrayItem` _outactors_2)))

(event `self.ReceiveTick`
  (params (DeltaSeconds :type "Float (single-precision)"))
  (bind _returnvalue_x (`KismetMathLibrary.BreakVector` (`SceneComponent.K2_GetComponentLocation` (`Character.Mesh` (`self.Perso`)))))
  (bind _returnvalue_x_2 (`KismetMathLibrary.BreakVector` (`SceneComponent.K2_GetComponentLocation` (`/Game/VFX/Blueprint/BP_SplineFish_2.Audio` (`self.Poisson`)))))
  (bind _output_get (set `self.NewVar` (`KismetMathLibrary.NormalizeToRange` (- _returnvalue_x _returnvalue_x_2) 1.0 4.0)))
  (`KismetSystemLibrary.PrintString` (`KismetStringLibrary.Conv_DoubleToString` _output_get)))

(fn `UserConstructionScript`)